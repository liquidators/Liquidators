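; BP_Computer_Terminal_Master is the base Blueprint for a computer terminal with a UI_ComputerTerminal widget as its interface.
; On BeginPlay it casts its widget component's user widget, assigns itself as that widget's terminal instance and keeps a reference to the widget.
; An UnlockTerminal event, meant for save-game restore, clears the lock on both actor and widget and switches the widget switcher to its first page.
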(event `self.ReceiveBeginPlay`
  ;[0 0.8796 1] Begin - Set self as Instance for respective User Interface Widget
  (bind _asui_computer_terminal (cast `/Game/WISTerminals/UserInterface/UI_ComputerTerminal` (`WidgetComponent.GetUserWidgetObject` (`self.Widget`))))
  (set `/Game/WISTerminals/UserInterface/UI_ComputerTerminal.TerminalInstance` self _asui_computer_terminal)
  (set `self.TerminalInterface` _asui_computer_terminal))

(event `UnlockTerminal`
  (bind _terminalinterface (`self.TerminalInterface`))
  ;[0 0.8796 1] Unlock from save game
  (set `/Game/WISTerminals/UserInterface/UI_ComputerTerminal.PasswordLocked` false _terminalinterface)
  (set `self.Locked` false)
  (`WidgetSwitcher.SetActiveWidgetIndex` (`/Game/WISTerminals/UserInterface/UI_ComputerTerminal.TerminalSwitch` _terminalinterface) 0))

(fn `UserConstructionScript`
  (`parent.UserConstructionScript`))