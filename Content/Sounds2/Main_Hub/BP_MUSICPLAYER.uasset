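; BP_MUSICPLAYER is a music player Blueprint that crossfades between tracks when the music intensity changes.
; Change Music Intensity stores the new index in Count and calls PlayMusicWithFade, which picks that track from the AOMUSIC array.
; Two audio components alternate roles based on whether the first is playing, while the Fades timeline, rate-scaled to the fade duration, drives both volumes and stops the outgoing one.
; The Play Music function is empty.
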(event `Play Music With Fade`
  (params (`Fade Duration` :type "Float (double-precision)"))
  (bind _audiotofadein (`self.AudioToFadein`))
  (set `self.FadeDuration` `Fade Duration`)
  (`|ExecutionSequence`
    (:`then_0`
      (if (`AudioComponent.IsPlaying` (`self.Audio`))
        (set `self.AudioToFadeout` (`self.Audio`))
        (set `self.AudioToFadein` (`self.Audio2`))
        (else
          (set `self.AudioToFadeout` (`self.Audio2`))
          (set `self.AudioToFadein` (`self.Audio`)))))
    (:`then_1`
      (`AudioComponent.SetSound` _audiotofadein (`|GetArrayItem` (`self.AOMUSIC`) (`self.Count`)))
      (`AudioComponent.Play` _audiotofadein 0.0)
      (`TimelineComponent.SetPlayRate` (`self.Fades`) (/ 1.0 (`self.FadeDuration`)))
      (bind (_direction _fadein _fadeout) (`Timeline|Fades` :!via `PlayFromStart`)
        (:`Update`
          (`AudioComponent.SetVolumeMultiplier` (`self.AudioToFadeout`) _fadeout)
          (`AudioComponent.SetVolumeMultiplier` (`self.AudioToFadein`) _fadein))
        (:`Finished`
          (`AudioComponent.Stop` (`self.AudioToFadeout`)))))))

(fn `Change Music Intensity`
  (params (NewVar_0 :type Integer))
  (set `self.Count` NewVar_0)
  (`self.Play Music With Fade` 3.0))

(fn `Play Music`
  (params (`Fade Duration` :type "Float (double-precision)")))

(fn `UserConstructionScript`)