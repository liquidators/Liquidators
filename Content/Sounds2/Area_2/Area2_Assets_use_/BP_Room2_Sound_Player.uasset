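; Room 2 sound player for Area 2 that builds a layered music sequence at a stored location.
; PlayMusic spawns seven cues in turn at fixed five-second delays, from liquid through percussion to Shepard tone and scream, keeping each audio component.
; ResetMusic stops each valid component but does not cancel the pending delay chain, so later layers can still start after a reset.
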(event `PlayMusic`
  (bind _location (`self.Location`))
  (bind _returnvalue (`GameplayStatics.SpawnSoundAtLocation` "/Game/Sounds2/Area_2/Area2_Assets_use_/Part_2/1_Liquid/Area2_Pt_Liquid_Cue.Area2_Pt_Liquid_Cue" _location (struct) 1.0 1.0 0.0 null null))
  (set `self.Sound_Liquid` _returnvalue)
  (`KismetSystemLibrary.Delay` 5.0)
  (bind _returnvalue_2 (`GameplayStatics.SpawnSoundAtLocation` "/Game/Sounds2/Area_2/Area2_Assets_use_/Part_2/2_Drain_Shuffle_/Area2_Pt2_Drain1_Cue.Area2_Pt2_Drain1_Cue" _location (struct) 1.0 1.0 0.0 null null))
  (set `self.Sound_Shuffle` _returnvalue_2)
  (`KismetSystemLibrary.Delay` 5.0)
  (bind _returnvalue_3 (`GameplayStatics.SpawnSoundAtLocation` "/Game/Sounds2/Area_2/Area2_Assets_use_/Part_2/3_Pulse/Area2_Pt2_Pulse_Cue.Area2_Pt2_Pulse_Cue" _location (struct) 1.0 1.0 0.0 null null))
  (set `self.Sound_Pulse` _returnvalue_3)
  (`KismetSystemLibrary.Delay` 5.0)
  (bind _returnvalue_4 (`GameplayStatics.SpawnSoundAtLocation` "/Game/Sounds2/Area_2/Area2_Assets_use_/Part_2/4_Percussion/Area2_Pt2_Percussion_Cue.Area2_Pt2_Percussion_Cue" _location (struct) 1.0 1.0 0.0 null null))
  (set `self.Sound_Percussion` _returnvalue_4)
  (`KismetSystemLibrary.Delay` 5.0)
  (bind _returnvalue_5 (`GameplayStatics.SpawnSoundAtLocation` "/Game/Sounds2/Area_2/Area2_Assets_use_/Part_2/5_Hit/Area2_Pt2_BigHit_Cue.Area2_Pt2_BigHit_Cue" _location (struct) 1.0 1.0 0.0 null null))
  (set `self.Sound_Hit` _returnvalue_5)
  (`KismetSystemLibrary.Delay` 5.0)
  (bind _returnvalue_6 (`GameplayStatics.SpawnSoundAtLocation` "/Game/Sounds2/Area_2/Area2_Assets_use_/Part_2/6_ShepardTone/Area2_Pt2_ShepardTone_Cue.Area2_Pt2_ShepardTone_Cue" _location (struct) 1.0 1.0 0.0 null null))
  (set `self.Sound_ShepardTone` _returnvalue_6)
  (`KismetSystemLibrary.Delay` 5.0)
  (bind _returnvalue_7 (`GameplayStatics.SpawnSoundAtLocation` "/Game/Sounds2/Area_2/Area2_Assets_use_/Part_2/7_Scream/Area2_Pt2_Scream_Cue.Area2_Pt2_Scream_Cue" _location (struct) 1.0 1.0 0.0 null null))
  (set `self.Sound_Scream` _returnvalue_7))

(event `ResetMusic`
  (bind _sound_liquid (`self.Sound_Liquid`))
  (bind _sound_shuffle (`self.Sound_Shuffle`))
  (bind _sound_pulse (`self.Sound_Pulse`))
  (bind _sound_percussion (`self.Sound_Percussion`))
  (bind _sound_hit (`self.Sound_Hit`))
  (bind _sound_shepardtone (`self.Sound_ShepardTone`))
  (bind _sound_scream (`self.Sound_Scream`))
  (`/Engine/EditorBlueprintResources/StandardMacros.IsValid` _sound_liquid
    (:`Is Valid`
      (`AudioComponent.Stop` _sound_liquid))
    (:`Is Not Valid`
      _))
  (`/Engine/EditorBlueprintResources/StandardMacros.IsValid` _sound_shuffle
    (:`Is Valid`
      (`AudioComponent.Stop` _sound_shuffle))
    (:`Is Not Valid`
      _))
  (`/Engine/EditorBlueprintResources/StandardMacros.IsValid` _sound_pulse
    (:`Is Valid`
      (`AudioComponent.Stop` _sound_pulse))
    (:`Is Not Valid`
      _))
  (`/Engine/EditorBlueprintResources/StandardMacros.IsValid` _sound_percussion
    (:`Is Valid`
      (`AudioComponent.Stop` _sound_percussion))
    (:`Is Not Valid`
      _))
  (`/Engine/EditorBlueprintResources/StandardMacros.IsValid` _sound_hit
    (:`Is Valid`
      (`AudioComponent.Stop` _sound_hit))
    (:`Is Not Valid`
      _))
  (`/Engine/EditorBlueprintResources/StandardMacros.IsValid` _sound_shepardtone
    (:`Is Valid`
      (`AudioComponent.Stop` _sound_shepardtone))
    (:`Is Not Valid`
      _))
  (`/Engine/EditorBlueprintResources/StandardMacros.IsValid` _sound_scream
    (:`Is Valid`
      (`AudioComponent.Stop` _sound_scream))))

(fn `UserConstructionScript`)