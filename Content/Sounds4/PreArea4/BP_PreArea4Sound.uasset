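; BP_PreArea4Sound is a sound actor that controls two audio components, a main track and a beat, for PreArea4.
; Both are stopped on BeginPlay and wait for play and stop events.
; Play events fade in over a few seconds, guarded by per-track flags against retriggering.
; Stop events clear the flag, with the main track fading out gradually and the beat cutting instantly.
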(event `self.ReceiveBeginPlay`
  (`AudioComponent.Stop` (`self.MainTrack`))
  (`AudioComponent.Stop` (`self.Beat`)))

(event `Stop MainTrack`
  (bind _maintrack (`self.MainTrack`))
  (`/Engine/EditorBlueprintResources/StandardMacros.IsValid` _maintrack
    (:`Is Valid`
      (`AudioComponent.FadeOut` _maintrack 3.0 0.0 "Linear")
      (set `self.Is Triggered` false))))

(event `Play MainTrack`
  (if (not (`self.Is Triggered`))
    (`AudioComponent.FadeIn` (`self.MainTrack`) 3.0 1.0 0.0 "Linear")
    (set `self.Is Triggered` true)))

(event `Play Beat`
  (if (not (`self.Is Triggered2`))
    (`AudioComponent.FadeIn` (`self.Beat`) 3.0 1.0 0.0 "Linear")
    (set `self.Is Triggered2` true)))

(event `Stop Beat`
  (bind _beat (`self.Beat`))
  (`/Engine/EditorBlueprintResources/StandardMacros.IsValid` _beat
    (:`Is Valid`
      (`AudioComponent.FadeOut` _beat 0.0 0.0 "Linear")
      (set `self.Is Triggered2` false))))

(fn `UserConstructionScript`)