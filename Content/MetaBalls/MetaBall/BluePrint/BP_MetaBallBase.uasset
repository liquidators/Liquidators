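; Base metaball actor that simulates randomly seeded spheres moving tangentially around a box center and feeds them to the ShowBox material.
; Construction creates a dynamic material, filler materials and optional local render targets.
; BeginPlay seeds positions, radii and velocities; Tick updates them on randomly staggered skipped frames.
; Canvas draws encode positions and radii as pixel blocks in data textures and render spheres into a volume texture for the shader.
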(event `self.ReceiveBeginPlay`
  ;[1 1 1] PostBeginPlay
  ;;[1 1 1] Clean
  (`self.ClearVolume`)
  (`self.ClearMetas`)
  (`self.InitBalls_Rand`))

(event `self.ReceiveTick`
  (params (DeltaSeconds :type "Float (single-precision)"))
  ;[1 1 1] Tick
  (bind _biskey (`self.FrameSkip`))
  (if _biskey
    (`self.ClearVolume`)
    (`self.UpdateMetaBalls_Rand` DeltaSeconds)
    (`self.SummitBalls` true)))

(event `self.ReceiveEndPlay`
  (params (EndPlayReason :type "EEndPlayReason Enum" :default "Destroyed"))
  ;[1 1 1] EndPlay
)

(fn `ClearMetas`
  (bind _returnvalue (`KismetMathLibrary.MakeColor` 0.0 0.0 0.0 0.0))
  ;[1 1 1] Clear Pos and Radius RT
  ;;[1 1 1] Clear Radius
  (`KismetRenderingLibrary.ClearRenderTarget2D` (`self.ShpereRaDataStoreRT`) _returnvalue)
  ;;[1 1 1] Clear Position
  (`KismetRenderingLibrary.ClearRenderTarget2D` (`self.ShperePosDataStoreRT`) _returnvalue))

(fn `ClearVolume`
  ;[1 1 1] Clean the Rt for next frame rendering
  ;;[1 1 1] Clear Volume
  (`KismetRenderingLibrary.ClearRenderTarget2D` (`self.SphereVolumeDataStoreRT`) (`KismetMathLibrary.MakeColor` 0.0 0.0 0.0 0.0)))

(fn `DrawPixelOnTarget`
  (params (PixelColor :type "LinearColor Structure (by ref)") (ScreenPosition :type "Vector2D Structure") (Target :type "Canvas Object Reference") (bPassingRadius :type Boolean))
  (bind (_r _g _b _a) (`KismetMathLibrary.BreakColor` PixelColor))
  (bind _colorfiller (`self.ColorFiller`))
  ;[1 1 1] Pass via param
  (`MaterialInstanceDynamic.SetVectorParameterValue` _colorfiller "Color" (`KismetMathLibrary.SelectColor` (`KismetMathLibrary.MakeColor` _a) (`KismetMathLibrary.MakeColor` _r _g _b) bPassingRadius))
  ;[1 1 1] Draw to render targets
  (`Canvas.K2_DrawMaterial` Target _colorfiller (* ScreenPosition (`KismetMathLibrary.Conv_IntToDouble` (`self.SizeScale`))) (* (1.0 1.0) (`KismetMathLibrary.Conv_IntToDouble` (`self.SizeScale`))) (0.0 0.0) (1.0 1.0) 0.0 (0.5 0.5)))

(fn `DrawSphereOnTarget`
  (params (SphereData :type "LinearColor Structure") (Target :type "Canvas Object Reference") (Size :type "Vector2D Structure"))
  (bind _volumefiller (`self.VolumeFiller`))
  ;[1 1 1] Set Params
  ;;[1 1 1] Eps Should be
  (`MaterialInstanceDynamic.SetScalarParameterValue` _volumefiller "VolumeEps" (`KismetMathLibrary.Conv_IntToDouble` (`self.RadiusEps_Volume`)))
  ;;[1 1 1] Sphere Location in local space
  (`MaterialInstanceDynamic.SetVectorParameterValue` _volumefiller "SpherePos" SphereData)
  ;[1 1 1] Draw Sphere on volume
  (`Canvas.K2_DrawMaterial` Target (`self.VolumeFiller`) (0.0 0.0) Size (0.0 0.0) (1.0 1.0) 0.0 (0.5 0.5)))

(fn `FrameSkip`
  (returns (bIsKey :type Boolean))
  (bind _framecnt (`self.FrameCnt`))
  (set `self.FrameCnt` (`KismetMathLibrary.SelectInt` (`KismetMathLibrary.RandomIntegerInRange` 0 (`self.UpdatePerFrame`)) _framecnt (== _framecnt 0)))
  (bind _result (`/Engine/EditorBlueprintResources/StandardMacros.IncrementInt` (`self.FrameCnt`))
    (:`  `
      (return (and (== (mod _result (`self.UpdatePerFrame`)) 0) (`self.bEnable`))))))

(fn `Init`
  (bind _planertsize (`self.PlaneRTSize`))
  (bind _planertsize_2 (`self.PlaneRTSize`))
  (bind _volumesize (`self.VolumeSize`))
  (bind _showbox (`self.ShowBox`))
  (bind _metaballmat (`self.MetaballMat`))
  ;[1 1 1] UseLocalTexture Or Global Texture?
  (if (`self.bUseLocalTex`)
    (`|ExecutionSequence`
      (:`then_0`
        ;;[1 1 1] Clear Sphere's Rendertarget
        (bind _returnvalue (`KismetRenderingLibrary.CreateRenderTarget2D` _planertsize _planertsize))
        (set `self.ShpereRaDataStoreRT` _returnvalue))
      (:`then_1`
        ;;[1 1 1] Clear Position's Rendertarget
        (bind _returnvalue_2 (`KismetRenderingLibrary.CreateRenderTarget2D` _planertsize_2 _planertsize_2))
        (set `self.ShperePosDataStoreRT` _returnvalue_2))
      (:`then_2`
        ;;[1 1 1] Clear Volum's RenderTarget
        (bind _returnvalue_3 (`KismetRenderingLibrary.CreateRenderTarget2D` _volumesize _volumesize))
        (set `self.SphereVolumeDataStoreRT` _returnvalue_3))
      (:`then_3`
        ;[1 1 1] Create an instance from ShowBox
        ;;[1 1 1] Create Mat Inst For the Box
        (bind _returnvalue_4 (`PrimitiveComponent.CreateDynamicMaterialInstance` _showbox 0 (`|GetArrayItem` (`MeshComponent.GetMaterials` _showbox)) "None" :!label _label))
        (set `self.MetaballMat` _returnvalue_4)
        ;[1 1 1] Setup the params
        ;;[1 1 1] Pass RT's Info to shader
        (`|ExecutionSequence`
          (:`then_0`
            ;;[1 1 1] Pass Metaball's Properties to shader
            (`MaterialInstanceDynamic.SetScalarParameterValue` _metaballmat "SizeScale" (`KismetMathLibrary.Conv_IntToDouble` (`self.SizeScale`)))
            (`MaterialInstanceDynamic.SetScalarParameterValue` _metaballmat "SphereDataStorageSize" (`KismetMathLibrary.Conv_IntToDouble` (`self.PlaneRTSize`)))
            (`MaterialInstanceDynamic.SetScalarParameterValue` _metaballmat "SphereNums" (`KismetMathLibrary.Conv_IntToDouble` (`self.BallNums`))))
          (:`then_1`
            (`MaterialInstanceDynamic.SetTextureParameterValue` _metaballmat "RadiusTex" (`self.ShpereRaDataStoreRT`))
            (`MaterialInstanceDynamic.SetTextureParameterValue` _metaballmat "PositionTex" (`self.ShperePosDataStoreRT`))
            (`MaterialInstanceDynamic.SetTextureParameterValue` _metaballmat "VolumeRT" (`self.SphereVolumeDataStoreRT`)))
          (:`then_2`
            ;[1 1 1] Create Filler Mat Instance
            ;;[1 1 1] Filler For single Point
            (bind _returnvalue_5 (`KismetMaterialLibrary.CreateDynamicMaterialInstance` (`self.ColorFillerMat`)))
            (set `self.ColorFiller` _returnvalue_5)
            ;;[1 1 1] Filler for Volume Texture
            (bind _returnvalue_6 (`KismetMaterialLibrary.CreateDynamicMaterialInstance` (`self.VolumeFillerMat`)))
            (set `self.VolumeFiller` _returnvalue_6)
            ;[1 1 1] SetDataProps
            (bind _output_get (set `self.SizeOfDataRow` (/ (`self.PlaneRTSize`) (`self.SizeScale`))))
            (set `self.MaxSphere` (* _output_get _output_get))))))
    (else
      (goto _label))))

(fn `InitBalls_Rand`
  ;[1 1 1] Set Ball Nums according to the Max Num
  (bind _output_get (set `self.BallNums` (`KismetMathLibrary.Min` (`self.MaxSphere`) (`self.BallNums`))))
  ;[1 1 1] For Each New Ball
  (for _ (range _output_get)
    ;[1 1 1] Init locs,sizes and vels
    ;;[1 1 1] Record New Location
    (`KismetArrayLibrary.Array_Add` (`self.MetaData_Pos`) (+ (* (`KismetMathLibrary.RandomUnitVector`) (`KismetMathLibrary.RandomFloatInRange` 0.0 (`self.BoundSizeScale`))) 0.5))
    ;;[1 1 1] Get Random Radius
    (`KismetArrayLibrary.Array_Add` (`self.MetaData_Size`) (`KismetMathLibrary.RandomFloatInRange` 0.08 0.1))
    (`KismetArrayLibrary.Array_Add` (`self.MetaData_Velocity`) (* (`KismetMathLibrary.RandomUnitVector`) (`KismetMathLibrary.RandomFloatInRange` 1.0 3.0)))))

(fn `SummitBalls`
  (params (bUsingVolume :type Boolean :default true))
  (locals (ScreenPositions :type "Array of Vector2D Structure") (Spheres :type "Array of LinearColor Structure") (ScreenSize :type "Array of Vector2D Structure") (PosCanvas :type "Canvas Object Reference") (RaCanvas :type "Canvas Object Reference") (VolumeCanvas :type "Canvas Object Reference") (RaContext :type "DrawToRenderTargetContext Structure") (PosContext :type "DrawToRenderTargetContext Structure") (VolumeContext :type "DrawToRenderTargetContext Structure"))
  (bind _sizeofdatarow (`self.SizeOfDataRow`))
  (bind _sizeofdatarow_2 (`self.SizeOfDataRow`))
  (`|ExecutionSequence`
    (:`then_0`
      (if bUsingVolume
        ;[1 1 1] Begin Draw
        (bind (_canvas _size _context) (`KismetRenderingLibrary.BeginDrawCanvasToRenderTarget` (`self.SphereVolumeDataStoreRT`)))
        (set `self.Canvas_Volume` _canvas)
        (set `self.Canvas_Size_Volume` _size)
        (set `self.Canvas_Context_Volume` _context)
        ;[1 1 1] Pass data to Volume
        (for (_array_element _array_index) (`self.MetaData_Pos`)
          (`self.DrawSphereOnTarget` (`KismetMathLibrary.MakeColor` (.x _array_element) (.y _array_element) (.z _array_element) (`|GetArrayItem` (`self.MetaData_Size`) _array_index)) (`self.Canvas_Volume`) (`self.Canvas_Size_Volume`)))
        (`KismetRenderingLibrary.EndDrawCanvasToRenderTarget` (`self.Canvas_Context_Volume`))))
    (:`then_1`
      ;[1 1 1] Begin Draw
      (bind (_canvas_2 _size_2 _context_2) (`KismetRenderingLibrary.BeginDrawCanvasToRenderTarget` (`self.ShperePosDataStoreRT`)))
      (set `self.Canvas_Pos` _canvas_2)
      (set `self.Canvas_Size_Pos` _size_2)
      (set `self.Canvas_Context_Pos` _context_2)
      ;[1 1 1] Pass Position
      ;;[1 1 1] For each sphere
      (for (_array_element_2 _array_index_2) (`self.MetaData_Pos`)
        (bind _returnvalue (`KismetMathLibrary.FFloor` (/ (`KismetMathLibrary.Conv_IntToDouble` _array_index_2) (`KismetMathLibrary.Conv_IntToDouble` _sizeofdatarow_2))))
        ;;[1 1 1] Draw data
        ;;;[1 1 1] Draw single pixel to store locaiton
        (`self.DrawPixelOnTarget` (`KismetMathLibrary.MakeColor` (.x _array_element_2) (.y _array_element_2) (.z _array_element_2)) (`KismetMathLibrary.MakeVector2D` (`KismetMathLibrary.Conv_IntToDouble` (- _array_index_2 (* _returnvalue _sizeofdatarow_2))) (`KismetMathLibrary.Conv_IntToDouble` (* (`self.SizeScale`) _returnvalue))) (`self.Canvas_Pos`)))
      (`KismetRenderingLibrary.EndDrawCanvasToRenderTarget` (`self.Canvas_Context_Pos`)))
    (:`then_2`
      ;[1 1 1] Begin draw
      (bind (_canvas_3 _size_3 _context_3) (`KismetRenderingLibrary.BeginDrawCanvasToRenderTarget` (`self.ShpereRaDataStoreRT`)))
      (set `self.Canvas_Radius` _canvas_3)
      (set `self.Canvas_Size_Radius` _size_3)
      (set `self.Canvas_Context_Radius` _context_3)
      ;[1 1 1] Pass Radius
      ;;[1 1 1] For each sphere
      (for (_array_element_3 _array_index_3) (`self.MetaData_Pos`)
        (bind _returnvalue_2 (`KismetMathLibrary.FFloor` (/ (`KismetMathLibrary.Conv_IntToDouble` _array_index_3) (`KismetMathLibrary.Conv_IntToDouble` _sizeofdatarow))))
        ;;[1 1 1] Draw data
        ;;;[1 1 1] Draw single pixel to store radius
        (`self.DrawPixelOnTarget` (`KismetMathLibrary.MakeColor` (.x _array_element_3) (.y _array_element_3) (.z _array_element_3) (`|GetArrayItem` (`self.MetaData_Size`) _array_index_3)) (`KismetMathLibrary.MakeVector2D` (`KismetMathLibrary.Conv_IntToDouble` (- _array_index_3 (* _returnvalue_2 _sizeofdatarow))) (`KismetMathLibrary.Conv_IntToDouble` (* (`self.SizeScale`) _returnvalue_2))) (`self.Canvas_Radius`) true))
      (`KismetRenderingLibrary.EndDrawCanvasToRenderTarget` (`self.Canvas_Context_Radius`)))))

(fn `UpdataLight`
  ;[1 1 1] Find and get light's transform
  ;;[1 1 1] GetAll Directional Light
  (bind _outactors (`GameplayStatics.GetAllActorsOfClass` "/Script/Engine.DirectionalLight"))
  ;;[1 1 1] Pass the Light Dir to shader
  (`MaterialInstanceDynamic.SetVectorParameterValue` (`self.MetaballMat`) "LightVec" (`KismetMathLibrary.Conv_VectorToLinearColor` (* (`KismetMathLibrary.TransformDirection` (`SceneComponent.K2_GetComponentToWorld` (`self.Root`)) (`SceneComponent.GetForwardVector` (`Light.LightComponent` (`|GetArrayItem` _outactors)))) -1.0))))

(fn `UpdateMetaBalls_Rand`
  (params (DeltaTime :type "Float (double-precision)"))
  (bind _metadata_pos (`self.MetaData_Pos`))
  ;[1 1 1] Rotate Around Center
  (for (_array_element _array_index) _metadata_pos
    ;;[1 1 1] Update Position
    (`KismetArrayLibrary.Array_Set` _metadata_pos _array_index (+ (* (`KismetMathLibrary.Normal` (`KismetMathLibrary.Cross_VectorVector` (`KismetMathLibrary.Normal` (- _array_element (0.5 0.5 0.5))) (`|GetArrayItem` (`self.MetaData_Velocity`) _array_index))) (* (* (`self.UpdatePerFrame`) DeltaTime) (`self.Speed`))) _array_element))))

(fn `UserConstructionScript`
  (`self.Init`))