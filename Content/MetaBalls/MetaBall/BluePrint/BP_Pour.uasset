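; Metaball pouring effect: simulates a stream of balls falling through a normalized volume to fill a looping water level.
; BeginPlay fills position, velocity and size arrays, then activates randomly sized balls one by one on a delay.
; Frame-skip-gated Tick clears the volume, applies XY drift and gravity, then submits balls and light direction to the shader.
; Balls reaching the bottom respawn on top and add cubed size to WaterHeight, wrapped by Fraction for the material.
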(event `self.ReceiveBeginPlay`
  (bind (_xyspawnlocation_x _xyspawnlocation_y) (`KismetMathLibrary.BreakVector2D` (`self.XYSpawnLocation`)))
  ;[1 1 1] Init the Dropper
  (for _ (range (`self.BallNums`))
    (`KismetArrayLibrary.Array_Add` (`self.MetaData_Pos`) (`KismetMathLibrary.MakeVector` _xyspawnlocation_x _xyspawnlocation_y 1.0))
    (`KismetArrayLibrary.Array_Add` (`self.MetaData_Velocity`))
    (`KismetArrayLibrary.Array_Add` (`self.MetaData_Size`)))
  ;[1 1 1] Spawn balls with delay
  (`self.AddBalls_Rand_Pour` :!label _label)
  (if (< (`self.CurrentAddedCnt`) (`self.BallNums`))
    (`KismetSystemLibrary.Delay` (`self.SpawnTime`))
    (goto _label)))

(event `self.ReceiveTick`
  (params (DeltaSeconds :type "Float (single-precision)"))
  ;[1 1 1] For each tick,Clear the Volume and Update Ball in the Tube,and summit it,and update the directional light from the scene
  (bind _biskey (`self.FrameSkip`))
  (if _biskey
    ;;[1 1 1] Clear the Volume
    (`self.ClearVolume`)
    ;;[1 1 1] Update Locations In Tube
    (`self.UpdateBalls_Pour` DeltaSeconds)
    ;;[1 1 1] ReSummit Locations to shader
    (`self.SummitBalls` false)
    ;;[1 1 1] Update Light direction to shader
    (`self.UpdataLight`)
    ;[1 1 1] Update Height of Water
    (`MaterialInstanceDynamic.SetScalarParameterValue` (`self.MetaballMat`) "WaterHeight" (`KismetMathLibrary.FClamp` (* (`KismetMathLibrary.Fraction` (`self.WaterHeight`)) 0.3) 0.01 0.5))))

(fn `AddBalls_Rand_Pour`
  (bind (_returnvalue_x _returnvalue_y) (`KismetMathLibrary.BreakVector2D` (* (`KismetMathLibrary.Normal2D` (`self.XYVelocity`)) (`self.XYVelocityScale`))))
  (`KismetArrayLibrary.Array_Set` (`self.MetaData_Pos`) (`self.CurrentAddedCnt`) (`self.InitialPosition`))
  (`KismetArrayLibrary.Array_Set` (`self.MetaData_Size`) (`self.CurrentAddedCnt`) (`KismetMathLibrary.RandomFloatInRange` (`self.minSize`) (`self.maxSize`)))
  (`KismetArrayLibrary.Array_Set` (`self.MetaData_Velocity`) (`self.CurrentAddedCnt`) (`KismetMathLibrary.MakeVector` _returnvalue_x _returnvalue_y))
  (`/Engine/EditorBlueprintResources/StandardMacros.IncrementInt` (`self.CurrentAddedCnt`)))

(fn `InitialPosition`
  (returns (ReturnValue :type "Vector Structure"))
  (bind (_xyspawnlocation_x _xyspawnlocation_y) (`KismetMathLibrary.BreakVector2D` (`self.XYSpawnLocation`)))
  (bind _startradius (`self.StartRadius`))
  (return (+ (`KismetMathLibrary.MakeVector` (* _startradius (.x (`KismetMathLibrary.RandomUnitVector`))) (* (.y (`KismetMathLibrary.RandomUnitVector`)) _startradius) 1.0) (`KismetMathLibrary.MakeVector` _xyspawnlocation_x _xyspawnlocation_y))))

(fn `UpdateBalls_Pour`
  (params (DeltaTime :type "Float (double-precision)"))
  (bind _metadata_pos (`self.MetaData_Pos`))
  (bind _metadata_velocity (`self.MetaData_Velocity`))
  (bind _returnvalue (* (`self.UpdatePerFrame`) DeltaTime))
  (bind (_returnvalue_x _returnvalue_y) (`KismetMathLibrary.BreakVector2D` (* (`KismetMathLibrary.Normal2D` (`self.XYVelocity`)) (`self.XYVelocityScale`))))
  (for (_array_element _array_index) _metadata_pos
    (if (> (`|GetArrayItem` (`self.MetaData_Size`) _array_index) 0.0)
      (bind _returnvalue_2 (- (.z _array_element) (* _returnvalue (.z (`|GetArrayItem` (`self.MetaData_Velocity`) _array_index)))))
      (if (<= _returnvalue_2 0.0)
        (`KismetArrayLibrary.Array_Set` _metadata_pos _array_index (`self.InitialPosition`))
        (`KismetArrayLibrary.Array_Set` _metadata_velocity _array_index (`KismetMathLibrary.MakeVector` _returnvalue_x _returnvalue_y (* (`KismetMathLibrary.RandomFloat`) (`self.GravityScale`))))
        (bind _output (`|GetArrayItem` (`self.MetaData_Size`) _array_index))
        (set `self.WaterHeight` (+ (* (`self.WaterHeightDeltaScale`) (* _output _output _output 100.0)) (`self.WaterHeight`)))
        (else
          (`KismetArrayLibrary.Array_Set` _metadata_pos _array_index (`KismetMathLibrary.MakeVector` (+ (* _returnvalue (.x (`|GetArrayItem` (`self.MetaData_Velocity`) _array_index))) (.x _array_element)) (+ (* _returnvalue (.y (`|GetArrayItem` (`self.MetaData_Velocity`) _array_index))) (.y _array_element)) (`KismetMathLibrary.FClamp` _returnvalue_2)))
          (bind (_output_x _output_y _output_z) (`KismetMathLibrary.BreakVector` (`|GetArrayItem` _metadata_velocity _array_index)))
          (`KismetArrayLibrary.Array_Set` _metadata_velocity _array_index (`KismetMathLibrary.MakeVector` _output_x _output_y (+ _output_z (* _returnvalue 9.8 (`self.GravityScale`))))))))))

(fn `UserConstructionScript`
  (`parent.UserConstructionScript`))