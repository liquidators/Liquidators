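; BP_Dropper is a metaball effect that streams balls along Z inside a tube in a normalized volume.
; BeginPlay scatters balls around the volume center with random radii and Z speeds.
; On ticks passed by FrameSkip, it clears the volume, moves the balls, resubmits them to the shader and updates the light direction.
; Movement subtracts scaled velocity from Z and wraps it fractionally within SideClip margins, looping the drops endlessly.
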(event `self.ReceiveBeginPlay`
  ;[1 1 1] Init the Dropper
  (`self.InitBalls_Rand_InTube`))

(event `self.ReceiveTick`
  (params (DeltaSeconds :type "Float (single-precision)"))
  ;[1 1 1] For each tick,Clear the Volume and Update Ball in the Tube,and summit it,and update the directional light from the scene
  (bind _biskey (`self.FrameSkip`))
  (if _biskey
    ;;[1 1 1] Clear the Volume
    (`self.ClearVolume`)
    ;;[1 1 1] Update Locations In Tube
    (`self.UpdateBalls_InTube` DeltaSeconds)
    ;;[1 1 1] ReSummit Locations to shader
    (`self.SummitBalls` true)
    ;;[1 1 1] Update Light direction to shader
    (`self.UpdataLight`)))

(fn `InitBalls_Rand_InTube`
  (bind _tuberadius (`self.TubeRadius`))
  (for _ (range (`self.BallNums`))
    (`KismetArrayLibrary.Array_Add` (`self.MetaData_Pos`) (`KismetMathLibrary.MakeVector` (+ (* _tuberadius (.x (`KismetMathLibrary.RandomUnitVector`))) 0.5) (+ (* (.y (`KismetMathLibrary.RandomUnitVector`)) _tuberadius) 0.5) (+ (* (.z (`KismetMathLibrary.RandomUnitVector`)) 0.5) 0.5)))
    (`KismetArrayLibrary.Array_Add` (`self.MetaData_Size`) (`KismetMathLibrary.RandomFloatInRange` (`self.minRadius`) (`self.maxRadius`)))
    (`KismetArrayLibrary.Array_Add` (`self.MetaData_Velocity`) (`KismetMathLibrary.MakeVector` 0.0 0.0 (`KismetMathLibrary.RandomFloatInRange` (`self.minSpeed`) (`self.maxSpeed`))))))

(fn `UpdateBalls_InTube`
  (params (DeltaTime :type "Float (double-precision)"))
  (bind _metadata_pos (`self.MetaData_Pos`))
  (bind _sideclip (`self.SideClip`))
  (bind _sideclip_2 (`self.SideClip`))
  (for (_array_element _array_index) _metadata_pos
    (bind _returnvalue (- (/ (- (.z _array_element) (* _sideclip_2 0.5)) (- 1.0 _sideclip_2)) (* (* (`self.UpdatePerFrame`) DeltaTime) (.z (`|GetArrayItem` (`self.MetaData_Velocity`) _array_index)))))
    (`KismetArrayLibrary.Array_Set` _metadata_pos _array_index (`KismetMathLibrary.MakeVector` (.x _array_element) (.y _array_element) (+ (* (`KismetMathLibrary.Abs` (- _returnvalue (`KismetMathLibrary.Conv_IntToDouble` (`KismetMathLibrary.FFloor` _returnvalue)))) (- 1.0 _sideclip)) (* _sideclip 0.5))))))

(fn `UserConstructionScript`
  (`parent.UserConstructionScript`))