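; BP_Rotator_Colorful is a metaball actor that gives each randomly initialized ball its own color.
; On BeginPlay it generates random-hue colors and writes them pixel by pixel into a render target, wrapping the 1D array into 2D rows as a data texture.
; On Tick, gated by FrameSkip, it clears the volume, updates the balls, submits them to the shader and updates the light.
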(event `self.ReceiveBeginPlay`
  ;[1 1 1] Init The Rotator
  (`self.InitBalls_Rand`)
  (`self.RandomColors`)
  (`self.SummitColors`))

(event `self.ReceiveTick`
  (params (DeltaSeconds :type "Float (single-precision)"))
  ;[1 1 1] Every tick,Update the locations of every ball and Summit it
  (bind _biskey (`self.FrameSkip`))
  (if _biskey
    ;;[1 1 1] Clear Volume
    (`self.ClearVolume`)
    ;;[1 1 1] Update Balls
    (`self.UpdateMetaBalls_Rand` DeltaSeconds)
    ;;[1 1 1] Summit to shader
    (`self.SummitBalls` true)
    ;;[1 1 1] Update Light
    (`self.UpdataLight`)))

(fn `RandomColors`
  (for _ (range (`self.BallNums`))
    (`KismetArrayLibrary.Array_Add` (`self.MetaData_Color`) (`KismetMathLibrary.HSVToRGB` (`KismetMathLibrary.RandomFloatInRange` 0.0 360.0) 0.7 1.0))))

(fn `SummitColors`
  (bind _sizeofdatarow (`self.SizeOfDataRow`))
  (bind (_canvas _size _context) (`KismetRenderingLibrary.BeginDrawCanvasToRenderTarget` (`self.ShpereColorDataStoreRT`)))
  (set `self.Canvas_Color` _canvas)
  (set `self.Canvas_Color_Size` _size)
  (set `self.Canvas_Color_Context` _context)
  (for (_array_element _array_index) (`self.MetaData_Color`)
    (bind _returnvalue (`KismetMathLibrary.FFloor` (/ (`KismetMathLibrary.Conv_IntToDouble` _array_index) (`KismetMathLibrary.Conv_IntToDouble` _sizeofdatarow))))
    (`self.DrawPixelOnTarget` _array_element (`KismetMathLibrary.MakeVector2D` (`KismetMathLibrary.Conv_IntToDouble` (- _array_index (* _returnvalue _sizeofdatarow))) (`KismetMathLibrary.Conv_IntToDouble` (* (`self.SizeScale`) _returnvalue))) (`self.Canvas_Color`)))
  (`KismetRenderingLibrary.EndDrawCanvasToRenderTarget` (`self.Canvas_Color_Context`)))

(fn `UserConstructionScript`
  (`parent.UserConstructionScript`))