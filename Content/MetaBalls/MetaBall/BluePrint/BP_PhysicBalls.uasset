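; Metaball actor that uses physics-simulated spheres to drive metaball data submitted to a volume.
; BeginPlay spawns randomly sized and placed mesh balls with size-based mass, recording position, radius and velocity arrays.
; On frames passing FrameSkip, Tick clears the volume, converts ball positions into roughly 0–1 box-local space, spins a cross component, submits balls and updates lighting.
; RotateSelf, a sine-driven box rock, is defined but not called here.
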(event `self.ReceiveBeginPlay`
  ;[1 1 1] Init and spawn physic balls
  (`self.SpawnBalls`))

(event `self.ReceiveTick`
  (params (DeltaSeconds :type "Float (single-precision)"))
  ;[1 1 1] Tick
  (bind _biskey (`self.FrameSkip`))
  (if _biskey
    ;;[1 1 1] Volume Should be cleared every frame
    (`self.ClearVolume`)
    ;;[1 1 1] Update and summit
    (`self.UpdataBalls`)
    ;;;[1 1 1] Rotate Cross
    (`self.RotateCir` DeltaSeconds)
    ;;;[1 1 1] Summit Balls
    (`self.SummitBalls` true)
    ;;;[1 1 1] Update Light
    (`self.UpdataLight`)))

(fn `RotateCir`
  (params (DeltaTime :type "Float (double-precision)"))
  ;[1 1 1] Apply Rotation To The Cross
  (`SceneComponent.K2_AddRelativeRotation` (`self.C`) (`KismetMathLibrary.MakeRotator` 0.0 0.0 (* DeltaTime (`self.RotateSpeed2`) (`KismetMathLibrary.Conv_IntToDouble` (`self.UpdatePerFrame`)))) false false))

(fn `RotateSelf`
  (params (DeltaTime :type "Float (double-precision)"))
  (bind _root (`self.Root`))
  ;[1 1 1] Set Show Box Relative Rotation
  (`SceneComponent.K2_SetRelativeRotation` _root (`KismetMathLibrary.MakeRotator` (.roll (.rotation (`SceneComponent.GetRelativeTransform` _root))) (* (`KismetMathLibrary.Sin` (`GameplayStatics.GetTimeSeconds`)) (`self.RotateSpeed1`)) (.yaw (.rotation (`SceneComponent.GetRelativeTransform` _root)))) false false))

(fn `SpawnBalls`
  ;[1 1 1] Add physic balls
  (for _ (range (`self.BallNums`))
    ;;[1 1 1] Add PhysicBall to simulate Physic
    (bind _returnvalue (`AddComponent|NODE_AddStaticMeshComponent-0` :`RelativeTransform` (`KismetMathLibrary.MakeTransform` (* (`KismetMathLibrary.RandomUnitVector`) (- 40.0 (* (`self.MaxRadius`) 100.0))) (struct) (`KismetMathLibrary.Conv_DoubleToVector` (* (`KismetMathLibrary.RandomFloatInRange` (`self.MinRadius`) (`self.MaxRadius`)) (`self.ScaleEps`))))))
    (bind _x (.x (`SceneComponent.RelativeScale3D` _returnvalue)))
    ;[1 1 1] The bigger they are the harder they fall
    (`PrimitiveComponent.SetMassOverrideInKg` _returnvalue "None" (* _x _x (`self.massScale`)) false)
    ;[1 1 1] Init data in bp
    (`KismetArrayLibrary.Array_Add` (`self.Balls`) _returnvalue)
    ;;[1 1 1] Update Position
    (`KismetArrayLibrary.Array_Add` (`self.MetaData_Pos`) (+ (/ (- (`SceneComponent.GetSocketLocation` _returnvalue "None") (`self.K2_GetActorLocation`)) 100.0) 0.5))
    ;;[1 1 1] Update Radius
    (`KismetArrayLibrary.Array_Add` (`self.MetaData_Size`) (/ _x (`self.ScaleEps`)))
    ;;[1 1 1] Update Velocity
    (`KismetArrayLibrary.Array_Add` (`self.MetaData_Velocity`) (`KismetMathLibrary.RandomUnitVector`))))

(fn `UpdataBalls`
  ;[1 1 1] Get location,update
  (for (_array_element _array_index) (`self.Balls`)
    ;;[1 1 1] Record New Position
    (`KismetArrayLibrary.Array_Set` (`self.MetaData_Pos`) _array_index (+ (/ (`KismetMathLibrary.InverseTransformDirection` (`SceneComponent.GetRelativeTransform` (`self.Root`)) (- (`SceneComponent.GetSocketLocation` _array_element "None") (`self.K2_GetActorLocation`))) 100.0) 0.5))))

(fn `UserConstructionScript`
  (`parent.UserConstructionScript`))