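; BP_AidKit1_01 is a first aid kit prop built from multiple static mesh components, with no active gameplay logic.
; Its construction script uses FirstAidVisible to switch visibility, shadow casting and collision together on every listed mesh except StaticMeshComponent0, which it leaves untouched.
; It also applies the DrawDistance0Infinity cull distance to all these meshes, including StaticMeshComponent0.
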(fn `UserConstructionScript`
  (bind _firstaid_visible (`self.FirstAid Visible`))
  (bind _staticmeshcomponent09 (`self.StaticMeshComponent09`))
  ;[1 1 1] Visible
  (`SceneComponent.SetVisibility` _staticmeshcomponent09 _firstaid_visible false)
  (`SceneComponent.SetVisibility` (`self.StaticMeshComponent01`) _firstaid_visible false)
  (`SceneComponent.SetVisibility` (`self.StaticMeshComponent02`) _firstaid_visible false)
  (`SceneComponent.SetVisibility` (`self.StaticMeshComponent04`) _firstaid_visible false)
  (`SceneComponent.SetVisibility` (`self.StaticMeshComponent05`) _firstaid_visible false)
  (`SceneComponent.SetVisibility` (`self.StaticMeshComponent03`) _firstaid_visible false)
  (`SceneComponent.SetVisibility` (`self.StaticMeshComponent06`) _firstaid_visible false)
  (`SceneComponent.SetVisibility` (`self.StaticMeshComponent07`) _firstaid_visible false)
  (`SceneComponent.SetVisibility` (`self.StaticMeshComponent08`) _firstaid_visible false)
  (`SceneComponent.SetVisibility` (`self.StaticMeshComponent010`) _firstaid_visible false)
  (`SceneComponent.SetVisibility` (`self.StaticMeshComponent011`) _firstaid_visible false)
  (`SceneComponent.SetVisibility` (`self.StaticMeshComponent012`) _firstaid_visible false)
  (`SceneComponent.SetVisibility` (`self.StaticMeshComponent013`) _firstaid_visible false)
  (`SceneComponent.SetVisibility` (`self.StaticMeshComponent014`) _firstaid_visible false)
  (`SceneComponent.SetVisibility` (`self.StaticMeshComponent015`) _firstaid_visible false)
  (`SceneComponent.SetVisibility` (`self.StaticMeshComponent016`) _firstaid_visible false)
  (`SceneComponent.SetVisibility` (`self.StaticMeshComponent017`) _firstaid_visible false)
  (`SceneComponent.SetVisibility` (`self.StaticMeshComponent018`) _firstaid_visible false)
  (`PrimitiveComponent.SetCollisionEnabled` _staticmeshcomponent09 (select `bool` _firstaid_visible :`false` "NoCollision" :`true` "QueryAndPhysics" :!type "ECollisionEnabled Enum"))
  (`PrimitiveComponent.SetCollisionEnabled` (`self.StaticMeshComponent01`) (select `bool` _firstaid_visible :`false` "NoCollision" :`true` "QueryAndPhysics" :!type "ECollisionEnabled Enum"))
  (`PrimitiveComponent.SetCollisionEnabled` (`self.StaticMeshComponent02`) (select `bool` _firstaid_visible :`false` "NoCollision" :`true` "QueryAndPhysics" :!type "ECollisionEnabled Enum"))
  (`PrimitiveComponent.SetCollisionEnabled` (`self.StaticMeshComponent03`) (select `bool` _firstaid_visible :`false` "NoCollision" :`true` "QueryAndPhysics" :!type "ECollisionEnabled Enum"))
  (`PrimitiveComponent.SetCollisionEnabled` (`self.StaticMeshComponent04`) (select `bool` _firstaid_visible :`false` "NoCollision" :`true` "QueryAndPhysics" :!type "ECollisionEnabled Enum"))
  (`PrimitiveComponent.SetCollisionEnabled` (`self.StaticMeshComponent05`) (select `bool` _firstaid_visible :`false` "NoCollision" :`true` "QueryAndPhysics" :!type "ECollisionEnabled Enum"))
  (`PrimitiveComponent.SetCollisionEnabled` (`self.StaticMeshComponent06`) (select `bool` _firstaid_visible :`false` "NoCollision" :`true` "QueryAndPhysics" :!type "ECollisionEnabled Enum"))
  (`PrimitiveComponent.SetCollisionEnabled` (`self.StaticMeshComponent07`) (select `bool` _firstaid_visible :`false` "NoCollision" :`true` "QueryAndPhysics" :!type "ECollisionEnabled Enum"))
  (`PrimitiveComponent.SetCollisionEnabled` (`self.StaticMeshComponent08`) (select `bool` _firstaid_visible :`false` "NoCollision" :`true` "QueryAndPhysics" :!type "ECollisionEnabled Enum"))
  (`PrimitiveComponent.SetCollisionEnabled` (`self.StaticMeshComponent010`) (select `bool` _firstaid_visible :`false` "NoCollision" :`true` "QueryAndPhysics" :!type "ECollisionEnabled Enum"))
  (`PrimitiveComponent.SetCollisionEnabled` (`self.StaticMeshComponent011`) (select `bool` _firstaid_visible :`false` "NoCollision" :`true` "QueryAndPhysics" :!type "ECollisionEnabled Enum"))
  (`PrimitiveComponent.SetCollisionEnabled` (`self.StaticMeshComponent012`) (select `bool` _firstaid_visible :`false` "NoCollision" :`true` "QueryAndPhysics" :!type "ECollisionEnabled Enum"))
  (`PrimitiveComponent.SetCollisionEnabled` (`self.StaticMeshComponent013`) (select `bool` _firstaid_visible :`false` "NoCollision" :`true` "QueryAndPhysics" :!type "ECollisionEnabled Enum"))
  (`PrimitiveComponent.SetCollisionEnabled` (`self.StaticMeshComponent014`) (select `bool` _firstaid_visible :`false` "NoCollision" :`true` "QueryAndPhysics" :!type "ECollisionEnabled Enum"))
  (`PrimitiveComponent.SetCollisionEnabled` (`self.StaticMeshComponent015`) (select `bool` _firstaid_visible :`false` "NoCollision" :`true` "QueryAndPhysics" :!type "ECollisionEnabled Enum"))
  (`PrimitiveComponent.SetCollisionEnabled` (`self.StaticMeshComponent016`) (select `bool` _firstaid_visible :`false` "NoCollision" :`true` "QueryAndPhysics" :!type "ECollisionEnabled Enum"))
  (`PrimitiveComponent.SetCollisionEnabled` (`self.StaticMeshComponent017`) (select `bool` _firstaid_visible :`false` "NoCollision" :`true` "QueryAndPhysics" :!type "ECollisionEnabled Enum"))
  (`PrimitiveComponent.SetCollisionEnabled` (`self.StaticMeshComponent018`) (select `bool` _firstaid_visible :`false` "NoCollision" :`true` "QueryAndPhysics" :!type "ECollisionEnabled Enum"))
  (`PrimitiveComponent.SetCastShadow` (`self.StaticMeshComponent09`) _firstaid_visible)
  (`PrimitiveComponent.SetCastShadow` (`self.StaticMeshComponent01`) _firstaid_visible)
  (`PrimitiveComponent.SetCastShadow` (`self.StaticMeshComponent02`) _firstaid_visible)
  (`PrimitiveComponent.SetCastShadow` (`self.StaticMeshComponent04`) _firstaid_visible)
  (`PrimitiveComponent.SetCastShadow` (`self.StaticMeshComponent05`) _firstaid_visible)
  (`PrimitiveComponent.SetCastShadow` (`self.StaticMeshComponent03`) _firstaid_visible)
  (`PrimitiveComponent.SetCastShadow` (`self.StaticMeshComponent06`) _firstaid_visible)
  (`PrimitiveComponent.SetCastShadow` (`self.StaticMeshComponent07`) _firstaid_visible)
  (`PrimitiveComponent.SetCastShadow` (`self.StaticMeshComponent08`) _firstaid_visible)
  (`PrimitiveComponent.SetCastShadow` (`self.StaticMeshComponent010`) _firstaid_visible)
  (`PrimitiveComponent.SetCastShadow` (`self.StaticMeshComponent011`) _firstaid_visible)
  (`PrimitiveComponent.SetCastShadow` (`self.StaticMeshComponent012`) _firstaid_visible)
  (`PrimitiveComponent.SetCastShadow` (`self.StaticMeshComponent013`) _firstaid_visible)
  (`PrimitiveComponent.SetCastShadow` (`self.StaticMeshComponent014`) _firstaid_visible)
  (`PrimitiveComponent.SetCastShadow` (`self.StaticMeshComponent015`) _firstaid_visible)
  (`PrimitiveComponent.SetCastShadow` (`self.StaticMeshComponent016`) _firstaid_visible)
  (`PrimitiveComponent.SetCastShadow` (`self.StaticMeshComponent017`) _firstaid_visible)
  (`PrimitiveComponent.SetCastShadow` (`self.StaticMeshComponent018`) _firstaid_visible)
  ;[1 1 1] Render distance
  (`PrimitiveComponent.SetCullDistance` (`self.StaticMeshComponent09`) (`self.Draw Distance (0 - Infinity)`))
  (`PrimitiveComponent.SetCullDistance` (`self.StaticMeshComponent01`) (`self.Draw Distance (0 - Infinity)`))
  (`PrimitiveComponent.SetCullDistance` (`self.StaticMeshComponent02`) (`self.Draw Distance (0 - Infinity)`))
  (`PrimitiveComponent.SetCullDistance` (`self.StaticMeshComponent04`) (`self.Draw Distance (0 - Infinity)`))
  (`PrimitiveComponent.SetCullDistance` (`self.StaticMeshComponent05`) (`self.Draw Distance (0 - Infinity)`))
  (`PrimitiveComponent.SetCullDistance` (`self.StaticMeshComponent03`) (`self.Draw Distance (0 - Infinity)`))
  (`PrimitiveComponent.SetCullDistance` (`self.StaticMeshComponent06`) (`self.Draw Distance (0 - Infinity)`))
  (`PrimitiveComponent.SetCullDistance` (`self.StaticMeshComponent07`) (`self.Draw Distance (0 - Infinity)`))
  (`PrimitiveComponent.SetCullDistance` (`self.StaticMeshComponent08`) (`self.Draw Distance (0 - Infinity)`))
  (`PrimitiveComponent.SetCullDistance` (`self.StaticMeshComponent0`) (`self.Draw Distance (0 - Infinity)`))
  (`PrimitiveComponent.SetCullDistance` (`self.StaticMeshComponent010`) (`self.Draw Distance (0 - Infinity)`))
  (`PrimitiveComponent.SetCullDistance` (`self.StaticMeshComponent011`) (`self.Draw Distance (0 - Infinity)`))
  (`PrimitiveComponent.SetCullDistance` (`self.StaticMeshComponent012`) (`self.Draw Distance (0 - Infinity)`))
  (`PrimitiveComponent.SetCullDistance` (`self.StaticMeshComponent013`) (`self.Draw Distance (0 - Infinity)`))
  (`PrimitiveComponent.SetCullDistance` (`self.StaticMeshComponent014`) (`self.Draw Distance (0 - Infinity)`))
  (`PrimitiveComponent.SetCullDistance` (`self.StaticMeshComponent015`) (`self.Draw Distance (0 - Infinity)`))
  (`PrimitiveComponent.SetCullDistance` (`self.StaticMeshComponent016`) (`self.Draw Distance (0 - Infinity)`))
  (`PrimitiveComponent.SetCullDistance` (`self.StaticMeshComponent017`) (`self.Draw Distance (0 - Infinity)`))
  (`PrimitiveComponent.SetCullDistance` (`self.StaticMeshComponent018`) (`self.Draw Distance (0 - Infinity)`)))