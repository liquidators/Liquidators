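; BP_FirstAidKit3_03 is a configurable first aid kit prop assembled from static meshes, with no active gameplay logic.
; Its Construction Script passes per-item visibility variables to OnOffMacro to show or hide seven contents: two pill items, painkillers, two bandages, an aid package and a syringe.
; It then applies one draw distance variable as the cull distance on all eight mesh components.
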(fn `UserConstructionScript`
  (`|ExecutionSequence`
    (:`then_0`
      ;[1 1 1] Visible
      (`/Game/First_Aid_Health_Kit/Blueprints/Macroses/On-Off_Macro.On/Off Macro` (`self.StaticMeshComponent07`) (`self.Pills 2 Visible`))
      (`/Game/First_Aid_Health_Kit/Blueprints/Macroses/On-Off_Macro.On/Off Macro` (`self.StaticMeshComponent01`) (`self.Painkiller Box Visible`))
      (`/Game/First_Aid_Health_Kit/Blueprints/Macroses/On-Off_Macro.On/Off Macro` (`self.StaticMeshComponent02`) (`self.Gauze Bandage Visible`))
      (`/Game/First_Aid_Health_Kit/Blueprints/Macroses/On-Off_Macro.On/Off Macro` (`self.StaticMeshComponent03`) (`self.Packed Bandage Visible`))
      (`/Game/First_Aid_Health_Kit/Blueprints/Macroses/On-Off_Macro.On/Off Macro` (`self.StaticMeshComponent04`) (`self.Aid Package Visible`))
      (`/Game/First_Aid_Health_Kit/Blueprints/Macroses/On-Off_Macro.On/Off Macro` (`self.StaticMeshComponent05`) (`self.Health Syringe Visible`))
      (`/Game/First_Aid_Health_Kit/Blueprints/Macroses/On-Off_Macro.On/Off Macro` (`self.StaticMeshComponent06`) (`self.Pills 1 Visible`)))
    (:`then_1`
      ;[1 1 1] Render distance
      (`PrimitiveComponent.SetCullDistance` (`self.StaticMeshComponent0`) (`self.Draw Distance (0 - Infinity)`))
      (`PrimitiveComponent.SetCullDistance` (`self.StaticMeshComponent01`) (`self.Draw Distance (0 - Infinity)`))
      (`PrimitiveComponent.SetCullDistance` (`self.StaticMeshComponent02`) (`self.Draw Distance (0 - Infinity)`))
      (`PrimitiveComponent.SetCullDistance` (`self.StaticMeshComponent03`) (`self.Draw Distance (0 - Infinity)`))
      (`PrimitiveComponent.SetCullDistance` (`self.StaticMeshComponent04`) (`self.Draw Distance (0 - Infinity)`))
      (`PrimitiveComponent.SetCullDistance` (`self.StaticMeshComponent05`) (`self.Draw Distance (0 - Infinity)`))
      (`PrimitiveComponent.SetCullDistance` (`self.StaticMeshComponent06`) (`self.Draw Distance (0 - Infinity)`))
      (`PrimitiveComponent.SetCullDistance` (`self.StaticMeshComponent07`) (`self.Draw Distance (0 - Infinity)`)))))