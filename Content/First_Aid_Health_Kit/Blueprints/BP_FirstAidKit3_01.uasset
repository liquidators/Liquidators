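; BP_FirstAidKit3_01 is a configurable first aid kit prop built from static mesh items such as aid packages, pots, syringes, bandages, painkillers and pills.
; The Construction Script toggles each item through OnOffMacro using its own visibility variable, leaving only StaticMeshComponent07 without a toggle.
; It then applies the shared DrawDistance0Infinity cull distance to all the meshes.
; The Event Graph holds no gameplay logic.
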(fn `UserConstructionScript`
  (`|ExecutionSequence`
    (:`then_0`
      ;[1 1 1] Visible
      (`/Game/First_Aid_Health_Kit/Blueprints/Macroses/On-Off_Macro.On/Off Macro` (`self.StaticMeshComponent0`) (`self.AidPackage 2 Visible`))
      (`/Game/First_Aid_Health_Kit/Blueprints/Macroses/On-Off_Macro.On/Off Macro` (`self.StaticMeshComponent01`) (`self.Aid Package 1 Visible`))
      (`/Game/First_Aid_Health_Kit/Blueprints/Macroses/On-Off_Macro.On/Off Macro` (`self.StaticMeshComponent02`) (`self.Aid Pot 1 Visible`))
      (`/Game/First_Aid_Health_Kit/Blueprints/Macroses/On-Off_Macro.On/Off Macro` (`self.StaticMeshComponent03`) (`self.Aid Pot 2 Visible`))
      (`/Game/First_Aid_Health_Kit/Blueprints/Macroses/On-Off_Macro.On/Off Macro` (`self.StaticMeshComponent04`) (`self.Energy Pot Visible`))
      (`/Game/First_Aid_Health_Kit/Blueprints/Macroses/On-Off_Macro.On/Off Macro` (`self.StaticMeshComponent05`) (`self.Energy Syringe 2 Visible`))
      (`/Game/First_Aid_Health_Kit/Blueprints/Macroses/On-Off_Macro.On/Off Macro` (`self.StaticMeshComponent06`) (`self.Energy Syringe 1 Visible`))
      (`/Game/First_Aid_Health_Kit/Blueprints/Macroses/On-Off_Macro.On/Off Macro` (`self.StaticMeshComponent08`) (`self.Gauze Bandage Visible`))
      (`/Game/First_Aid_Health_Kit/Blueprints/Macroses/On-Off_Macro.On/Off Macro` (`self.StaticMeshComponent09`) (`self.Gauze Bandage 2 Visible`))
      (`/Game/First_Aid_Health_Kit/Blueprints/Macroses/On-Off_Macro.On/Off Macro` (`self.StaticMeshComponent010`) (`self.Health Syringe Visible`))
      (`/Game/First_Aid_Health_Kit/Blueprints/Macroses/On-Off_Macro.On/Off Macro` (`self.StaticMeshComponent011`) (`self.Packed Bandage Visible`))
      (`/Game/First_Aid_Health_Kit/Blueprints/Macroses/On-Off_Macro.On/Off Macro` (`self.StaticMeshComponent012`) (`self.Painkiller 1 Visible`))
      (`/Game/First_Aid_Health_Kit/Blueprints/Macroses/On-Off_Macro.On/Off Macro` (`self.StaticMeshComponent013`) (`self.Painkiller 2 Visible`))
      (`/Game/First_Aid_Health_Kit/Blueprints/Macroses/On-Off_Macro.On/Off Macro` (`self.StaticMeshComponent014`) (`self.Pills 7 Visible`))
      (`/Game/First_Aid_Health_Kit/Blueprints/Macroses/On-Off_Macro.On/Off Macro` (`self.StaticMeshComponent015`) (`self.Pills 5 Visible`))
      (`/Game/First_Aid_Health_Kit/Blueprints/Macroses/On-Off_Macro.On/Off Macro` (`self.StaticMeshComponent016`) (`self.Pills 6 Visible`))
      (`/Game/First_Aid_Health_Kit/Blueprints/Macroses/On-Off_Macro.On/Off Macro` (`self.StaticMeshComponent017`) (`self.Pills 4 Visible`))
      (`/Game/First_Aid_Health_Kit/Blueprints/Macroses/On-Off_Macro.On/Off Macro` (`self.StaticMeshComponent018`) (`self.Pills 2 Visible`))
      (`/Game/First_Aid_Health_Kit/Blueprints/Macroses/On-Off_Macro.On/Off Macro` (`self.StaticMeshComponent019`) (`self.Pills 3 Visible`))
      (`/Game/First_Aid_Health_Kit/Blueprints/Macroses/On-Off_Macro.On/Off Macro` (`self.StaticMeshComponent020`) (`self.Pills 1 Visible`)))
    (:`then_1`
      ;[1 1 1] Render distance
      (`PrimitiveComponent.SetCullDistance` (`self.StaticMeshComponent09`) (`self.Draw Distance (0 - Infinity)`))
      (`PrimitiveComponent.SetCullDistance` (`self.StaticMeshComponent0`) (`self.Draw Distance (0 - Infinity)`))
      (`PrimitiveComponent.SetCullDistance` (`self.StaticMeshComponent01`) (`self.Draw Distance (0 - Infinity)`))
      (`PrimitiveComponent.SetCullDistance` (`self.StaticMeshComponent02`) (`self.Draw Distance (0 - Infinity)`))
      (`PrimitiveComponent.SetCullDistance` (`self.StaticMeshComponent03`) (`self.Draw Distance (0 - Infinity)`))
      (`PrimitiveComponent.SetCullDistance` (`self.StaticMeshComponent04`) (`self.Draw Distance (0 - Infinity)`))
      (`PrimitiveComponent.SetCullDistance` (`self.StaticMeshComponent05`) (`self.Draw Distance (0 - Infinity)`))
      (`PrimitiveComponent.SetCullDistance` (`self.StaticMeshComponent06`) (`self.Draw Distance (0 - Infinity)`))
      (`PrimitiveComponent.SetCullDistance` (`self.StaticMeshComponent07`) (`self.Draw Distance (0 - Infinity)`))
      (`PrimitiveComponent.SetCullDistance` (`self.StaticMeshComponent08`) (`self.Draw Distance (0 - Infinity)`))
      (`PrimitiveComponent.SetCullDistance` (`self.StaticMeshComponent020`) (`self.Draw Distance (0 - Infinity)`))
      (`PrimitiveComponent.SetCullDistance` (`self.StaticMeshComponent010`) (`self.Draw Distance (0 - Infinity)`))
      (`PrimitiveComponent.SetCullDistance` (`self.StaticMeshComponent011`) (`self.Draw Distance (0 - Infinity)`))
      (`PrimitiveComponent.SetCullDistance` (`self.StaticMeshComponent012`) (`self.Draw Distance (0 - Infinity)`))
      (`PrimitiveComponent.SetCullDistance` (`self.StaticMeshComponent013`) (`self.Draw Distance (0 - Infinity)`))
      (`PrimitiveComponent.SetCullDistance` (`self.StaticMeshComponent014`) (`self.Draw Distance (0 - Infinity)`))
      (`PrimitiveComponent.SetCullDistance` (`self.StaticMeshComponent015`) (`self.Draw Distance (0 - Infinity)`))
      (`PrimitiveComponent.SetCullDistance` (`self.StaticMeshComponent016`) (`self.Draw Distance (0 - Infinity)`))
      (`PrimitiveComponent.SetCullDistance` (`self.StaticMeshComponent017`) (`self.Draw Distance (0 - Infinity)`))
      (`PrimitiveComponent.SetCullDistance` (`self.StaticMeshComponent018`) (`self.Draw Distance (0 - Infinity)`))
      (`PrimitiveComponent.SetCullDistance` (`self.StaticMeshComponent019`) (`self.Draw Distance (0 - Infinity)`)))))