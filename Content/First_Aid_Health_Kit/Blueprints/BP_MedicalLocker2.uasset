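; BP_MedicalLocker2 is a configurable medical locker prop, set up entirely in the construction script with no active event logic.
; It toggles the visibility of the cap mesh and applies a negated yaw offset to it from exposed cap settings.
; A shared render-distance value sets the cull distance on both static mesh components.
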(fn `UserConstructionScript`
  ;[1 1 1] Cap Visible
  (`/Game/First_Aid_Health_Kit/Blueprints/Macroses/On-Off_Macro.On/Off Macro` (`self.StaticMeshComponent0`) (`self.Cap Visible`))
  ;[1 1 1] Cap rotation
  (`SceneComponent.K2_AddRelativeRotation` (`self.StaticMeshComponent0`) (`KismetMathLibrary.MakeRotator` 0.0 0.0 (* (`self.Cap Rotation`) -1.0)) false false)
  ;[1 1 1] Render distance
  (`PrimitiveComponent.SetCullDistance` (`self.StaticMeshComponent01`) (`self.Draw Distance (0 - Infinity)`))
  (`PrimitiveComponent.SetCullDistance` (`self.StaticMeshComponent0`) (`self.Draw Distance (0 - Infinity)`)))