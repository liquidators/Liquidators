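; BP_Room1Sound is a trigger box that plays boss English audio cues, apparently for Room 1, chosen by the current player character.
; On any overlap with the box, it reads the player's CurrentCharacterName and plays the matching 2D cue for Alexei, Valeri or Boris.
; A separate boolean per character makes each cue play only once.
; The overlapping actor itself is not checked.
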(event `self.Box.OnComponentBeginOverlap`
  (params (OverlappedComponent :type "PrimitiveComponent Object Reference") (OtherActor :type "Actor Object Reference") (OtherComp :type "PrimitiveComponent Object Reference") (OtherBodyIndex :type Integer) (bFromSweep :type Boolean) (SweepResult :type "HitResult Structure (by ref)"))
  (bind _asmaster (`/Game/HorrorEngine/Blueprints/Core/HorrorEngineFunctions.GetPlayer`))
  (bind _currentcharactername (`/Game/HorrorEngine/HorrorEngine.CurrentCharacterName` _asmaster))
  (if (`KismetStringLibrary.EqualEqual_StrStr` _currentcharactername "Alexei")
    (if (not (`self.isPlayedAlexei`))
      (`GameplayStatics.PlaySound2D` "/Game/Sounds5/Boss/Boss_English_3_1Boss_English_Cue.Boss_English_3_1Boss_English_Cue" 1.0 1.0 0.0 null null)
      (set `self.isPlayedAlexei` true))
    (elif (`KismetStringLibrary.EqualEqual_StrStr` _currentcharactername "Valeri")
      (if (not (`self.isPlayedValeri`))
        (`GameplayStatics.PlaySound2D` "/Game/Sounds5/Boss/Boss_English_15Boss_English_Cue.Boss_English_15Boss_English_Cue" 1.0 1.0 0.0 null null)
        (set `self.isPlayedValeri` true))
      (elif (`KismetStringLibrary.EqualEqual_StrStr` _currentcharactername "Boris")
        (if (not (`self.isPlayedBoris`))
          (`GameplayStatics.PlaySound2D` "/Game/Sounds5/Boss/Boss_English_18_1Boss_English_Cue.Boss_English_18_1Boss_English_Cue" 1.0 1.0 0.0 null null)
          (set `self.isPlayedBoris` true))))))

(fn `UserConstructionScript`)