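; Trigger actor that plays a one-time English Boss voice cue for Room 2, chosen by the current player character.
; On Box overlap, it checks the player's character name (Alexei, Valeri or Boris) without filtering the overlapping actor.
; The 2D cue plays only if both that character's flag on BP_RoomSoundManager and the local IsPlayedRoom2 flag are unset.
; Playing sets both flags, blocking repeats.
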(event `self.Box.OnComponentBeginOverlap`
  (params (OverlappedComponent :type "PrimitiveComponent Object Reference") (OtherActor :type "Actor Object Reference") (OtherComp :type "PrimitiveComponent Object Reference") (OtherBodyIndex :type Integer) (bFromSweep :type Boolean) (SweepResult :type "HitResult Structure (by ref)"))
  (bind _asmaster (`/Game/HorrorEngine/Blueprints/Core/HorrorEngineFunctions.GetPlayer`))
  (bind _currentcharactername (`/Game/HorrorEngine/HorrorEngine.CurrentCharacterName` _asmaster))
  (if (`KismetStringLibrary.EqualEqual_StrStr` _currentcharactername "Alexei")
    (bind _returnvalue (`GameplayStatics.GetActorOfClass` "/Game/Sounds5/Boss/BP_RoomSoundManager.BP_RoomSoundManager_C"))
    (if (`/Game/Sounds5/Boss/BP_RoomSoundManager.isPlayedForAlexei` _returnvalue)
      _
      (elif (not (`self.isPlayedRoom2`))
        (`GameplayStatics.PlaySound2D` "/Game/Sounds5/Boss/Boss_English_3_1Boss_English_Cue.Boss_English_3_1Boss_English_Cue" 1.0 1.0 0.0 null null)
        (set `/Game/Sounds5/Boss/BP_RoomSoundManager.isPlayedForAlexei` true _returnvalue)
        (set `self.isPlayedRoom2` true)))
    (elif (`KismetStringLibrary.EqualEqual_StrStr` _currentcharactername "Valeri")
      (bind _returnvalue_2 (`GameplayStatics.GetActorOfClass` "/Game/Sounds5/Boss/BP_RoomSoundManager.BP_RoomSoundManager_C"))
      (if (`/Game/Sounds5/Boss/BP_RoomSoundManager.isPlayedForValeri` _returnvalue_2)
        _
        (elif (not (`self.isPlayedRoom2`))
          (`GameplayStatics.PlaySound2D` "/Game/Sounds5/Boss/Boss_English_15Boss_English_Cue.Boss_English_15Boss_English_Cue" 1.0 1.0 0.0 null null)
          (set `/Game/Sounds5/Boss/BP_RoomSoundManager.isPlayedForValeri` true _returnvalue_2)
          (set `self.isPlayedRoom2` true)))
      (elif (`KismetStringLibrary.EqualEqual_StrStr` _currentcharactername "Boris")
        (bind _returnvalue_3 (`GameplayStatics.GetActorOfClass` "/Game/Sounds5/Boss/BP_RoomSoundManager.BP_RoomSoundManager_C"))
        (if (`/Game/Sounds5/Boss/BP_RoomSoundManager.isPlayedForBoris` _returnvalue_3)
          _
          (elif (not (`self.isPlayedRoom2`))
            (`GameplayStatics.PlaySound2D` "/Game/Sounds5/Boss/Boss_English_18_1Boss_English_Cue.Boss_English_18_1Boss_English_Cue" 1.0 1.0 0.0 null null)
            (set `/Game/Sounds5/Boss/BP_RoomSoundManager.isPlayedForBoris` true _returnvalue_3)
            (set `self.isPlayedRoom2` true)))))))

(fn `UserConstructionScript`)