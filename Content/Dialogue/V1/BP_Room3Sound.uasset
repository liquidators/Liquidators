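; Trigger volume for Room 3 that plays a 2D radio dialogue cue specific to the current player character (Alexei, Valeri or Boris).
; On box overlap it checks that character's flag in BP_RoomSoundManager and its own IsPlayedRoom3, then sets both after playing.
; As a result the room plays only once, and only for a character not yet marked in the manager.
; The spawned audio is kept in RadioSound so StopRadioSound can cut it off.
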(event `self.Box.OnComponentBeginOverlap`
  (params (OverlappedComponent :type "PrimitiveComponent Object Reference") (OtherActor :type "Actor Object Reference") (OtherComp :type "PrimitiveComponent Object Reference") (OtherBodyIndex :type Integer) (bFromSweep :type Boolean) (SweepResult :type "HitResult Structure (by ref)"))
  (bind _asmaster (`/Game/HorrorEngine/Blueprints/Core/HorrorEngineFunctions.GetPlayer`))
  (bind _currentcharactername (`/Game/HorrorEngine/HorrorEngine.CurrentCharacterName` _asmaster))
  (if (`KismetStringLibrary.EqualEqual_StrStr` _currentcharactername "Alexei")
    (bind _returnvalue (`GameplayStatics.GetActorOfClass` "/Game/Dialogue/V1/BP_RoomSoundManager.BP_RoomSoundManager_C"))
    (if (`/Game/Dialogue/V1/BP_RoomSoundManager.isPlayedForAlexei` _returnvalue)
      _
      (elif (not (`self.isPlayedRoom3`))
        (bind _returnvalue_2 (`GameplayStatics.SpawnSound2D` "/Game/Sounds6/bosswifev10_Cue.bosswifev10_Cue" 1.0 1.0 0.0 null))
        (set `self.Radio Sound` _returnvalue_2)
        (set `/Game/Dialogue/V1/BP_RoomSoundManager.isPlayedForAlexei` true _returnvalue)
        (set `self.isPlayedRoom3` true)))
    (elif (`KismetStringLibrary.EqualEqual_StrStr` _currentcharactername "Valeri")
      (bind _returnvalue_3 (`GameplayStatics.GetActorOfClass` "/Game/Dialogue/V1/BP_RoomSoundManager.BP_RoomSoundManager_C"))
      (if (`/Game/Dialogue/V1/BP_RoomSoundManager.isPlayedForValeri` _returnvalue_3)
        _
        (elif (not (`self.isPlayedRoom3`))
          (bind _returnvalue_4 (`GameplayStatics.SpawnSound2D` "/Game/Dialogue/V1/boss_father__maybe_needs_fix__Cue.boss_father__maybe_needs_fix__Cue" 1.0 1.0 0.0 null))
          (set `self.Radio Sound` _returnvalue_4)
          (set `/Game/Dialogue/V1/BP_RoomSoundManager.isPlayedForValeri` true _returnvalue_3)
          (set `self.isPlayedRoom3` true)))
      (elif (`KismetStringLibrary.EqualEqual_StrStr` _currentcharactername "Boris")
        (bind _returnvalue_5 (`GameplayStatics.GetActorOfClass` "/Game/Dialogue/V1/BP_RoomSoundManager.BP_RoomSoundManager_C"))
        (if (`/Game/Dialogue/V1/BP_RoomSoundManager.isPlayedForBoris` _returnvalue_5)
          _
          (elif (not (`self.isPlayedRoom3`))
            (bind _returnvalue_6 (`GameplayStatics.SpawnSound2D` "/Game/Dialogue/V1/Boris_Family_Cue.Boris_Family_Cue" 1.0 1.0 0.0 null))
            (set `self.Radio Sound` _returnvalue_6)
            (set `/Game/Dialogue/V1/BP_RoomSoundManager.isPlayedForBoris` true _returnvalue_5)
            (set `self.isPlayedRoom3` true)))))))

(event `Stop Radio Sound`
  (bind _radio_sound (`self.Radio Sound`))
  (`/Engine/EditorBlueprintResources/StandardMacros.IsValid` _radio_sound
    (:`Is Valid`
      (`AudioComponent.Stop` _radio_sound))))

(fn `UserConstructionScript`)