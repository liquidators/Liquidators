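; BP_PoisonToxicGooLake is a toxic goo lake actor with a tinted skeletal mesh and configurable bubble particles.
; The construction script applies the color to the mesh materials, adds the bubble particle system with itself as actor parameter, and runs SetupParticle.
; SetupParticle pushes enable state, half-intensity color, spawn amount, randomized lifetime and size, and Z velocity to the particles.
; Tick reruns SetupParticle, re-rolling the random values every frame.
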(event `self.ReceiveTick`
  (params (DeltaSeconds :type "Float (single-precision)"))
  ;[1 1 1] Runtime Setup Particle
  (`self.Setup Particle`))

(fn `Setup Particle`
  ;[1 1 1] Check if Valid
  (`/Engine/EditorBlueprintResources/StandardMacros.IsValid` (`self.P_Bubbles`)
    (:`Is Valid`
      (`|ExecutionSequence`
        (:`then_0`
          ;[1 1 1] Toggle Enabled
          (`ParticleSystemComponent.SetEmitterEnable` (`self.P_Bubbles`) "Bubbles" (`self.Enable Bubbles`)))
        (:`then_1`
          ;[1 1 1] Set Bubble Color
          (`ParticleSystemComponent.SetColorParameter` (`self.P_Bubbles`) "Color" (* (`self.Color`) 0.5)))
        (:`then_2`
          ;[1 1 1] Set Bubbles Spawn Amount
          (`ParticleSystemComponent.SetFloatParameter` (`self.P_Bubbles`) "Spawn" (`self.Spawn Amount`)))
        (:`then_3`
          ;[1 1 1] Set Bubbles Lifetime Min and Max
          (`ParticleSystemComponent.SetFloatParameter` (`self.P_Bubbles`) "Lifetime" (`KismetMathLibrary.RandomFloatInRange` (`self.Lifetime Min`) (`self.Lifetime Max`))))
        (:`then_4`
          ;[1 1 1] Set Bubble Size Min and Max
          (`ParticleSystemComponent.SetFloatParameter` (`self.P_Bubbles`) "Size" (`KismetMathLibrary.RandomFloatInRange` (`self.Size Min`) (`self.Size Max`))))
        (:`then_5`
          ;[1 1 1] Set Bubble Velocity Min and Max
          (`ParticleSystemComponent.SetVectorParameter` (`self.P_Bubbles`) "Velocity" (`KismetMathLibrary.MakeVector` 0.0 0.0 (`self.Z Velocity`))))))))

(fn `UserConstructionScript`
  ;[1 1 1] Setup Color on Construct
  (`MeshComponent.SetVectorParameterValueOnMaterials` (`self.SkeletalMesh`) "Color" (`KismetMathLibrary.Conv_LinearColorToVector` (`self.Color`)))
  ;[1 1 1] Add Bubble Particle Component, Set Actor to self, then call Setup Particle Function
  (bind _returnvalue (`AddComponent|NODE_AddParticleSystemComponent-0`))
  (bind _output_get (set `self.P_Bubbles` _returnvalue))
  (`ParticleSystemComponent.SetActorParameter` _output_get "Actor" self)
  (`self.Setup Particle`))