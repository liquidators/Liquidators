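; Hanging industrial spot light prop that can be switched on or off, flicker and optionally be destroyed by damage.
; The construction script and every Tick apply the on/off intensity, color and emissive settings to the light and mesh material.
; When flickering, Tick recreates the dynamic material and plays a timeline that modulates intensity and emissive brightness.
; The first damage to a destroyable light triggers sparks, swaps to an opaque material, hides the light and stops flicker updates.
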(event `self.ReceiveAnyDamage`
  (params (Damage :type "Float (single-precision)") (DamageType :type "DamageType Object Reference") (InstigatedBy :type "Controller Object Reference") (DamageCauser :type "Actor Object Reference"))
  ;[1 1 1] Damage
  (if (`self.Destroyable_?`)
    (`/Engine/EditorBlueprintResources/StandardMacros.DoOnce` false
      (:`Completed`
        (`AudioComponent.Play` (`self.Reflections_SparkTail_Cue`) 0.0)
        (`ActorComponent.Activate` (`self.P_SparkBurst`) false)
        (`PrimitiveComponent.CreateDynamicMaterialInstance` (`self.SkeletalMesh`) 1 "/Game/RaP_industrial_lights_and_switches/Lights/Materials/Opaque_Inst.Opaque_Inst")
        (`SceneComponent.SetVisibility` (`self.SpotLight`) false false)
        (set `self.Destroyed_?` true)))))

(event `self.ReceiveTick`
  (params (DeltaSeconds :type "Float (single-precision)"))
  (bind _spotlight (`self.SpotLight`))
  (`|ExecutionSequence`
    (:`then_0`
      (`self.ON/OFF` _spotlight _spotlight))
    (:`then_1`
      (if (not (`self.Destroyed_?`))
        ;[1 1 1] Flicker
        (if (`self.ON/OFF_?`)
          (if (`self.Flicker_?`)
            (bind _returnvalue (`PrimitiveComponent.CreateDynamicMaterialInstance` (`self.SkeletalMesh`) 1 "/Game/RaP_industrial_lights_and_switches/Lights/Materials/Emissive_Inst.Emissive_Inst"))
            (bind _output_get (set `self.Emissive_brightness` _returnvalue))
            (set `self.emissive_color` _output_get)
            (`LightComponent.SetIntensity` (`self.SpotLight`) 0.0)
            (bind (_direction _newtrack_0) (`Timeline|Timeline_0`) ; Timeline curve is used to make the light and material emissive flicker
              (:`Update`
                (`MaterialInstanceDynamic.SetScalarParameterValue` (`self.Emissive_brightness`) "Emissive_brightness" (+ (* _newtrack_0 0.1) 0.001))
                (`LightComponent.SetIntensity` (`self.SpotLight`) (* 1500.0 _newtrack_0))
                (`MaterialInstanceDynamic.SetVectorParameterValue` (`self.emissive_color`) "emissive_color" (`self.Color_Material_Emissive`))))))))))

(fn `ON/OFF`
  (params (self2 :type "LightComponent Object Reference") (self3 :type "LightComponent Object Reference"))
  (bind _spotlight (`self.SpotLight`))
  (if (`self.ON/OFF_?`)
    (`LightComponent.SetIntensity` self3 (`self.Brightness_Light`))
    (`LightComponent.SetLightColor` self2 (`self.Color_Light`) true)
    (`MaterialInstanceDynamic.SetVectorParameterValue` (`self.emissive_color`) "emissive_color" (`self.Color_Material_Emissive`))
    (`MaterialInstanceDynamic.SetScalarParameterValue` (`self.Emissive_brightness`) "Emissive_brightness" (`self.Brightness_Emissive`))
    (else
      (`LightComponent.SetIntensity` _spotlight 0.0)
      (`LightComponent.SetLightColor` :`self` _spotlight)
      (`MaterialInstanceDynamic.SetVectorParameterValue` (`self.Emissive_Color`) "emissive_color" (struct :`R` 0.509804 :`G` 0.509804 :`B` 0.509804 :`A` 1.0))
      (`MaterialInstanceDynamic.SetScalarParameterValue` (`self.Emissive_brightness`) "Emissive_brightness" 0.05)))
  (return))

(fn `UserConstructionScript`
  (bind _spotlight (`self.SpotLight`))
  (bind _returnvalue (`PrimitiveComponent.CreateDynamicMaterialInstance` (`self.SkeletalMesh`) 1 "/Game/RaP_industrial_lights_and_switches/Lights/Materials/Emissive_Inst.Emissive_Inst"))
  (bind _output_get (set `self.Opacity` _returnvalue))
  (bind _output_get_2 (set `self.Emissive_Brightness` _output_get))
  (set `self.emissive_color` _output_get_2)
  (`self.ON/OFF` _spotlight _spotlight))