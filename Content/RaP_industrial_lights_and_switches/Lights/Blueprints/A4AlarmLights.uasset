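; A4AlarmLights is an alarm light prop with a rotating mesh, a spotlight and an emissive glow.
; While ActivateAlarm is set, Tick spins the mesh, shows the spotlight and raises emissive brightness through a dynamic material created in the construction script; otherwise it hides and dims them.
; If Destroyable, any damage plays a spark sound and particle burst, destroys both meshes and switches the alarm off.
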(event `self.ReceiveAnyDamage`
  (params (Damage :type "Float (single-precision)") (DamageType :type "DamageType Object Reference") (InstigatedBy :type "Controller Object Reference") (DamageCauser :type "Actor Object Reference"))
  (if (`self.Destroyable_?`)
    (`AudioComponent.Play` (`self.Reflections_Spark_Cue`) 0.0)
    (`ActorComponent.K2_DestroyComponent` (`self.StaticMesh2`))
    (`ActorComponent.K2_DestroyComponent` (`self.StaticMesh1`))
    (`ActorComponent.Activate` (`self.P_SparkBurst`) false)
    (set `self.Activate_Alarm` false)
    (`SceneComponent.SetVisibility` (`self.SpotLight`) false false :!label _label)
    (`MaterialInstanceDynamic.SetScalarParameterValue` (`self.Emissive_brightness`) "Emissive_brightness" 0.1)))

(event `self.ReceiveTick`
  (params (DeltaSeconds :type "Float (single-precision)"))
  (if (`self.Activate_Alarm`)
    (`SceneComponent.K2_AddLocalRotation` (`self.StaticMesh1`) (struct :`Yaw` 2.0) false false)
    (`SceneComponent.SetVisibility` (`self.SpotLight`) true false)
    (`MaterialInstanceDynamic.SetScalarParameterValue` (`self.Emissive_brightness`) "Emissive_brightness" 8.0)
    (else
      (goto _label))))

(fn `UserConstructionScript`
  (bind _returnvalue (`PrimitiveComponent.CreateDynamicMaterialInstance` (`self.StaticMesh1`) 1 "/Game/RaP_industrial_lights_and_switches/Lights/Materials/Emissive_Alarm_INST.Emissive_Alarm_INST" "None"))
  (set `self.Emissive_brightness` _returnvalue))