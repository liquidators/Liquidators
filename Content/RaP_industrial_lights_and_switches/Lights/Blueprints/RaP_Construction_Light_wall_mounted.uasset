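; A wall-mounted construction light prop that can be broken by damage and optionally simulates physics.
; When Damagable, the first damage event plays a spark sound, fires a particle burst, destroys the spotlight and swaps a mesh material slot to an opaque dynamic instance.
; A DoOnce limits the break to a single time, and the construction script enables mesh physics when the Physics flag is set.
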(event `self.ReceiveAnyDamage`
  (params (Damage :type "Float (single-precision)") (DamageType :type "DamageType Object Reference") (InstigatedBy :type "Controller Object Reference") (DamageCauser :type "Actor Object Reference"))
  (if (`self.Damagable_?`)
    (`/Engine/EditorBlueprintResources/StandardMacros.DoOnce` false
      (:`Completed`
        (`AudioComponent.Play` (`self.Reflections_Spark_Cue`) 0.0)
        (`ActorComponent.Activate` (`self.P_SparkBurst`) false)
        (`ActorComponent.K2_DestroyComponent` (`self.SpotLight`))
        (`PrimitiveComponent.CreateDynamicMaterialInstance` (`self.StaticMesh`) 1 "/Game/RaP_industrial_lights_and_switches/Lights/Materials/Opaque_Inst.Opaque_Inst" "None")))))

(fn `UserConstructionScript`
  (if (`self.Physics_?`)
    (`PrimitiveComponent.SetSimulatePhysics` (`self.StaticMesh`) true)))