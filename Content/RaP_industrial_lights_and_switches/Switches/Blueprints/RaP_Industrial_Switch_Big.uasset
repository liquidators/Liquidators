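; Big industrial wall switch actor that the player flips with the Use input while inside its trigger volume.
; Overlap events set an in-range flag and handle enabling and disabling input.
; Each press plays a sound cue and alternates a timeline forward or backward through a FlipFlop, pitching the handle.
; The timeline disables the switch's input while it moves and re-enables it when finished, blocking presses mid-animation.
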(event `InputAction|Use` :consume false
  (params (Key :type "Key Structure" :default "AnyKey"))
  (:`Pressed`
    (if (`self.Switch_Big_?`)
      (`AudioComponent.Play` (`self.Switch_Big_Cue`) 0.0)
      (`/Engine/EditorBlueprintResources/StandardMacros.FlipFlop`
        (:`A`
          (bind (_direction _rotation) (`Timeline|Timeline_0` :!label _label)
            (:`Update`
              (`SceneComponent.K2_SetRelativeRotation` (`self.Handle`) (`KismetMathLibrary.MakeRotator` 0.0 _rotation) false false)
              (`self.DisableInput` (`GameplayStatics.GetPlayerController` 0)))
            (:`Finished`
              (`self.EnableInput` (`GameplayStatics.GetPlayerController` 0)))))
        (:`B`
          (goto _label :!via `Reverse`))))))

(event `self.Trigger.OnComponentBeginOverlap`
  (params (OtherActor :type "Actor Object Reference") (OtherComp :type "PrimitiveComponent Object Reference") (OtherBodyIndex :type Integer) (bFromSweep :type Boolean) (SweepResult :type "HitResult Structure (by ref)"))
  (set `self.Switch_Big_?` true)
  (`self.EnableInput` (`GameplayStatics.GetPlayerController` 0)))

(event `self.Trigger.OnComponentEndOverlap`
  (params (OtherActor :type "Actor Object Reference") (OtherComp :type "PrimitiveComponent Object Reference") (OtherBodyIndex :type Integer))
  (set `self.Switch_Big_?` false)
  (`self.DisableInput` (`GameplayStatics.GetPlayerController` 0) null))

(fn `UserConstructionScript`)