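; Small industrial switch Blueprint with a button that animates and plays a sound when used.
; Any Trigger overlap sets a flag and enables input on the switch; leaving clears it and calls DisableInput on the player controller, not the switch.
; While flagged, Use plays the cue and restarts a timeline that moves the button along local Y.
; A FlipFlop play/reverse branch is unconnected, and the switch controls nothing else.
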(event `InputAction|Use` :consume false
  (params (Key :type "Key Structure" :default "AnyKey"))
  (:`Pressed`
    (if (`self.Trigger_?`)
      (`AudioComponent.Play` (`self.Switch_Small_Cue`) 0.0)
      (bind (_direction _newtrack_0) (`Timeline|Timeline_0` :!via `PlayFromStart`)
        (:`Update`
          (`SceneComponent.K2_SetRelativeLocation` (`self.Button`) (`KismetMathLibrary.MakeVector` 0.0 _newtrack_0) false false))))))

(event `self.Trigger.OnComponentBeginOverlap`
  (params (OtherActor :type "Actor Object Reference") (OtherComp :type "PrimitiveComponent Object Reference") (OtherBodyIndex :type Integer) (bFromSweep :type Boolean) (SweepResult :type "HitResult Structure (by ref)"))
  (set `self.Trigger_?` true)
  (`self.EnableInput` (`GameplayStatics.GetPlayerController` 0)))

(event `self.Trigger.OnComponentEndOverlap`
  (params (OtherActor :type "Actor Object Reference") (OtherComp :type "PrimitiveComponent Object Reference") (OtherBodyIndex :type Integer))
  (set `self.Trigger_?` false)
  (`self.DisableInput` (`GameplayStatics.GetPlayerController` 0) null))

(fn `UserConstructionScript`)