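; Interactive medium industrial switch with a hinged lid and a flippable handle, operated with the Use input.
; Two trigger volumes enable player input on overlap and set the flags that gate lid and handle.
; A DoOnce timeline swings the lid open with sound, then a FlipFlop alternates the handle timeline forward and back, briefly locking input during the forward throw.
; Lid-closing logic is present but unconnected.
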(event `InputAction|Use` :consume false
  (params (Key :type "Key Structure" :default "AnyKey"))
  (:`Pressed`
    (`|ExecutionSequence`
      (:`then_0`
        (if (and (not (`self.Door_Open_?`)) (`self.Trigger`))
          (`/Engine/EditorBlueprintResources/StandardMacros.DoOnce` false
            (:`Completed`
              (`AudioComponent.Play` (`self.Door_Open_Cue`) 0.0)
              (bind (_direction _newtrack_0) (`Timeline|Lit`)
                (:`Update`
                  (`SceneComponent.K2_SetRelativeRotation` (`self.Switch_LIt`) (`KismetMathLibrary.MakeRotator` 0.0 0.0 _newtrack_0) false false))
                (:`Finished`
                  (set `self.Door_Open_?` true)
                  (set `self.Switch_?` true)))))))
      (:`then_1`
        (if (and (`self.Door_Open_?`) (`self.Switch_?`))
          (`AudioComponent.Play` (`self.Switch_Handle_Cue`) 0.0)
          (`/Engine/EditorBlueprintResources/StandardMacros.FlipFlop`
            (:`A`
              (bind (_direction_2 _newtrack_0_2) (`Timeline|Timeline_1` :!label _label)
                (:`Update`
                  (`SceneComponent.K2_SetRelativeRotation` (`self.Switch`) (`KismetMathLibrary.MakeRotator` _newtrack_0_2) false false)
                  (`self.DisableInput` (`GameplayStatics.GetPlayerController` 0))
                  (`KismetSystemLibrary.RetriggerableDelay` 0.5)
                  (`self.EnableInput` (`GameplayStatics.GetPlayerController` 0)))))
            (:`B`
              (goto _label :!via `Reverse`))))))))

(event `self.Lit_Trigger.OnComponentBeginOverlap`
  (params (OtherActor :type "Actor Object Reference") (OtherComp :type "PrimitiveComponent Object Reference") (OtherBodyIndex :type Integer) (bFromSweep :type Boolean) (SweepResult :type "HitResult Structure (by ref)"))
  (set `self.Trigger` true)
  (`self.EnableInput` (`GameplayStatics.GetPlayerController` 0) :!label _label_2))

(event `self.Lit_Trigger.OnComponentEndOverlap`
  (params (OtherActor :type "Actor Object Reference") (OtherComp :type "PrimitiveComponent Object Reference") (OtherBodyIndex :type Integer))
  (set `self.Trigger` false)
  (`self.DisableInput` (`GameplayStatics.GetPlayerController` 0) null :!label _label_3))

(event `self.Switch_Trigger.OnComponentBeginOverlap`
  (params (OtherActor :type "Actor Object Reference") (OtherComp :type "PrimitiveComponent Object Reference") (OtherBodyIndex :type Integer) (bFromSweep :type Boolean) (SweepResult :type "HitResult Structure (by ref)"))
  (set `self.Switch_?` true)
  (goto _label_2))

(event `self.Switch_Trigger.OnComponentEndOverlap`
  (params (OtherActor :type "Actor Object Reference") (OtherComp :type "PrimitiveComponent Object Reference") (OtherBodyIndex :type Integer))
  (set `self.Switch_?` false)
  (goto _label_3))

(fn `UserConstructionScript`)