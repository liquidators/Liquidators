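; Wall-mounted warning light prop with a static mesh and a point light that is switched visible on BeginPlay.
; It hooks into the player's HESaveGameComponent asset cache; restoring reads OnOff and shows the light when true, but never hides it.
; The save builder leaves its name and OnOff struct node unused.
; Despite the spinning-reflector name, Tick is empty and the mesh rotation node is disconnected, so nothing spins.
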(event `self.ReceiveBeginPlay`
  (`SceneComponent.SetVisibility` (`self.PointLight`) true false))

(event `self.ReceiveTick`
  (params (DeltaSeconds :type "Float (single-precision)")))

(event `/Game/HorrorEngine/Blueprints/Core/HorrorEngineInterface.CollectSaveData`
  (bind _asmaster (`/Game/HorrorEngine/Blueprints/Core/HorrorEngineFunctions.GetPlayer`))
  (`KismetArrayLibrary.Array_Add` (`/Game/HorrorEngine/Blueprints/Core/HE_SaveGameComponent.AssetCache` (`/Game/HorrorEngine/HorrorEngine.HE_SaveGameComponent` _asmaster)) (make `/Game/HorrorEngine/Blueprints/Structures/SaveStructures/AssetsSave` (`KismetSystemLibrary.GetObjectName` self) (`self.On / Off`) false false false 0.0 0.0 0 "+00000000.00:00:00.000000000" "NewEnumerator0" (struct :`Actor` "NewEnumerator0" :`MeshSettings` (struct) :`InspectionSettings` (struct :`InspectionPivotLocation` (0.0 0.0 0.0) :`Takeable` true :`InspectionAnimation` true :`InspectionAnimationSpeedSec` 0.5 :`InspectionBeginRotation` (struct) :`InspectionBeginScale` 1.0 :`MinZoomScale` 1.0 :`MaxZoomScale` 2.0 :`RotationSpeed` 2.5 :`SlideSpeed` 1.0 :`MaxSlideValue` 10.0 :`ItemName` "NSLOCTEXT(\"[49A72E6F4EE21BDF79E865A7D2D59EBD]\", \"D52DCAA54F270EC455423DBE9B198F9C\", \"Item Name\")" :`ItemInformation` "NSLOCTEXT(\"[49A72E6F4EE21BDF79E865A7D2D59EBD]\", \"5506EEEB4B3086BCE24AAEA130A9B040\", \"Item Information\")" :`ReadingText` "NSLOCTEXT(\"[49A72E6F4EE21BDF79E865A7D2D59EBD]\", \"97AB22C44C772F4155E717A129396C7A\", \"Reading Text\")" :`TakeButton` (struct :`ButtonText` "NSLOCTEXT(\"[49A72E6F4EE21BDF79E865A7D2D59EBD]\", \"F4BACD094FCA210355090BB30FF5137D\", \"Take\")") :`ExamineButton` (struct :`ButtonText` "NSLOCTEXT(\"[49A72E6F4EE21BDF79E865A7D2D59EBD]\", \"A1FFA795468AD4E35B61A38999C9B934\", \"Examine\")") :`ZoomSlideButton` (struct :`ButtonText` "NSLOCTEXT(\"[49A72E6F4EE21BDF79E865A7D2D59EBD]\", \"05D304D247F2B1784408B39A20F93E32\", \"Zoom/Slide\")") :`DismissButton` (struct :`ButtonText` "NSLOCTEXT(\"[49A72E6F4EE21BDF79E865A7D2D59EBD]\", \"BCC6174D4F9D2E593F4FA094CE09305E\", \"Dismiss\")")) :`InventorySettings` (struct :`StorageType` "NewEnumerator3" :`NumberofItemstoAddInventory` 1 :`Interactable` true :`InteractionButton` (struct :`ButtonText` "NSLOCTEXT(\"[49A72E6F4EE21BDF79E865A7D2D59EBD]\", \"CF9E4D9B4D5BD2B3AAA33CB892D31E06\", \"Use\")") :`SwitchButton` (struct :`ButtonText` "NSLOCTEXT(\"[49A72E6F4EE21BDF79E865A7D2D59EBD]\", \"2810A7174288D9A63DD308BE8C478E16\", \"Switch\")") :`ZoomSlideButton` (struct :`ButtonText` "NSLOCTEXT(\"[49A72E6F4EE21BDF79E865A7D2D59EBD]\", \"ACF25EAB409323220385A2BA43B5C82F\", \"Zoom/Slide\")") :`CloseInventoryButton` (struct :`ButtonText` "NSLOCTEXT(\"[49A72E6F4EE21BDF79E865A7D2D59EBD]\", \"333F06AF4CFF638D7889D0B7C0CF3C43\", \"Close\")")) :`Pistol_MeshSettingsTop` (struct) :`Vhs_CurrentTime` "+00000000.00:00:00.000000000"))))

(event `/Game/HorrorEngine/Blueprints/Core/HorrorEngineInterface.RestoreSaveData`
  (params (AssetSave :type "/Game/HorrorEngine/Blueprints/Structures/SaveStructures/AssetsSave Structure"))
  (set `self.On / Off` (`.BooleanSlot01_63_ED79FB5D49E9ED6768D7AE96EDFDE8DB` (break `/Game/HorrorEngine/Blueprints/Structures/SaveStructures/AssetsSave` AssetSave)))
  (if (`self.On / Off`)
    (`SceneComponent.SetVisibility` (`self.PointLight`) true false)))

(fn `UserConstructionScript`)