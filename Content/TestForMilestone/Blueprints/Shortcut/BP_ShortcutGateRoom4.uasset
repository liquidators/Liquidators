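; BP_ShortcutGateRoom4 is a shortcut gate that opens when switched on and keeps that state through saves.
; Open/On runs an interaction check, waits briefly, sets OnOff, then eases the Billboard component to a target transform while a mechanical door sound plays.
; Save events store OnOff through the player's save component cache and, on restore, snap an opened gate straight to that transform.
; The target passes the actor's location as a relative location.
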(event `self.Open/On`
  (params (HorrorEvent :type Boolean))
  (bind _billboard (`self.Billboard`))
  (`/Game/HorrorEngine/Blueprints/Core/HorrorEngineMacros.HM_CheckInteraction`)
  (`KismetSystemLibrary.Delay` 1.0)
  (bind _returnvalue (`GameplayStatics.SpawnSoundAttached` "/Game/Sounds4/MechDoorOpening.MechDoorOpening" _billboard "None" (0.0 0.0 0.0) (struct) "KeepRelativeOffset" false 1.0 1.0 0.0 null null))
  (set `self.DoorSound` _returnvalue)
  (set `self.On / Off` true)
  (`KismetSystemLibrary.MoveComponentTo` _billboard (`self.K2_GetActorLocation`) (`self.Rotator`) true true 4.0)
  (`AudioComponent.Stop` (`self.DoorSound`)))

(event `/Game/HorrorEngine/Blueprints/Core/HorrorEngineInterface.CollectSaveData`
  (bind _asmaster (`/Game/HorrorEngine/Blueprints/Core/HorrorEngineFunctions.GetPlayer`))
  (`KismetArrayLibrary.Array_Add` (`/Game/HorrorEngine/Blueprints/Core/HE_SaveGameComponent.AssetCache` (`/Game/HorrorEngine/HorrorEngine.HE_SaveGameComponent` _asmaster)) (make `/Game/HorrorEngine/Blueprints/Structures/SaveStructures/AssetsSave` (`KismetSystemLibrary.GetObjectName` self) (`self.On / Off`) false false false 0.0 0.0 0 "+00000000.00:00:00.000000000" "NewEnumerator0" (struct :`Actor` "NewEnumerator0" :`MeshSettings` (struct) :`InspectionSettings` (struct :`InspectionPivotLocation` (0.0 0.0 0.0) :`Takeable` true :`InspectionAnimation` true :`InspectionAnimationSpeedSec` 0.5 :`InspectionBeginRotation` (struct) :`InspectionBeginScale` 1.0 :`MinZoomScale` 1.0 :`MaxZoomScale` 2.0 :`RotationSpeed` 2.5 :`SlideSpeed` 1.0 :`MaxSlideValue` 10.0 :`ItemName` "NSLOCTEXT(\"[9E6C87BD41F93F6DEA60AABA858AC7A8]\", \"6A6D9A4246684EE8043E719EC2A82245\", \"Item Name\")" :`ItemInformation` "NSLOCTEXT(\"[9E6C87BD41F93F6DEA60AABA858AC7A8]\", \"ED47920B4C36E7377CE3869C6C8E4D4A\", \"Item Information\")" :`ReadingText` "NSLOCTEXT(\"[9E6C87BD41F93F6DEA60AABA858AC7A8]\", \"6D5AF6014576E1E5E0DD46B43C4900C7\", \"Reading Text\")" :`TakeButton` (struct :`ButtonText` "NSLOCTEXT(\"[9E6C87BD41F93F6DEA60AABA858AC7A8]\", \"702120AF41B067F781C77EBD3C1645BC\", \"Take\")") :`ExamineButton` (struct :`ButtonText` "NSLOCTEXT(\"[9E6C87BD41F93F6DEA60AABA858AC7A8]\", \"16F8C04643629CF00C07CE81A7483811\", \"Examine\")") :`ZoomSlideButton` (struct :`ButtonText` "NSLOCTEXT(\"[9E6C87BD41F93F6DEA60AABA858AC7A8]\", \"E04B7C3345EBC535540F34862B76E969\", \"Zoom/Slide\")") :`DismissButton` (struct :`ButtonText` "NSLOCTEXT(\"[9E6C87BD41F93F6DEA60AABA858AC7A8]\", \"8A97D6D343E9C5B63F0D8493937C9344\", \"Dismiss\")")) :`InventorySettings` (struct :`StorageType` "NewEnumerator3" :`NumberofItemstoAddInventory` 1 :`Interactable` true :`InteractionButton` (struct :`ButtonText` "NSLOCTEXT(\"[9E6C87BD41F93F6DEA60AABA858AC7A8]\", \"A6B6D8A14C0A7A17D858A4A70C48444D\", \"Use\")") :`SwitchButton` (struct :`ButtonText` "NSLOCTEXT(\"[9E6C87BD41F93F6DEA60AABA858AC7A8]\", \"0AA6195B4E09FFD64E316EBBDAECDFD5\", \"Switch\")") :`ZoomSlideButton` (struct :`ButtonText` "NSLOCTEXT(\"[9E6C87BD41F93F6DEA60AABA858AC7A8]\", \"FF16A6334D0BFFF0EA353FBBB9590408\", \"Zoom/Slide\")") :`CloseInventoryButton` (struct :`ButtonText` "NSLOCTEXT(\"[9E6C87BD41F93F6DEA60AABA858AC7A8]\", \"0B078CB443246115E2089EA78222A308\", \"Close\")")) :`Pistol_MeshSettingsTop` (struct) :`Vhs_CurrentTime` "+00000000.00:00:00.000000000"))))

(event `/Game/HorrorEngine/Blueprints/Core/HorrorEngineInterface.RestoreSaveData`
  (params (AssetSave :type "/Game/HorrorEngine/Blueprints/Structures/SaveStructures/AssetsSave Structure"))
  (set `self.On / Off` (`.BooleanSlot01_63_ED79FB5D49E9ED6768D7AE96EDFDE8DB` (break `/Game/HorrorEngine/Blueprints/Structures/SaveStructures/AssetsSave` AssetSave)))
  (if (`self.On / Off`)
    (`SceneComponent.K2_SetRelativeTransform` (`self.Billboard`) (`KismetMathLibrary.MakeTransform` (`self.K2_GetActorLocation`) (`self.Rotator`)) false false)))

(fn `UserConstructionScript`)