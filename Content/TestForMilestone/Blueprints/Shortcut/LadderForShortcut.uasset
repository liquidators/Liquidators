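; Climbable ladder actor that puts the player into Flying movement inside its box and restores Walking on exit, firing horror event checks both ways.
; The construction script builds it from instanced bottom, middle, connector and top meshes by step count, sizing the box to match.
; While climbing, forward input follows camera pitch and yaw, Run changes fly speed, and Jump optionally launches the player off.
; Climb sounds play at vertical distance intervals.
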(event `self.Box.OnComponentBeginOverlap`
  (params (OverlappedComponent :type "PrimitiveComponent Object Reference") (OtherActor :type "Actor Object Reference") (OtherComp :type "PrimitiveComponent Object Reference") (OtherBodyIndex :type Integer) (bFromSweep :type Boolean) (SweepResult :type "HitResult Structure (by ref)"))
  ;[1 1 1] Interaction Settings
  (if (== OtherActor (`GameplayStatics.GetPlayerPawn` 0))
    (`CharacterMovementComponent.SetMovementMode` (`Character.CharacterMovement` (`GameplayStatics.GetPlayerCharacter` 0)) "MOVE_Flying" 0)
    (`self.ControllerInput` true)
    (`self.HorrorEventCheck` "NewEnumerator41")))

(event `Leave Ladder`
  ;[1 1 1] Interaction Settings
  (`CharacterMovementComponent.SetMovementMode` (`Character.CharacterMovement` (`GameplayStatics.GetPlayerCharacter` 0)) "MOVE_Walking" 0 :!label _label)
  (`self.ControllerInput` false)
  (set `CharacterMovementComponent.MaxFlySpeed` 80.0 (`Character.CharacterMovement` (`GameplayStatics.GetPlayerCharacter` 0)))
  (`self.HorrorEventCheck` "NewEnumerator42"))

(event `self.Box.OnComponentEndOverlap`
  (params (OverlappedComponent :type "PrimitiveComponent Object Reference") (OtherActor :type "Actor Object Reference") (OtherComp :type "PrimitiveComponent Object Reference") (OtherBodyIndex :type Integer))
  ;[1 1 1] Interaction Settings
  (if (== OtherActor (`GameplayStatics.GetPlayerPawn` 0))
    (goto _label)))

(event `InputAxis|[HE]MoveForward`
  (params (AxisValue :type "Float (single-precision)"))
  (bind _returnvalue (`GameplayStatics.GetPlayerCharacter` 0))
  (bind (_returnvalue_roll _returnvalue_pitch _returnvalue_yaw) (`KismetMathLibrary.BreakRotator` (`Pawn.GetControlRotation` _returnvalue)))
  ;[1 1 1] Interaction Settings
  (`Pawn.AddMovementInput` _returnvalue (`KismetMathLibrary.GetForwardVector` (`KismetMathLibrary.MakeRotator` 0.0 _returnvalue_pitch _returnvalue_yaw)) AxisValue false)
  (`self.LadderFootsteps`))

(event `InputAction|[HE]Run`
  (params (Key :type "Key Structure"))
  (bind _charactermovement (`Character.CharacterMovement` (`GameplayStatics.GetPlayerCharacter` 0)))
  ;[1 1 1] Interaction Settings
  (:`Pressed`
    (set `CharacterMovementComponent.MaxFlySpeed` (`self.FastClimbSpeed`) _charactermovement))
  (:`Released`
    (set `CharacterMovementComponent.MaxFlySpeed` (`self.ClimbSpeed`) _charactermovement)))

(event `InputAction|[HE]Jump`
  (params (Key :type "Key Structure"))
  (bind _returnvalue (`GameplayStatics.GetPlayerCharacter` 0))
  (bind _jumpscale (`self.JumpScale`))
  (bind (_returnvalue_x _returnvalue_y) (`KismetMathLibrary.BreakVector` (* (`SceneComponent.GetForwardVector` (`Character.CapsuleComponent` _returnvalue)) _jumpscale)))
  ;[1 1 1] Interaction Settings
  (:`Pressed`
    (if (`self.CanJump`)
      (`self.Leave Ladder`)
      (`Character.LaunchCharacter` _returnvalue (`KismetMathLibrary.MakeVector` _returnvalue_x _returnvalue_y _jumpscale) false false))))

(event `self.Open/On`
  (params (HorrorEvent :type Boolean))
  (`/Game/HorrorEngine/Blueprints/Core/HorrorEngineMacros.HM_CheckInteraction`))

(fn `LadderFootsteps`
  (bind _climbsound (`self.ClimbSound`))
  (bind _capsulecomponent (`Character.CapsuleComponent` (`GameplayStatics.GetPlayerCharacter` 0)))
  (bind (_returnvalue_x _returnvalue_y _returnvalue_z) (`KismetMathLibrary.BreakVector` (`SceneComponent.K2_GetComponentLocation` _capsulecomponent)))
  (if (or (<= (+ (`self.LastFootstepLocation`) (`self.ClimbSoundRate`)) _returnvalue_z) (>= (- (`self.LastFootstepLocation`) (`self.ClimbSoundRate`)) _returnvalue_z))
    (`/Game/HorrorEngine/Blueprints/Core/HorrorEngineMacros.HM_3DSound` _climbsound false _climbsound _capsulecomponent "/Game/HorrorEngine/Audio/_ATT_Profiles/ATT_General.ATT_General")
    (set `self.LastFootstepLocation` _returnvalue_z)))

(fn `UserConstructionScript`
  (bind _returnvalue (- (`self.LadderStep`) 1))
  (`/Game/HorrorEngine/Blueprints/Core/HorrorEngineMacros.HM_DefaultConstructions` (`self.CreateNewHorrorEvent`))
  (`/Game/HorrorEngine/Blueprints/Core/HorrorEngineFunctions.SetMesh` (`self.LadderTop`) (`self.LadderTopMesh`))
  (`/Game/HorrorEngine/Blueprints/Core/HorrorEngineFunctions.SetMesh` (`self.LadderMiddle`) (`self.LadderMiddleMesh`))
  (`/Game/HorrorEngine/Blueprints/Core/HorrorEngineFunctions.SetMesh` (`self.LadderConnect`) (`self.LadderConnectMesh`))
  (`/Game/HorrorEngine/Blueprints/Core/HorrorEngineFunctions.SetMesh` (`self.LadderBottom`) (`self.LadderBottomMesh`))
  (for _index (range (+ _returnvalue 1))
    (if (== _index 0)
      (bind _returnvalue_2 (* _index (`self.LadderHeight`)))
      (`InstancedStaticMeshComponent.AddInstance` (`self.LadderBottom`) (`KismetMathLibrary.MakeTransform` (`KismetMathLibrary.MakeVector` 0.0 0.0 _returnvalue_2)))
      (elif (== _index _returnvalue)
        (`InstancedStaticMeshComponent.AddInstance` (`self.LadderTop`) (`KismetMathLibrary.MakeTransform` (`KismetMathLibrary.MakeVector` 0.0 0.0 _returnvalue_2)))
        (`SceneComponent.K2_SetRelativeLocation` (`self.Box`) (`KismetMathLibrary.MakeVector` 0.0 25.0 (- (`KismetMathLibrary.Conv_IntToDouble` (* (`self.LadderStep`) 20)) 20.0)) false false)
        (`BoxComponent.SetBoxExtent` (`self.Box`) (`KismetMathLibrary.MakeVector` 30.0 25.0 (`KismetMathLibrary.Conv_IntToDouble` (* (`self.LadderStep`) 20))) true)
        (elif (== (mod _index (`self.ConnectRate`)) 0)
          (`InstancedStaticMeshComponent.AddInstance` (`self.LadderConnect`) (`KismetMathLibrary.MakeTransform` (`KismetMathLibrary.MakeVector` 0.0 0.0 _returnvalue_2)))
          (else
            (`InstancedStaticMeshComponent.AddInstance` (`self.LadderMiddle`) (`KismetMathLibrary.MakeTransform` (`KismetMathLibrary.MakeVector` 0.0 0.0 _returnvalue_2)))))))))