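; Sound manager Blueprint that fades out the level's ambient sounds for an underwater death.
; PlayUnderwaterDeath, or a debug O key press, gathers every AmbientSound actor and runs a timeline that drives each audio component's volume multiplier along a FadeOut curve.
; Despite the EQ naming only volume changes: the Tick flag check and ResetEQonallsounds are empty, and the FadeIn volume node is never executed.
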(event `self.ReceiveTick`
  (params (DeltaSeconds :type "Float (single-precision)"))
  (if (`self.TriggerUnderwaterDeath EQ`)
    _))

(event `Key|O`
  (params (Key :type "Key Structure"))
  (:`Pressed`
    (`KismetSystemLibrary.PrintString` "Hello")
    (bind _outactors (`GameplayStatics.GetAllActorsOfClass` "/Script/Engine.AmbientSound" :!label _label))
    (set `self.CurrentAmbientSounds` _outactors)
    (bind (_direction _fadeout _fadein) (`Timeline|Timeline_0` :!via `PlayFromStart`)
      (:`Update`
        (for _array_element (`self.CurrentAmbientSounds`)
          (`AudioComponent.SetVolumeMultiplier` (`AmbientSound.AudioComponent` _array_element) _fadeout))))))

(event `Play Underwater Death`
  (set `self.TriggerUnderwaterDeath EQ` true)
  (goto _label))

(event `Reset EQ on all sounds`)

(fn `UserConstructionScript`)