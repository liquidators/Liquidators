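; BP_ElephantFootDmg is a hazard actor that damages the player while it has line of sight, with damage rising as distance shrinks.
; BeginPlay starts a looping timer that traces on the Visibility channel from the actor to the player camera.
; A hit on the player pawn calls GetDamage with inverse-distance damage scaled by DMGMultiplier.
; StopDMG pauses the timer; debug trace drawing and damage printing are left on.
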(event `self.ReceiveBeginPlay`
  (`self.Start DMG`))

(event `Start DMG`
  (bind _returnvalue (`KismetSystemLibrary.K2_SetTimerDelegate` (delegate `LineTraceForDMG`) (`self.Time Between Line Traces`) true))
  (set `self.Timer Handle` _returnvalue))

(event `LineTraceForDMG`
  (bind _outhit (`KismetSystemLibrary.LineTraceSingle` (`self.K2_GetActorLocation`) (`PlayerCameraManager.GetCameraLocation` (`GameplayStatics.GetPlayerCameraManager` 0)) "TraceTypeQuery1" true (`self.Actors For Trace To Ignore`) "ForDuration" true (struct :`R` 1.0 :`A` 1.0) (struct :`G` 1.0 :`A` 1.0) 1.0))
  (bind (_bblockinghit _binitialoverlap _time _distance _location _impactpoint _normal _impactnormal _physmat _hitactor) (`GameplayStatics.BreakHitResult` _outhit))
  (if (== _hitactor (`GameplayStatics.GetPlayerPawn` 0))
    (bind _returnvalue (* (/ 600.0 _distance) (`self.DMG Multiplier`)))
    (`KismetSystemLibrary.PrintString` (`KismetStringLibrary.Conv_DoubleToString` _returnvalue))
    (bind _asmaster (`/Game/HorrorEngine/Blueprints/Core/HorrorEngineFunctions.GetPlayer`))
    (`/Game/HorrorEngine/HorrorEngine.GetDamage` :`self` _asmaster :`DamagePoint` _returnvalue)))

(event `Stop DMG`
  (`KismetSystemLibrary.K2_PauseTimerHandle` (`self.Timer Handle`)))

(fn `UserConstructionScript`)