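; Interactable worker corpse the player can pick up and carry, with inspection and inventory setup from its horror-event parent.
; Use checks the player is neither carrying nor crawling; inspection joins the same pickup when Takeable, skipping those checks.
; Pickup fades the camera, records the body's name on the player, updates hand material, speed and terminal mission text, then destroys the actor.
; A name-based event sets the worker material, while front and back lights blink until hidden.
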(event `Blink Light`
  (`SceneComponent.ToggleVisibility` (`self.Front Light`) false :!label _label)
  (`SceneComponent.ToggleVisibility` (`self.Back Light`) false)
  (`KismetSystemLibrary.RetriggerableDelay` 0.2)
  (if (`self.bHidden`)
    (`SceneComponent.SetVisibility` (`self.Front Light`) false false)
    (`SceneComponent.SetVisibility` (`self.Back Light`) false false)
    (else
      (goto _label))))

(event `Pick Up Body Animation`
  (bind _returnvalue (`GameplayStatics.GetPlayerCameraManager` 0))
  (`PlayerCameraManager.StartCameraFade` :`self` _returnvalue :`ToAlpha` 1.0 :`Duration` 0.5 :`bHoldWhenFinished` true)
  (`KismetSystemLibrary.Delay` 1.0)
  (`PlayerCameraManager.StartCameraFade` _returnvalue 1.0 0.0 0.5 (struct :`A` 1.0) false true))

(event `/Game/HorrorEngine/Blueprints/Core/Use.Use`
  (params (HorrorEvent :type Boolean))
  ;[1 1 1] Take Settings
  (bind _asmy_character (cast `/Game/TestForMilestone/Blueprints/MyCharacter` (`GameplayStatics.GetPlayerCharacter` 0)))
  (if (not (`/Game/TestForMilestone/Blueprints/MyCharacter.CarryingBody` _asmy_character))
    (bind _asmaster (`/Game/HorrorEngine/Blueprints/Core/HorrorEngineFunctions.GetPlayer`))
    (if (not (`/Game/HorrorEngine/HorrorEngine.Crawling` _asmaster))
      (`self.Pick Up Body Animation` :!label _label_2)
      (`GameplayStatics.SpawnSound2D` "/Game/Sounds5/Latest_Sound_Effects/BodyPickup_Cue.BodyPickup_Cue" 1.0 1.0 0.0 null)
      (`KismetSystemLibrary.Delay` 1.0)
      (set `/Game/TestForMilestone/Blueprints/MyCharacter.CarryingBody` true (`self.PlayerPawn`))
      (bind _asmaster_2 (`/Game/HorrorEngine/Blueprints/Core/HorrorEngineFunctions.GetPlayer`))
      (set `/Game/HorrorEngine/HorrorEngine.CurrentBodyBeingCarried` (`self.name`) _asmaster_2)
      (`/Game/TestForMilestone/Blueprints/MyCharacter.Change Body Hand Material` (`self.PlayerPawn`))
      (`self.SetActorHiddenInGame` true)
      (bind _asmaster_3 (`/Game/HorrorEngine/Blueprints/Core/HorrorEngineFunctions.GetPlayer`))
      (`/Game/HorrorEngine/HorrorEngine.CalculateSpeed` _asmaster_3)
      (bind _returnvalue (`GameplayStatics.GetActorOfClass` "/Game/WISTerminals/Blueprints/BP_TerminalController.BP_TerminalController_C"))
      (`/Game/WISTerminals/Blueprints/BP_TerminalController.Change Start Mission Text` _returnvalue)
      (`self.K2_DestroyActor`))))

(event `self.InspectionUse`
  ;[1 1 1] Take Settings
  (if (`self.Takeable`)
    (`self.Take` true true true)
    (goto _label_2)))

(event `Change Mesh Based On Character Name`
  (params (Name :type String))
  (bind _asmy_character (cast `/Game/TestForMilestone/Blueprints/MyCharacter` (`GameplayStatics.GetPlayerPawn` 0)))
  (set `self.PlayerPawn` _asmy_character)
  (if (`KismetStringLibrary.EqualEqual_StrStr` Name "Alexei")
    (`PrimitiveComponent.SetMaterial` (`self.body`) 0 "/Game/ChemicalWorker/Materials/Instances/MI_WorkerAlexei.MI_WorkerAlexei")
    (elif (`KismetStringLibrary.EqualEqual_StrStr` Name "Boris")
      (`PrimitiveComponent.SetMaterial` (`self.body`) 0 "/Game/ChemicalWorker/Materials/Instances/M_WorkerBoris.M_WorkerBoris")
      (elif (`KismetStringLibrary.EqualEqual_StrStr` Name "Valeri")
        (`PrimitiveComponent.SetMaterial` (`self.body`) 0 "/Game/ChemicalWorker/Materials/Instances/MI_WorkerValeri.MI_WorkerValeri")))))

(fn `UserConstructionScript`
  (`parent.UserConstructionScript`)
  (`SkinnedMeshComponent.SetSkinnedAssetAndUpdate` (`self.body`) (`self.skeletalmesh`) true)
  (`/Game/HorrorEngine/Blueprints/Core/HorrorEngineMacros.HM_DefaultConstructions` (`self.CreateNewHorrorEvent`))
  (`self.SetInspection` (`self.InspectionSettings`))
  (`self.SetInventory` (`self.InventorySettings`))
  (`SceneComponent.K2_AttachToComponent` (`self.mask`) (`self.body`) "head" "KeepRelative" "KeepRelative" "KeepRelative" true))