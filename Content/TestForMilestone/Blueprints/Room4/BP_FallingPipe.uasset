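; BP_FallingPipe is a one-shot scare prop: a pipe that swings to a set rotation when its trigger is overlapped.
; A separate volume fades creaking audio in and out.
; After a short delay, the trigger plays a loud break sound, starts and increments BP_HeartBeatSound, then eases the mesh rotation.
; Save hooks use the player's asset cache, and restore snaps the pipe to its fallen rotation if triggered.
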(event `self.ReceiveBeginPlay`
  (`AudioComponent.Stop` (`self.Medium`)))

(event `self.Creaking Sound.OnComponentBeginOverlap`
  (params (OverlappedComponent :type "PrimitiveComponent Object Reference") (OtherActor :type "Actor Object Reference") (OtherComp :type "PrimitiveComponent Object Reference") (OtherBodyIndex :type Integer) (bFromSweep :type Boolean) (SweepResult :type "HitResult Structure (by ref)"))
  (`AudioComponent.FadeIn` (`self.Medium`) 1.0 1.0 0.0 "Linear"))

(event `self.Creaking Sound.OnComponentEndOverlap`
  (params (OverlappedComponent :type "PrimitiveComponent Object Reference") (OtherActor :type "Actor Object Reference") (OtherComp :type "PrimitiveComponent Object Reference") (OtherBodyIndex :type Integer))
  (`AudioComponent.FadeOut` (`self.Medium`) 1.0 0.0 "Linear"))

(event `self.Trigger.OnComponentBeginOverlap`
  (params (OverlappedComponent :type "PrimitiveComponent Object Reference") (OtherActor :type "Actor Object Reference") (OtherComp :type "PrimitiveComponent Object Reference") (OtherBodyIndex :type Integer) (bFromSweep :type Boolean) (SweepResult :type "HitResult Structure (by ref)"))
  (if (not (`self.isTriggered`))
    (set `self.isTriggered` true)
    (`KismetSystemLibrary.Delay` 1.0)
    (`GameplayStatics.SpawnSound2D` "/Game/Sounds5/Latest_Sound_Effects/PipeBreak_Large_Cue.PipeBreak_Large_Cue" 3.0 1.0 0.0 null)
    (bind _returnvalue (`GameplayStatics.GetActorOfClass` "/Game/Sounds2/Area_4/BP_HeartBeatSound.BP_HeartBeatSound_C"))
    (`/Game/Sounds2/Area_4/BP_HeartBeatSound.Play HeartBeat` _returnvalue)
    (`/Engine/EditorBlueprintResources/StandardMacros.IncrementInt` (`/Game/Sounds2/Area_4/BP_HeartBeatSound.Heart_Count` _returnvalue)
      (:`  `
        (`KismetSystemLibrary.MoveComponentTo` (`self.PipeMesh`) (0.0 0.0 0.0) (`self.Rotator`) true true 1.0)))))

(event `/Game/HorrorEngine/Blueprints/Core/HorrorEngineInterface.CollectSaveData`
  (bind _asmaster (`/Game/HorrorEngine/Blueprints/Core/HorrorEngineFunctions.GetPlayer`))
  (`KismetArrayLibrary.Array_Add` (`/Game/HorrorEngine/Blueprints/Core/HE_SaveGameComponent.AssetCache` (`/Game/HorrorEngine/HorrorEngine.HE_SaveGameComponent` _asmaster)) (make `/Game/HorrorEngine/Blueprints/Structures/SaveStructures/AssetsSave` (`KismetSystemLibrary.GetObjectName` self) (`self.isTriggered`) false false false 0.0 0.0 0 "+00000000.00:00:00.000000000" "NewEnumerator0" (struct :`Actor` "NewEnumerator0" :`MeshSettings` (struct) :`InspectionSettings` (struct :`InspectionPivotLocation` (0.0 0.0 0.0) :`Takeable` true :`InspectionAnimation` true :`InspectionAnimationSpeedSec` 0.5 :`InspectionBeginRotation` (struct) :`InspectionBeginScale` 1.0 :`MinZoomScale` 1.0 :`MaxZoomScale` 2.0 :`RotationSpeed` 2.5 :`SlideSpeed` 1.0 :`MaxSlideValue` 10.0 :`ItemName` "NSLOCTEXT(\"[1F6CBE9247ABC2BFA63ABAA4A705EE01]\", \"744EB2954247801815E16DAC21B1E0E8\", \"Item Name\")" :`ItemInformation` "NSLOCTEXT(\"[1F6CBE9247ABC2BFA63ABAA4A705EE01]\", \"578BD3F645647F2BEB6D7CBB48EB9B06\", \"Item Information\")" :`ReadingText` "NSLOCTEXT(\"[1F6CBE9247ABC2BFA63ABAA4A705EE01]\", \"C0A5FA784218F3359A5471AE1C09882A\", \"Reading Text\")" :`TakeButton` (struct :`ButtonText` "NSLOCTEXT(\"[1F6CBE9247ABC2BFA63ABAA4A705EE01]\", \"C85986E346A1BC8298CFCDA6BF7A79AD\", \"Take\")") :`ExamineButton` (struct :`ButtonText` "NSLOCTEXT(\"[1F6CBE9247ABC2BFA63ABAA4A705EE01]\", \"6F5F186646B4613EFC157D8CB0B60145\", \"Examine\")") :`ZoomSlideButton` (struct :`ButtonText` "NSLOCTEXT(\"[1F6CBE9247ABC2BFA63ABAA4A705EE01]\", \"D9F0511A4E6A3A6CD4FA61BC638362CF\", \"Zoom/Slide\")") :`DismissButton` (struct :`ButtonText` "NSLOCTEXT(\"[1F6CBE9247ABC2BFA63ABAA4A705EE01]\", \"16BC8CBE456EF968CF50D291C4264F00\", \"Dismiss\")")) :`InventorySettings` (struct :`StorageType` "NewEnumerator3" :`NumberofItemstoAddInventory` 1 :`Interactable` true :`InteractionButton` (struct :`ButtonText` "NSLOCTEXT(\"[1F6CBE9247ABC2BFA63ABAA4A705EE01]\", \"434A536647DE4363A1A148867824BB86\", \"Use\")") :`SwitchButton` (struct :`ButtonText` "NSLOCTEXT(\"[1F6CBE9247ABC2BFA63ABAA4A705EE01]\", \"89C1AF8646E8D8050E2B9B9B9AD03CB7\", \"Switch\")") :`ZoomSlideButton` (struct :`ButtonText` "NSLOCTEXT(\"[1F6CBE9247ABC2BFA63ABAA4A705EE01]\", \"4140315F413D873C779769958E91E2A5\", \"Zoom/Slide\")") :`CloseInventoryButton` (struct :`ButtonText` "NSLOCTEXT(\"[1F6CBE9247ABC2BFA63ABAA4A705EE01]\", \"A84E6525453F4BEFED49CD9274C42243\", \"Close\")")) :`Pistol_MeshSettingsTop` (struct) :`Vhs_CurrentTime` "+00000000.00:00:00.000000000"))))

(event `/Game/HorrorEngine/Blueprints/Core/HorrorEngineInterface.RestoreSaveData`
  (params (AssetSave :type "/Game/HorrorEngine/Blueprints/Structures/SaveStructures/AssetsSave Structure"))
  (set `self.isTriggered` (`.BooleanSlot01_63_ED79FB5D49E9ED6768D7AE96EDFDE8DB` (break `/Game/HorrorEngine/Blueprints/Structures/SaveStructures/AssetsSave` AssetSave)))
  (if (`self.isTriggered`)
    (`SceneComponent.K2_SetRelativeRotation` (`self.PipeMesh`) (`self.Rotator`) false false)))

(fn `UserConstructionScript`)