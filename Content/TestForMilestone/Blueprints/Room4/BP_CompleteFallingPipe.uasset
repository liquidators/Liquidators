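; BP_CompleteFallingPipe is a one-shot scare prop in Room 4: a pipe that breaks and falls.
; Overlapping Trigger once waits a second, plays a break sound, enables physics on Pipe, then starts the BP_HeartBeatSound actor's heartbeat and increments its HeartCount.
; A separate CreakingSound overlap volume fades the Large audio in and out on enter and exit.
; An eased MoveComponentTo drop remains in the graph but is unconnected.
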(event `self.ReceiveBeginPlay`
  (`AudioComponent.Stop` (`self.large`)))

(event `self.Trigger.OnComponentBeginOverlap`
  (params (OverlappedComponent :type "PrimitiveComponent Object Reference") (OtherActor :type "Actor Object Reference") (OtherComp :type "PrimitiveComponent Object Reference") (OtherBodyIndex :type Integer) (bFromSweep :type Boolean) (SweepResult :type "HitResult Structure (by ref)"))
  (if (not (`self.IsTriggered`))
    (set `self.IsTriggered` true)
    (`KismetSystemLibrary.Delay` 1.0)
    (`GameplayStatics.SpawnSound2D` "/Game/Sounds5/Latest_Sound_Effects/PipeBreak_Smaller_Cue.PipeBreak_Smaller_Cue" 1.0 1.0 0.0 null)
    (`PrimitiveComponent.SetSimulatePhysics` (`self.Pipe`) true)
    (bind _returnvalue (`GameplayStatics.GetActorOfClass` "/Game/Sounds2/Area_4/BP_HeartBeatSound.BP_HeartBeatSound_C"))
    (`/Game/Sounds2/Area_4/BP_HeartBeatSound.Play HeartBeat` _returnvalue)
    (`/Engine/EditorBlueprintResources/StandardMacros.IncrementInt` (`/Game/Sounds2/Area_4/BP_HeartBeatSound.Heart_Count` _returnvalue))))

(event `self.Creaking Sound.OnComponentBeginOverlap`
  (params (OverlappedComponent :type "PrimitiveComponent Object Reference") (OtherActor :type "Actor Object Reference") (OtherComp :type "PrimitiveComponent Object Reference") (OtherBodyIndex :type Integer) (bFromSweep :type Boolean) (SweepResult :type "HitResult Structure (by ref)"))
  (`AudioComponent.FadeIn` (`self.large`) 1.0 2.0 0.0 "Linear"))

(event `self.Creaking Sound.OnComponentEndOverlap`
  (params (OverlappedComponent :type "PrimitiveComponent Object Reference") (OtherActor :type "Actor Object Reference") (OtherComp :type "PrimitiveComponent Object Reference") (OtherBodyIndex :type Integer))
  (`AudioComponent.FadeOut` (`self.large`) 1.0 0.0 "Linear"))

(fn `UserConstructionScript`)