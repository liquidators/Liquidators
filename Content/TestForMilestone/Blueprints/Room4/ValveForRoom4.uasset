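; One-way interactable valve for Room 4 that lowers the room's fluid, with a tag selecting the first or second drop.
; Use drives a timeline turn animation with 3D sounds and bumps a dialogue actor counter that triggers a win sound.
; BeginPlay polls, blinking a warning light until the turn finishes, then turns it green, moves BP_Room4Fluid and increments saved progress.
; Save restore reapplies valve pose and fluid state.
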(event `self.ReceiveBeginPlay`
  (bind _warninglight (`self.WarningLight`))
  ;[1 1 1] Light Modification
  (`KismetSystemLibrary.RetriggerableDelay` 0.2 :!label _label)
  (`SceneComponent.ToggleVisibility` _warninglight false)
  (if (`self.IsUsed`)
    (`SceneComponent.SetVisibility` _warninglight true false)
    (`LightComponent.SetLightColor` _warninglight (struct :`R` 0.142161 :`G` 1.0 :`B` 0.019228 :`A` 1.0) true)
    (`GameplayStatics.PlaySound2D` "/Game/Sounds2/Misc_Sounds/ValveTurn_Cue.ValveTurn_Cue" 1.0 1.0 0.0 null null)
    (bind _returnvalue (`GameplayStatics.GetActorOfClass` "/Game/TestForMilestone/Blueprints/Room2/BP_Room4Fluid.BP_Room4Fluid_C"))
    (if (`self.ActorHasTag` "SecondValveRoom4")
      (`/Game/TestForMilestone/Blueprints/Room2/BP_Room4Fluid.Second Move Down` _returnvalue)
      (else
        (`/Game/TestForMilestone/Blueprints/Room2/BP_Room4Fluid.First Move Down` _returnvalue)))
    (`self.Update Game Progress`)
    (else
      (goto _label))))

(event `Temporary Game Over Event`
  (`self.DisableInput` (`GameplayStatics.GetPlayerPawn` 0) (`GameplayStatics.GetPlayerController` 0))
  (`PlayerCameraManager.StartCameraFade` :`self` (`GameplayStatics.GetPlayerCameraManager` 0) :`ToAlpha` 1.0 :`Duration` 3.0 :`bShouldFadeAudio` true :`bHoldWhenFinished` true)
  (`KismetSystemLibrary.Delay` 3.0)
  (`WidgetLayoutLibrary.RemoveAllWidgets`)
  (bind _returnvalue (`|CreateWidget` "/Game/TestForMilestone/Blueprints/Room1Hazards/Temporary_widget/ComingSoonScreen.ComingSoonScreen_C"))
  (`UserWidget.AddToViewport` _returnvalue 0)
  (`KismetSystemLibrary.Delay` 8.0)
  (`GameplayStatics.OpenLevel` "1"))

(event `self.Use`
  (params (HorrorEvent :type Boolean))
  ;[1 1 1] Interact Settings
  (`/Game/HorrorEngine/Blueprints/Core/HorrorEngineMacros.HM_CheckInteraction`)
  (if (`self.On / Off`)
    (`self.Close/Off` false)
    (else
      (`self.Open/On` false)
      (`KismetSystemLibrary.Delay` 5.0)
      (bind _returnvalue (`GameplayStatics.GetActorOfClass` "/Game/Dialogue/V1/BP_Room4Dialogue.BP_Room4Dialogue_C"))
      (bind _result (`/Engine/EditorBlueprintResources/StandardMacros.IncrementInt` (`/Game/Dialogue/V1/BP_Room4Dialogue.Counting` _returnvalue))
        (:`  `
          (if (== _result 2)
            (`GameplayStatics.PlaySound2D` "/Game/Dialogue/V1/Win_Cue.Win_Cue" 1.0 1.0 0.0 null null)))))))

(event `self.Open/On`
  (params (HorrorEvent :type Boolean))
  (bind _actorstouse (`self.ActorsToUse`))
  ;[1 1 1] Open / Close Settings
  (`/Game/HorrorEngine/Blueprints/Core/HorrorEngineMacros.HM_CheckInteraction`)
  (if (not (`self.On / Off`))
    (if (not (`self.UseAfterAnimation`))
      (set `self.On / Off` true)
      (`self.Open/On` (`self.ActorsToUse`) false)
      (`self.HorrorEventCheck` "NewEnumerator3"))
    (set `self.InteractionEnabled` false)
    (`/Game/HorrorEngine/Blueprints/Core/HorrorEngineMacros.HM_3DSound` (`self.HitSound`) false (`self.TurnOnSound`) (`self.ValvePivot`) (`self.SoundAttenuation`))
    (`/Game/HorrorEngine/Blueprints/Core/HorrorEngineMacros.HM_3DSound` null false (`self.LoopSound`) (`self.ValvePivot`) (`self.SoundAttenuation`))
    (bind (_direction _animation) (`Timeline|ButtonTimeline` :!via `PlayFromStart`)
      (:`Update`
        (`SceneComponent.K2_SetRelativeLocationAndRotation` (`self.ValvePivot`) (`KismetMathLibrary.VLerp` (`self.OffLocation`) (`self.OnLocation`) _animation) (`KismetMathLibrary.RLerp` (`self.OffRotation`) (`self.OnRotation`) _animation) false false))
      (:`Finished`
        (set `self.IsUsed` true)
        (switch `ETimelineDirection` _direction
          (:`Forward`
            (if (`self.UseAfterAnimation`)
              (set `self.On / Off` true)
              (`self.Open/On` _actorstouse false)
              (`self.HorrorEventCheck` "NewEnumerator3")))
          (:`Backward`
            (if (`self.UseAfterAnimation`)
              (set `self.On / Off` false)
              (`self.Close/Off` _actorstouse false)
              (`self.HorrorEventCheck` "NewEnumerator4"))))
        (set `self.InteractionEnabled` true)
        (if (`self.StopSoundsAfterAnimation`)
          (`/Game/HorrorEngine/Blueprints/Core/HorrorEngineMacros.HM_StopAll3DSounds`))
        (`/Game/HorrorEngine/Blueprints/Core/HorrorEngineMacros.HM_3DSound` null false (`self.HitSound`) (`self.ValvePivot`) (`self.SoundAttenuation`))))))

(event `self.Close/Off`
  (params (HorrorEvent :type Boolean))
  ;[1 1 1] Open / Close Settings
)

(event `/Game/HorrorEngine/Blueprints/Core/HorrorEngineInterface.CollectSaveData`
  ;[0 1 0.5572] Save Settings
  (bind _asmaster (`/Game/HorrorEngine/Blueprints/Core/HorrorEngineFunctions.GetPlayer`))
  (`KismetArrayLibrary.Array_Add` (`/Game/HorrorEngine/Blueprints/Core/HE_SaveGameComponent.AssetCache` (`/Game/HorrorEngine/HorrorEngine.HE_SaveGameComponent` _asmaster)) (make `/Game/HorrorEngine/Blueprints/Structures/SaveStructures/AssetsSave` (`KismetSystemLibrary.GetObjectName` self) (`self.On / Off`) false false false 0.0 0.0 0 "+00000000.00:00:00.000000000" "NewEnumerator0" (struct :`Actor` "NewEnumerator0" :`MeshSettings` (struct) :`InspectionSettings` (struct :`InspectionPivotLocation` (0.0 0.0 0.0) :`Takeable` true :`InspectionAnimation` true :`InspectionAnimationSpeedSec` 0.5 :`InspectionBeginRotation` (struct) :`InspectionBeginScale` 1.0 :`MinZoomScale` 1.0 :`MaxZoomScale` 2.0 :`RotationSpeed` 2.5 :`SlideSpeed` 1.0 :`MaxSlideValue` 10.0 :`ItemName` "NSLOCTEXT(\"[A4A9726D421AC31E3509178E9589978C]\", \"2E30B9A241A6DD1DD402F08BA0083EEB\", \"Item Name\")" :`ItemInformation` "NSLOCTEXT(\"[A4A9726D421AC31E3509178E9589978C]\", \"A1D4F772436505ADF854418EDDADD381\", \"Item Information\")" :`ReadingText` "NSLOCTEXT(\"[A4A9726D421AC31E3509178E9589978C]\", \"A4DDE728417DBB65994F3FAD67FC13F3\", \"Reading Text\")" :`TakeButton` (struct :`ButtonText` "NSLOCTEXT(\"[A4A9726D421AC31E3509178E9589978C]\", \"997DB02B445DFBA26573538809FBB0EF\", \"Take\")") :`ExamineButton` (struct :`ButtonText` "NSLOCTEXT(\"[A4A9726D421AC31E3509178E9589978C]\", \"7F13DC2C4543C3B5B29EF196D65DE799\", \"Examine\")") :`ZoomSlideButton` (struct :`ButtonText` "NSLOCTEXT(\"[A4A9726D421AC31E3509178E9589978C]\", \"337FD2194B75764765B5CCAAEFB1A03B\", \"Zoom/Slide\")") :`DismissButton` (struct :`ButtonText` "NSLOCTEXT(\"[A4A9726D421AC31E3509178E9589978C]\", \"EF5578EE441E2D8BB9FE96A925EE0085\", \"Dismiss\")")) :`InventorySettings` (struct :`StorageType` "NewEnumerator3" :`NumberofItemstoAddInventory` 1 :`Interactable` true :`InteractionButton` (struct :`ButtonText` "NSLOCTEXT(\"[A4A9726D421AC31E3509178E9589978C]\", \"F28E00BB45AA297BD25A7EB5E079C0F2\", \"Use\")") :`SwitchButton` (struct :`ButtonText` "NSLOCTEXT(\"[A4A9726D421AC31E3509178E9589978C]\", \"E0D38E7C474F32409FB898A997CC2BBB\", \"Switch\")") :`ZoomSlideButton` (struct :`ButtonText` "NSLOCTEXT(\"[A4A9726D421AC31E3509178E9589978C]\", \"C4BC190843ED4BECF38B6A9D34662E19\", \"Zoom/Slide\")") :`CloseInventoryButton` (struct :`ButtonText` "NSLOCTEXT(\"[A4A9726D421AC31E3509178E9589978C]\", \"ECEAE094498B3ECF8208349A8E2932F2\", \"Close\")")) :`Pistol_MeshSettingsTop` (struct) :`Vhs_CurrentTime` "+00000000.00:00:00.000000000"))))

(event `/Game/HorrorEngine/Blueprints/Core/HorrorEngineInterface.RestoreSaveData`
  (params (AssetSave :type "/Game/HorrorEngine/Blueprints/Structures/SaveStructures/AssetsSave Structure"))
  (bind (_relativelocation_x _relativelocation_y) (`KismetMathLibrary.BreakVector` (`SceneComponent.RelativeLocation` (`StaticMeshActor.StaticMeshComponent` (`self.Room4 Fluid`)))))
  ;[0 1 0.5572] Save Settings
  (set `self.On / Off` (`.BooleanSlot01_63_ED79FB5D49E9ED6768D7AE96EDFDE8DB` (break `/Game/HorrorEngine/Blueprints/Structures/SaveStructures/AssetsSave` AssetSave)))
  (`SceneComponent.K2_SetRelativeLocationAndRotation` (`self.ValvePivot`) (select `bool` (`self.On / Off`) :`false` (`self.OffLocation`) :`true` (`self.OnLocation`)) (select `bool` (`self.On / Off`) :`false` (`self.OffRotation`) :`true` (`self.OnRotation`)) false false)
  (set `self.IsUsed` (`self.On / Off`))
  (if (`self.On / Off`)
    (bind _returnvalue (`GameplayStatics.GetActorOfClass` "/Game/TestForMilestone/Blueprints/Room2/BP_Room4Fluid.BP_Room4Fluid_C"))
    (set `self.Room4 Fluid` _returnvalue)
    (bind _asmaster (`/Game/HorrorEngine/Blueprints/Core/HorrorEngineFunctions.GetPlayer`))
    (`SceneComponent.K2_SetRelativeLocation` (`StaticMeshActor.StaticMeshComponent` (`self.Room4 Fluid`)) (`KismetMathLibrary.MakeVector` _relativelocation_x _relativelocation_y (.z (`.Room4FluidLocation_49_B3F18BD64D5338F9FA8044A59CF3CF70` (break `/Game/HorrorEngine/Blueprints/Structures/SaveStructures/CharacterStatus` (`/Game/HorrorEngine/HorrorEngine.CharacterStatus` _asmaster))))) false false)
    (if (`self.ActorHasTag` "SecondValveRoom4")
      (`/Game/TestForMilestone/Blueprints/Room2/BP_Room4Fluid.Second Move Down` (`self.Room4 Fluid`))
      (else
        (`/Game/TestForMilestone/Blueprints/Room2/BP_Room4Fluid.First Move Down` (`self.Room4 Fluid`))))))

(fn `Update Game Progress`
  (bind _asmaster (`/Game/HorrorEngine/Blueprints/Core/HorrorEngineFunctions.GetPlayer`))
  (bind _characterstatus (`/Game/HorrorEngine/HorrorEngine.CharacterStatus` _asmaster))
  (bind _result (`/Engine/EditorBlueprintResources/StandardMacros.IncrementInt` (`.OpenedValve_44_404451FA4BA5A79D6A14F1BC3FF5ABBF` (break `/Game/HorrorEngine/Blueprints/Structures/SaveStructures/CharacterStatus` _characterstatus)))
    (:`  `
      (setmembers `/Game/HorrorEngine/Blueprints/Structures/SaveStructures/CharacterStatus` :`StructRef` _characterstatus :`OpenedValve` _result))))

(fn `UserConstructionScript`
  (`/Game/HorrorEngine/Blueprints/Core/HorrorEngineMacros.HM_DefaultConstructions` (`self.CreateNewHorrorEvent`))
  (`/Game/HorrorEngine/Blueprints/Core/HorrorEngineFunctions.SetMesh` (`self.Valve`) (`self.ValveMesh`))
  (`/Game/HorrorEngine/Blueprints/Core/HorrorEngineFunctions.PlayRate` (`self.ButtonTimeline`) (`self.Animation Speed (Sec)`))
  (`SceneComponent.K2_SetRelativeLocationAndRotation` (`self.ValvePivot`) (select `bool` (`self.On / Off`) :`false` (`self.OffLocation`) :`true` (`self.OnLocation`)) (select `bool` (`self.On / Off`) :`false` (`self.OffRotation`) :`true` (`self.OnRotation`)) false false))