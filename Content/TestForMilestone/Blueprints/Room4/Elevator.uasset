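; Elevator actor for Room 4 that travels up and down as a timed, eased movement.
; MovingUp and MovingDown each wait briefly, then move the Billboard component to the actor's location plus an up or down offset.
; Afterwards each flips IsAllowedUp and resets both elevator buttons, found with GetActorOfClass.
; The Open/On event is empty.
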(event `self.Open/On`
  (params (HorrorEvent :type Boolean)))

(event `MovingUp`
  (`KismetSystemLibrary.Delay` 4.0)
  (`KismetSystemLibrary.MoveComponentTo` (`self.Billboard`) (+ (`self.K2_GetActorLocation`) (`self.UpDistance`)) (struct) true true 15.0)
  (set `self.IsAllowedUp` false)
  (bind _returnvalue (`GameplayStatics.GetActorOfClass` "/Game/TestForMilestone/Blueprints/Room4/ButtonForElevator1.ButtonForElevator1_C"))
  (`/Game/TestForMilestone/Blueprints/Room4/ButtonForElevator1.Reset Button1` _returnvalue)
  (bind _returnvalue_2 (`GameplayStatics.GetActorOfClass` "/Game/TestForMilestone/Blueprints/Room4/ButtonForElevator2.ButtonForElevator2_C"))
  (`/Game/TestForMilestone/Blueprints/Room4/ButtonForElevator2.Reset Button2` _returnvalue_2))

(event `MovingDown`
  (`KismetSystemLibrary.Delay` 4.0)
  (`KismetSystemLibrary.MoveComponentTo` (`self.Billboard`) (+ (`self.K2_GetActorLocation`) (`self.DownDistance`)) (struct) true true 15.0)
  (set `self.IsAllowedUp` true)
  (bind _returnvalue (`GameplayStatics.GetActorOfClass` "/Game/TestForMilestone/Blueprints/Room4/ButtonForElevator2.ButtonForElevator2_C"))
  (`/Game/TestForMilestone/Blueprints/Room4/ButtonForElevator2.Reset Button2` _returnvalue)
  (bind _returnvalue_2 (`GameplayStatics.GetActorOfClass` "/Game/TestForMilestone/Blueprints/Room4/ButtonForElevator1.ButtonForElevator1_C"))
  (`/Game/TestForMilestone/Blueprints/Room4/ButtonForElevator1.Reset Button1` _returnvalue_2))

(fn `UserConstructionScript`)