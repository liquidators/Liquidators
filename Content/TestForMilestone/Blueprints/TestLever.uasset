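; Horror-engine lever that triggers the Room 2 radioactive waste hazard.
; Switching on lowers the entrance door, turns the room light red, resets its button and animates the lever by timeline with sounds.
; First use also raises fluid, re-allows the button, starts five waste phases and spawns delayed toxic sprays at hardcoded locations.
; On/off state supports save data; restoring an on lever replays the phases with zero delay.
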(event `ResetLever`
  (`self.Close/Off` false))

(event `self.Use`
  (params (HorrorEvent :type Boolean))
  (`/Game/HorrorEngine/Blueprints/Core/HorrorEngineMacros.HM_CheckInteraction`)
  (if (not (`self.On / Off`))
    (`self.Open/On` false)
    (if (not (`self.isTriggered`))
      (`self.Start Phases Movement` 1.0))))

(event `self.Open/On`
  (params (HorrorEvent :type Boolean))
  (bind _actorstouse (`self.ActorsToUse`))
  (bind _returnvalue (`GameplayStatics.GetActorOfClass` "/Game/TestForMilestone/Blueprints/E-DoorForRoom2Entrance.E-DoorForRoom2Entrance_C"))
  (`/Game/TestForMilestone/Blueprints/E-DoorForRoom2Entrance.Move Down` _returnvalue)
  (bind _returnvalue_2 (`GameplayStatics.GetActorOfClass` "/Game/TestForMilestone/Blueprints/ButtonForRoom2Entrance.ButtonForRoom2Entrance_C"))
  (`/Game/TestForMilestone/Blueprints/ButtonForRoom2Entrance.ResetButtom` _returnvalue_2)
  (bind _returnvalue_3 (`GameplayStatics.GetActorOfClass` "/Game/TestForMilestone/Blueprints/BP_PointLightRoom2.BP_PointLightRoom2_C"))
  (`/Game/TestForMilestone/Blueprints/BP_PointLightRoom2.Become Red` _returnvalue_3)
  ;[1 1 1] Open / Close Settings
  (`/Game/HorrorEngine/Blueprints/Core/HorrorEngineMacros.HM_CheckInteraction`)
  (if (not (`self.On / Off`))
    (if (not (`self.UseAfterAnimation`))
      (set `self.On / Off` true)
      (`self.Open/On` (`self.ActorsToUse`) false)
      (`self.HorrorEventCheck` "NewEnumerator3"))
    (set `self.InteractionEnabled` false)
    (`/Game/HorrorEngine/Blueprints/Core/HorrorEngineMacros.HM_3DSound` (`self.HitSound`) false (`self.TurnOnSound`) (`self.LeverPivot`) (`self.SoundAttenuation`))
    (`/Game/HorrorEngine/Blueprints/Core/HorrorEngineMacros.HM_3DSound` null false (`self.LoopSound`) (`self.LeverPivot`) (`self.SoundAttenuation`))
    (bind (_direction _animation) (`Timeline|ButtonTimeline` :!via `PlayFromStart` :!label _label)
      (:`Update`
        (`SceneComponent.K2_SetRelativeLocationAndRotation` (`self.LeverPivot`) (`KismetMathLibrary.VLerp` (`self.OffLocation`) (`self.OnLocation`) _animation) (`KismetMathLibrary.RLerp` (`self.OffRotation`) (`self.OnRotation`) _animation) false false))
      (:`Finished`
        (switch `ETimelineDirection` _direction
          (:`Forward`
            (if (`self.UseAfterAnimation`)
              (set `self.On / Off` true)
              (`self.Open/On` _actorstouse false)
              (`self.HorrorEventCheck` "NewEnumerator3")))
          (:`Backward`
            (if (`self.UseAfterAnimation`)
              (set `self.On / Off` false)
              (`self.Close/Off` _actorstouse false)
              (`self.HorrorEventCheck` "NewEnumerator4"))))
        (set `self.InteractionEnabled` true)
        (if (`self.StopSoundsAfterAnimation`)
          (`/Game/HorrorEngine/Blueprints/Core/HorrorEngineMacros.HM_StopAll3DSounds`))
        (`/Game/HorrorEngine/Blueprints/Core/HorrorEngineMacros.HM_3DSound` null false (`self.HitSound`) (`self.LeverPivot`) (`self.SoundAttenuation`))))))

(event `self.Close/Off`
  (params (HorrorEvent :type Boolean))
  ;[1 1 1] Open / Close Settings
  (`/Game/HorrorEngine/Blueprints/Core/HorrorEngineMacros.HM_CheckInteraction`)
  (if (`self.On / Off`)
    (if (not (`self.UseAfterAnimation`))
      (set `self.On / Off` false)
      (`self.Close/Off` (`self.ActorsToUse`) false)
      (`self.HorrorEventCheck` "NewEnumerator4"))
    (set `self.InteractionEnabled` false)
    (`/Game/HorrorEngine/Blueprints/Core/HorrorEngineMacros.HM_3DSound` (`self.HitSound`) false (`self.TurnOffSound`) (`self.LeverPivot`) (`self.SoundAttenuation`))
    (`/Game/HorrorEngine/Blueprints/Core/HorrorEngineMacros.HM_3DSound` null false (`self.LoopSound`) (`self.LeverPivot`) (`self.SoundAttenuation`))
    (goto _label :!via `ReverseFromEnd`)))

(event `/Game/HorrorEngine/Blueprints/Core/HorrorEngineInterface.CollectSaveData`
  ;[0 1 0.5572] Save Settings
  (bind _asmaster (`/Game/HorrorEngine/Blueprints/Core/HorrorEngineFunctions.GetPlayer`))
  (`KismetArrayLibrary.Array_Add` (`/Game/HorrorEngine/Blueprints/Core/HE_SaveGameComponent.AssetCache` (`/Game/HorrorEngine/HorrorEngine.HE_SaveGameComponent` _asmaster)) (make `/Game/HorrorEngine/Blueprints/Structures/SaveStructures/AssetsSave` (`KismetSystemLibrary.GetObjectName` self) (`self.On / Off`) false false false 0.0 0.0 0 "+00000000.00:00:00.000000000" "NewEnumerator0" (struct :`Actor` "NewEnumerator0" :`MeshSettings` (struct) :`InspectionSettings` (struct :`InspectionPivotLocation` (0.0 0.0 0.0) :`Takeable` true :`InspectionAnimation` true :`InspectionAnimationSpeedSec` 0.5 :`InspectionBeginRotation` (struct) :`InspectionBeginScale` 1.0 :`MinZoomScale` 1.0 :`MaxZoomScale` 2.0 :`RotationSpeed` 2.5 :`SlideSpeed` 1.0 :`MaxSlideValue` 10.0 :`ItemName` "NSLOCTEXT(\"[36F2CAC74962AB94CD79BF9209510EA0]\", \"777C3D4148A15E519C4571BDEEDDF0C6\", \"Item Name\")" :`ItemInformation` "NSLOCTEXT(\"[36F2CAC74962AB94CD79BF9209510EA0]\", \"7053CD694055B38929676082E13C15B2\", \"Item Information\")" :`ReadingText` "NSLOCTEXT(\"[36F2CAC74962AB94CD79BF9209510EA0]\", \"69CF35CA4D73DD02FE3964898BA4561F\", \"Reading Text\")" :`TakeButton` (struct :`ButtonText` "NSLOCTEXT(\"[36F2CAC74962AB94CD79BF9209510EA0]\", \"9782AB014987F70A3CAB9FB453E2BA82\", \"Take\")") :`ExamineButton` (struct :`ButtonText` "NSLOCTEXT(\"[36F2CAC74962AB94CD79BF9209510EA0]\", \"9C1ACFBE41D0AD5D2EE404AF9B0D397D\", \"Examine\")") :`ZoomSlideButton` (struct :`ButtonText` "NSLOCTEXT(\"[36F2CAC74962AB94CD79BF9209510EA0]\", \"3D1EA72A4FA8E5B992190A9169CEBEB5\", \"Zoom/Slide\")") :`DismissButton` (struct :`ButtonText` "NSLOCTEXT(\"[36F2CAC74962AB94CD79BF9209510EA0]\", \"0100FB8A4C9CA6E3168D50B9AB82CB16\", \"Dismiss\")")) :`InventorySettings` (struct :`StorageType` "NewEnumerator3" :`NumberofItemstoAddInventory` 1 :`Interactable` true :`InteractionButton` (struct :`ButtonText` "NSLOCTEXT(\"[36F2CAC74962AB94CD79BF9209510EA0]\", \"833BA7274E830F4A4D9D468571D13F65\", \"Use\")") :`SwitchButton` (struct :`ButtonText` "NSLOCTEXT(\"[36F2CAC74962AB94CD79BF9209510EA0]\", \"BD48DBD740E1769C2DBADCB2DBB815E3\", \"Switch\")") :`ZoomSlideButton` (struct :`ButtonText` "NSLOCTEXT(\"[36F2CAC74962AB94CD79BF9209510EA0]\", \"A177D65A4E5F22F1D11BF28F7C2C34CC\", \"Zoom/Slide\")") :`CloseInventoryButton` (struct :`ButtonText` "NSLOCTEXT(\"[36F2CAC74962AB94CD79BF9209510EA0]\", \"DC687B8B4323E2EDF7B1FB93B6F9E7D7\", \"Close\")")) :`Pistol_MeshSettingsTop` (struct) :`Vhs_CurrentTime` "+00000000.00:00:00.000000000"))))

(event `/Game/HorrorEngine/Blueprints/Core/HorrorEngineInterface.RestoreSaveData`
  (params (AssetSave :type "/Game/HorrorEngine/Blueprints/Structures/SaveStructures/AssetsSave Structure"))
  ;[0 1 0.5572] Save Settings
  (set `self.On / Off` (`.BooleanSlot01_63_ED79FB5D49E9ED6768D7AE96EDFDE8DB` (break `/Game/HorrorEngine/Blueprints/Structures/SaveStructures/AssetsSave` AssetSave)))
  (`SceneComponent.K2_SetRelativeLocationAndRotation` (`self.LeverPivot`) (select `bool` (`self.On / Off`) :`false` (`self.OffLocation`) :`true` (`self.OnLocation`)) (select `bool` (`self.On / Off`) :`false` (`self.OffRotation`) :`true` (`self.OnRotation`)) false false)
  (if (`self.On / Off`)
    (`self.Start Phases Movement` 0.0)))

(fn `UserConstructionScript`
  (`/Game/HorrorEngine/Blueprints/Core/HorrorEngineMacros.HM_DefaultConstructions` (`self.CreateNewHorrorEvent`))
  (`/Game/HorrorEngine/Blueprints/Core/HorrorEngineFunctions.SetMesh` (`self.LeverBase`) (`self.LeverBaseMesh`))
  (`/Game/HorrorEngine/Blueprints/Core/HorrorEngineFunctions.SetMesh` (`self.Lever`) (`self.LeverMesh`))
  (`/Game/HorrorEngine/Blueprints/Core/HorrorEngineFunctions.PlayRate` (`self.ButtonTimeline`) (`self.Animation Speed (Sec)`))
  (`SceneComponent.K2_SetRelativeLocationAndRotation` (`self.LeverPivot`) (select `bool` (`self.On / Off`) :`false` (`self.OffLocation`) :`true` (`self.OnLocation`)) (select `bool` (`self.On / Off`) :`false` (`self.OffRotation`) :`true` (`self.OnRotation`)) false false))