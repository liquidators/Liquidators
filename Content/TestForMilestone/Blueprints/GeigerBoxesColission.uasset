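; Detection-box actor for the player's Geiger counter that warns of nearby waste actors (Bwaste_MASTER).
; On BeginPlay it snaps onto the player pawn and caches the counter reference, though detection looks the counter up again.
; Every Tick, InnerBoxDetection polls overlaps on the inner front boxes.
; Each overlapping waste actor triggers the counter's matching center, left or right fast blink.
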(event `self.ReceiveBeginPlay`
  (`self.K2_AttachToActor` (`GameplayStatics.GetPlayerPawn` 0) "None" "SnapToTarget" "SnapToTarget" "SnapToTarget")
  (bind _asmy_character (cast `/Game/TestForMilestone/Blueprints/MyCharacter` (`GameplayStatics.GetPlayerPawn` 0)))
  (set `self.BP_GeigerCounterRef` (`/Game/GeigerCounter/Blueprints/BP_GeigerCounterComponent.BP_GeigerCounter` (`/Game/TestForMilestone/Blueprints/MyCharacter.BP_GeigerCounterComponent` _asmy_character))))

(event `InnerBoxDetection`
  (`|ExecutionSequence`
    (:`then_0`
      ;[1 1 1] Inner Front Center Box
      (for _array_element (`PrimitiveComponent.GetOverlappingActors` (`self.01`) "/Game/TestForMilestone/Blueprints/Room1Hazards/Bwaste_MASTER.Bwaste_MASTER_C")
        (bind _asmy_character (cast `/Game/TestForMilestone/Blueprints/MyCharacter` (`GameplayStatics.GetPlayerPawn` 0)))
        (`/Game/GeigerCounter/Blueprints/BP_GeigerCounter.Front Center Fast Blink` (`/Game/GeigerCounter/Blueprints/BP_GeigerCounterComponent.BP_GeigerCounter` (`/Game/TestForMilestone/Blueprints/MyCharacter.BP_GeigerCounterComponent` _asmy_character)))))
    (:`then_1`
      ;[1 1 1] Inner Front Left Box
      (for _array_element_2 (`PrimitiveComponent.GetOverlappingActors` (`self.-11`) "/Game/TestForMilestone/Blueprints/Room1Hazards/Bwaste_MASTER.Bwaste_MASTER_C")
        (bind _asmy_character_2 (cast `/Game/TestForMilestone/Blueprints/MyCharacter` (`GameplayStatics.GetPlayerPawn` 0)))
        (`/Game/GeigerCounter/Blueprints/BP_GeigerCounter.Front Left Fast Blink` (`/Game/GeigerCounter/Blueprints/BP_GeigerCounterComponent.BP_GeigerCounter` (`/Game/TestForMilestone/Blueprints/MyCharacter.BP_GeigerCounterComponent` _asmy_character_2)))))
    (:`then_2`
      ;[1 1 1] Inner Front Right Box
      (for _array_element_3 (`PrimitiveComponent.GetOverlappingActors` (`self.11`) "/Game/TestForMilestone/Blueprints/Room1Hazards/Bwaste_MASTER.Bwaste_MASTER_C")
        (bind _asmy_character_3 (cast `/Game/TestForMilestone/Blueprints/MyCharacter` (`GameplayStatics.GetPlayerPawn` 0)))
        (`/Game/GeigerCounter/Blueprints/BP_GeigerCounter.Front Right Fast Blink` (`/Game/GeigerCounter/Blueprints/BP_GeigerCounterComponent.BP_GeigerCounter` (`/Game/TestForMilestone/Blueprints/MyCharacter.BP_GeigerCounterComponent` _asmy_character_3)))))))

(event `self.ReceiveTick`
  (params (DeltaSeconds :type "Float (single-precision)"))
  (`|ExecutionSequence`
    (:`then_0`
      (`self.InnerBoxDetection`))))

(fn `UserConstructionScript`)