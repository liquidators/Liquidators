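; Player-attached detector that drives the character's Geiger counter by sensing Bwaste_MASTER actors in inner and outer directional boxes.
; Each Tick it polls front, back, left and right overlaps: inner hits fast-blink that light, outer-only hits slow-blink it, empty outer boxes switch it off.
; Overlap totals start one inner or outer beep through DoOnce gates, with inner taking priority.
; Diagonal-box logic exists but is disconnected.
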(event `Attach Detection Box`
  (`self.K2_AttachToActor` (`GameplayStatics.GetPlayerPawn` 0) "None" "SnapToTarget" "SnapToTarget" "SnapToTarget" :!label _label))

(event `self.ReceiveBeginPlay`
  (goto _label))

(event `InnerBoxDetection`
  (bind _overlappingactors (`PrimitiveComponent.GetOverlappingActors` (`self.InnerLeftCenter`) "/Game/TestForMilestone/Blueprints/Room1Hazards/Bwaste_MASTER.Bwaste_MASTER_C"))
  (bind _overlappingactors_2 (`PrimitiveComponent.GetOverlappingActors` (`self.InnerFrontCenter`) "/Game/TestForMilestone/Blueprints/Room1Hazards/Bwaste_MASTER.Bwaste_MASTER_C"))
  (bind _overlappingactors_3 (`PrimitiveComponent.GetOverlappingActors` (`self.InnerBackCenter`) "/Game/TestForMilestone/Blueprints/Room1Hazards/Bwaste_MASTER.Bwaste_MASTER_C"))
  (bind _overlappingactors_4 (`PrimitiveComponent.GetOverlappingActors` (`self.InnerRightCenter`) "/Game/TestForMilestone/Blueprints/Room1Hazards/Bwaste_MASTER.Bwaste_MASTER_C"))
  (`|ExecutionSequence`
    (:`then_0`
      ;[1 1 1] Inner Front Center Box
      (if (== (`KismetArrayLibrary.Array_Length` _overlappingactors_2) 0)
        (set `self.InnerFC` false)
        (else
          (for _ _overlappingactors_2
            (`/Game/GeigerCounter/Blueprints/BP_GeigerCounter.Front Center Fast Blink` (`self.BP_GeigerCounterRef`))
            (set `self.InnerFC` true)))))
    (:`then_3`
      ;[1 1 1] Inner Left Center Box
      (if (== (`KismetArrayLibrary.Array_Length` _overlappingactors) 0)
        (set `self.InnerLC` false)
        (else
          (for _ _overlappingactors
            (`/Game/GeigerCounter/Blueprints/BP_GeigerCounter.Left Center Fast Blink` (`self.BP_GeigerCounterRef`))
            (set `self.InnerLC` true)))))
    (:`then_4`
      ;[1 1 1] Inner Right Center Box
      (if (== (`KismetArrayLibrary.Array_Length` _overlappingactors_4) 0)
        (set `self.InnerRC` false)
        (else
          (for _ _overlappingactors_4
            (`/Game/GeigerCounter/Blueprints/BP_GeigerCounter.Right Center Fast Blink` (`self.BP_GeigerCounterRef`))
            (set `self.InnerRC` true)))))
    (:`then_5`
      ;[1 1 1] Inner Back Center Box
      (if (== (`KismetArrayLibrary.Array_Length` _overlappingactors_3) 0)
        (set `self.InnerBC` false)
        (else
          (for _ _overlappingactors_3
            (`/Game/GeigerCounter/Blueprints/BP_GeigerCounter.Back Center Fast Blink` (`self.BP_GeigerCounterRef`))
            (set `self.InnerBC` true)))))))

(event `self.ReceiveTick`
  (params (DeltaSeconds :type "Float (single-precision)"))
  (`self.Set Geiger Counter`)
  (`|ExecutionSequence`
    (:`then_0`
      (`self.InnerBoxDetection`)
      (`self.OuterBoxDetection`))
    (:`then_2`
      (`self.Set Inner Beeping`)
      (`self.Set Outer Beeping`))))

(event `OuterBoxDetection`
  (bind _overlappingactors (`PrimitiveComponent.GetOverlappingActors` (`self.OuterFrontCenter`) "/Game/TestForMilestone/Blueprints/Room1Hazards/Bwaste_MASTER.Bwaste_MASTER_C"))
  (bind _overlappingactors_2 (`PrimitiveComponent.GetOverlappingActors` (`self.OuterLeftCenter`) "/Game/TestForMilestone/Blueprints/Room1Hazards/Bwaste_MASTER.Bwaste_MASTER_C"))
  (bind _overlappingactors_3 (`PrimitiveComponent.GetOverlappingActors` (`self.OuterRightCenter`) "/Game/TestForMilestone/Blueprints/Room1Hazards/Bwaste_MASTER.Bwaste_MASTER_C"))
  (bind _overlappingactors_4 (`PrimitiveComponent.GetOverlappingActors` (`self.OuterBackCenter`) "/Game/TestForMilestone/Blueprints/Room1Hazards/Bwaste_MASTER.Bwaste_MASTER_C"))
  (`|ExecutionSequence`
    (:`then_0`
      ;[1 1 1] Outer Front Center Box
      (if (== (`KismetArrayLibrary.Array_Length` _overlappingactors) 0)
        (`/Game/GeigerCounter/Blueprints/BP_GeigerCounter.Front Center Off` (`self.BP_GeigerCounterRef`))
        (else
          (for _ _overlappingactors
            (if (not (`self.InnerFC`))
              (`/Game/GeigerCounter/Blueprints/BP_GeigerCounter.Front Center Slow Blink` (`self.BP_GeigerCounterRef`)))))))
    (:`then_3`
      ;[1 1 1] Outer Left Center Box
      (if (== (`KismetArrayLibrary.Array_Length` _overlappingactors_2) 0)
        (`/Game/GeigerCounter/Blueprints/BP_GeigerCounter.Left Center Off` (`self.BP_GeigerCounterRef`))
        (else
          (for _ _overlappingactors_2
            (if (not (`self.InnerLC`))
              (`/Game/GeigerCounter/Blueprints/BP_GeigerCounter.Left Center Slow Blink` (`self.BP_GeigerCounterRef`)))))))
    (:`then_4`
      ;[1 1 1] Outer Right Center Box
      (if (== (`KismetArrayLibrary.Array_Length` _overlappingactors_3) 0)
        (`/Game/GeigerCounter/Blueprints/BP_GeigerCounter.Right Center Off` (`self.BP_GeigerCounterRef`))
        (else
          (for _ _overlappingactors_3
            (if (not (`self.InnerRC`))
              (`/Game/GeigerCounter/Blueprints/BP_GeigerCounter.Right Center Slow Blink` (`self.BP_GeigerCounterRef`)))))))
    (:`then_5`
      ;[1 1 1] Outer Back Center Box
      (if (== (`KismetArrayLibrary.Array_Length` _overlappingactors_4) 0)
        (`/Game/GeigerCounter/Blueprints/BP_GeigerCounter.Back Center Off` (`self.BP_GeigerCounterRef`))
        (else
          (for _ _overlappingactors_4
            (if (not (`self.InnerBC`))
              (`/Game/GeigerCounter/Blueprints/BP_GeigerCounter.Back Center Slow Blink` (`self.BP_GeigerCounterRef`)))))))))

(event `Set Geiger Counter`
  (bind _asmy_character (cast `/Game/TestForMilestone/Blueprints/MyCharacter` (`GameplayStatics.GetPlayerPawn` 0)))
  (set `self.BP_GeigerCounterRef` (`/Game/GeigerCounter/Blueprints/BP_GeigerCounterComponent.BP_GeigerCounter` (`/Game/TestForMilestone/Blueprints/MyCharacter.BP_GeigerCounterComponent` _asmy_character))))

(event `Set Inner Beeping`
  (bind _innertotaldetection (`self.InnerTotalDetection`))
  ;[1 1 1] Inner beeping sound set
  (set `self.InnerTotalDetection` 0)
  (for _array_element (`|MakeArray` (`self.InnerRightCenter`) (`self.InnerBackCenter`) (`self.InnerLeftCenter`) (`self.InnerFrontCenter`))
    (set `self.InnerTotalDetection` (+ _innertotaldetection (`KismetArrayLibrary.Array_Length` (`PrimitiveComponent.GetOverlappingActors` _array_element "/Game/TestForMilestone/Blueprints/Room1Hazards/Bwaste_MASTER.Bwaste_MASTER_C")))))
  (if (> _innertotaldetection 0)
    (set `self.InnerSoundOn` true)
    (`/Engine/EditorBlueprintResources/StandardMacros.DoOnce` false :!label _label_2
      (:`Completed`
        (bind _returnvalue (`GameplayStatics.SpawnSound2D` (`self.innerBeep`) 1.0 1.0 0.0 null))
        (set `self.inner beep sound` _returnvalue)))
    (else
      (set `self.InnerSoundOn` false)
      (if (`KismetSystemLibrary.IsValid` (`self.inner beep sound`))
        (`AudioComponent.Stop` (`self.inner beep sound`))
        (goto _label_2 :!via `Reset`)
        (else
          (goto _label_2 :!via `Reset`))))))

(event `Set Outer Beeping`
  (bind _inner_beep_sound (`self.inner beep sound`))
  (bind _outerbeepsound (`self.OuterBeepSound`))
  (bind _outertotaldetection (`self.OuterTotalDetection`))
  (bind _outerbeepsound_2 (`self.OuterBeepSound`))
  ;[1 1 1] Outer beeping sound set
  (set `self.OuterTotalDetection` 0)
  (for _array_element (`|MakeArray` (`self.OuterFrontCenter`) (`self.OuterRightCenter`) (`self.OuterBackCenter`) (`self.OuterLeftCenter`))
    (set `self.OuterTotalDetection` (+ _outertotaldetection (`KismetArrayLibrary.Array_Length` (`PrimitiveComponent.GetOverlappingActors` _array_element "/Game/TestForMilestone/Blueprints/Room1Hazards/Bwaste_MASTER.Bwaste_MASTER_C")))))
  (if (> _outertotaldetection 0)
    (if (`self.InnerSoundOn`)
      (if (`KismetSystemLibrary.IsValid` _outerbeepsound)
        (`AudioComponent.Stop` _outerbeepsound)
        (`self.ResetOuterPeepingSound`))
      (else
        (if (`KismetSystemLibrary.IsValid` _inner_beep_sound)
          (`AudioComponent.Stop` _inner_beep_sound))
        (`/Engine/EditorBlueprintResources/StandardMacros.DoOnce` false :!label _label_3
          (:`Completed`
            (bind _returnvalue (`GameplayStatics.SpawnSound2D` (`self.outerBeep`) 1.0 1.0 0.0 null))
            (set `self.OuterBeepSound` _returnvalue)))))
    (elif (`KismetSystemLibrary.IsValid` _outerbeepsound_2)
      (`AudioComponent.Stop` _outerbeepsound_2)
      (`self.ResetOuterPeepingSound`))))

(event `ResetOuterPeepingSound`
  ;[1 1 1] Outer beeping sound set
  (goto _label_3 :!via `Reset`))

(fn `UserConstructionScript`)