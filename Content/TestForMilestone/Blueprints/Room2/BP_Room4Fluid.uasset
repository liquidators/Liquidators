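; Fluid volume for Room 4 that tracks when the player is in or under it, drowns them after prolonged submersion, and can lower in two timed stages.
; A looping timer checks box overlap and camera height, using DoOnce gates to update player speed and submerge state.
; The BlurStart timeline drives sounds-accompanied, tag-found Chameleon post-process effects, triggering death at full value and reversing faster on surfacing.
; Tick copies the fluid's location into the player's CharacterStatus.
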(event `Update Water Visuals`
  (params (UnderWaterTimer :type "Float (double-precision)"))
  (set `self.UnderWaterTimer` UnderWaterTimer)
  (`self.Underwater Visuals`)
  (`self.ToggleOffUnderWaterEffect`)
  (if (>= (`self.UnderWaterTimer`) 1.0)
    (`self.TriggerDeath`)))

(event `self.ReceiveBeginPlay`
  (bind (_relativelocation_x _relativelocation_y _relativelocation_z) (`KismetMathLibrary.BreakVector` (`SceneComponent.RelativeLocation` (`self.StaticMeshComponent`))))
  (bind _returnvalue (- _relativelocation_z 400.0))
  (`|ExecutionSequence`
    (:`then_0`
      (bind _outactors (`GameplayStatics.GetAllActorsWithTag` "UnderWaterEffect"))
      (set `self.UnderWaterEffect` (cast `/Game/Chameleon/Chameleon` (`|GetArrayItem` _outactors) :!pure true))
      (`KismetSystemLibrary.K2_SetTimerDelegate` (delegate `UnderWater`) 0.2 true))
    (:`then_1`
      (bind _outactors_2 (`GameplayStatics.GetAllActorsWithTag` "UnderWaterBlur"))
      (set `self.UnderwaterBlur` (cast `/Game/Chameleon/Chameleon` (`|GetArrayItem` _outactors_2) :!pure true)))
    (:`then_2`
      (bind _outactors_3 (`GameplayStatics.GetAllActorsWithTag` "UnderWaterFlare"))
      (set `self.UnderwaterFlare` (cast `/Game/Chameleon/Chameleon` (`|GetArrayItem` _outactors_3) :!pure true)))
    (:`then_3`
      (bind _outactors_4 (`GameplayStatics.GetAllActorsWithTag` "UnderWaterBlue"))
      (set `self.UnderwaterBlue` (cast `/Game/Chameleon/Chameleon` (`|GetArrayItem` _outactors_4) :!pure true))
      (bind _asmaster (`/Game/HorrorEngine/Blueprints/Core/HorrorEngineFunctions.GetPlayer`))
      (setmembers `/Game/HorrorEngine/Blueprints/Structures/SaveStructures/CharacterStatus` :`StructRef` (`/Game/HorrorEngine/HorrorEngine.CharacterStatus` _asmaster) :`Room4FluidLocation` (`SceneComponent.RelativeLocation` (`self.StaticMeshComponent`)))
      (set `self.InitialLocationZ` _relativelocation_z)
      (set `self.FirstTargetLocationZ` _returnvalue)
      (set `self.SecondTargetLocationZ` (- _returnvalue 400.0)))))

(event `StartUnderWaterVisualEffect`
  (set `self.UnderwaterOrNot` true)
  (set `self.IsTriggered` true)
  (`GameplayStatics.PlaySound2D` "/Game/Sounds3/Underwater/Underwater_Submerge_Cue.Underwater_Submerge_Cue" 1.0 1.0 0.0 null null)
  (`TimelineComponent.SetPlayRate` (`self.Blur Start`) (* 1.0 1.0))
  (set `/Game/Chameleon/Chameleon.Unbound` true (`self.UnderWaterEffect`))
  (set `/Game/Chameleon/Chameleon.Unbound` true (`self.UnderwaterFlare`))
  (set `/Game/Chameleon/Chameleon.Unbound` true (`self.UnderwaterBlur`))
  (bind _returnvalue (`GameplayStatics.SpawnSound2D` "/Game/Sounds3/Underwater/Underwater_White_Noise_Cue.Underwater_White_Noise_Cue" 1.0 1.0 0.0 null))
  (set `self.WhiteSound` _returnvalue)
  (bind (_direction _newtrack_0) (`Timeline|Blur Start` :!via `PlayFromStart` :!label _label)
    (:`Update`
      (`self.Update Water Visuals` _newtrack_0))))

(event `Start In Water Walk`
  (goto _label_2 :!via `Reset`))

(event `Reset Start Underwater`
  (goto _label_3 :!via `Reset`))

(event `UnderWater`
  (bind (_returnvalue_x _returnvalue_y _returnvalue_z) (`KismetMathLibrary.BreakVector` (`self.K2_GetActorLocation`)))
  (bind (_returnvalue_x_2 _returnvalue_y_2 _returnvalue_z_2) (`KismetMathLibrary.BreakVector` (`PlayerCameraManager.GetCameraLocation` (`GameplayStatics.GetPlayerCameraManager` 0))))
  (if (`PrimitiveComponent.IsOverlappingActor` (`self.Box`) (`GameplayStatics.GetPlayerPawn` 0))
    (`|ExecutionSequence`
      (:`then_0`
        (`/Engine/EditorBlueprintResources/StandardMacros.DoOnce` false :!label _label_2
          (:`Completed`
            (set `self.IsInWater` true)
            (bind _asmaster (`/Game/HorrorEngine/Blueprints/Core/HorrorEngineFunctions.GetPlayer`))
            (`/Game/HorrorEngine/HorrorEngine.CalculateSpeed` _asmaster)
            (`self.Stop In Water Walk`))))
      (:`then_1`
        (if (> (+ _returnvalue_z 5.0) _returnvalue_z_2)
          (`/Engine/EditorBlueprintResources/StandardMacros.DoOnce` false :!label _label_3
            (:`Completed`
              (`self.StartUnderWaterVisualEffect`)
              (`self.Reset Stop Underwater`)
              (set `self.IsUnderWater` true)
              (bind _asmaster_2 (`/Game/HorrorEngine/Blueprints/Core/HorrorEngineFunctions.GetPlayer`))
              (`/Game/HorrorEngine/HorrorEngine.CalculateSpeed` _asmaster_2)))
          (else
            (`/Engine/EditorBlueprintResources/StandardMacros.DoOnce` false :!label _label_4
              (:`Completed`
                (`self.StopUnderWaterVisualEffect`)
                (`self.Reset Start Underwater`)
                (set `self.IsUnderWater` false)
                (bind _asmaster_3 (`/Game/HorrorEngine/Blueprints/Core/HorrorEngineFunctions.GetPlayer`))
                (`/Game/HorrorEngine/HorrorEngine.CalculateSpeed` _asmaster_3)))))))
    (else
      (`/Engine/EditorBlueprintResources/StandardMacros.DoOnce` false :!label _label_5
        (:`Completed`
          (set `self.IsInWater` false)
          (bind _asmaster_4 (`/Game/HorrorEngine/Blueprints/Core/HorrorEngineFunctions.GetPlayer`))
          (`/Game/HorrorEngine/HorrorEngine.CalculateSpeed` _asmaster_4)
          (`self.Start In Water Walk`))))))

(event `Reset Stop Underwater`
  (goto _label_4 :!via `Reset`))

(event `Stop In Water Walk`
  (goto _label_5 :!via `Reset`))

(event `StopUnderWaterVisualEffect`
  (bind _whitesound (`self.WhiteSound`))
  (set `self.UnderwaterOrNot` false)
  (if (`self.IsTriggered`)
    (if (`KismetSystemLibrary.IsValid` _whitesound)
      (`AudioComponent.Stop` _whitesound)
      (`GameplayStatics.PlaySound2D` "/Game/Sounds3/Underwater/Underwater_RiseToSurface_Cue.Underwater_RiseToSurface_Cue" 1.0 1.0 0.0 null null)
      (set `/Game/Chameleon/Chameleon.Unbound` false (`self.UnderwaterBlue`) :!label _label_6)
      (`TimelineComponent.SetPlayRate` (`self.Blur Start`) (* 1.0 4.0))
      (goto _label :!via `Reverse`))
    (else
      (goto _label_6))))

(event `First Move Down`
  (bind _staticmeshcomponent (`self.StaticMeshComponent`))
  (bind (_relativelocation_x _relativelocation_y) (`KismetMathLibrary.BreakVector` (`SceneComponent.RelativeLocation` _staticmeshcomponent)))
  (bind (_relativelocation_x_2 _relativelocation_y_2 _relativelocation_z) (`KismetMathLibrary.BreakVector` (`SceneComponent.RelativeLocation` (`self.StaticMeshComponent`))))
  (if (> _relativelocation_z (`self.FirstTargetLocationZ`))
    (`KismetSystemLibrary.MoveComponentTo` _staticmeshcomponent (`KismetMathLibrary.MakeVector` _relativelocation_x _relativelocation_y (`self.FirstTargetLocationZ`)) (struct) false false 10.0)))

(event `Second Move Down`
  (bind _staticmeshcomponent (`self.StaticMeshComponent`))
  (bind (_relativelocation_x _relativelocation_y _relativelocation_z) (`KismetMathLibrary.BreakVector` (`SceneComponent.RelativeLocation` (`self.StaticMeshComponent`))))
  (bind (_relativelocation_x_2 _relativelocation_y_2) (`KismetMathLibrary.BreakVector` (`SceneComponent.RelativeLocation` _staticmeshcomponent)))
  (if (> _relativelocation_z (`self.SecondTargetLocationZ`))
    (`KismetSystemLibrary.MoveComponentTo` _staticmeshcomponent (`KismetMathLibrary.MakeVector` _relativelocation_x_2 _relativelocation_y_2 (`self.SecondTargetLocationZ`)) (struct) false false 10.0)))

(event `self.ReceiveTick`
  (params (DeltaSeconds :type "Float (single-precision)"))
  (bind _asmaster (`/Game/HorrorEngine/Blueprints/Core/HorrorEngineFunctions.GetPlayer`))
  (setmembers `/Game/HorrorEngine/Blueprints/Structures/SaveStructures/CharacterStatus` :`StructRef` (`/Game/HorrorEngine/HorrorEngine.CharacterStatus` _asmaster) :`Room4FluidLocation` (`SceneComponent.RelativeLocation` (`self.StaticMeshComponent`))))

(fn `ToggleOffUnderWaterEffect`
  (if (<= (`self.UnderWaterTimer`) 0.0)
    (set `/Game/Chameleon/Chameleon.Unbound` false (`self.UnderWaterEffect`))
    (set `/Game/Chameleon/Chameleon.Unbound` false (`self.UnderwaterFlare`))
    (set `/Game/Chameleon/Chameleon.Unbound` false (`self.UnderwaterBlur`))
    (else
      (set `/Game/Chameleon/Chameleon.Unbound` true (`self.UnderWaterEffect`))
      (set `/Game/Chameleon/Chameleon.Unbound` true (`self.UnderwaterFlare`))
      (set `/Game/Chameleon/Chameleon.Unbound` true (`self.UnderwaterBlur`)))))

(fn `Underwater Visuals`
  (bind _underwatereffect (`self.UnderWaterEffect`))
  (bind _returnvalue (`KismetMathLibrary.MapRangeClamped` (`self.UnderWaterTimer`) 0.0 1.0 0.0 25.0))
  (bind (_r _g _b) (`KismetMathLibrary.BreakColor` (`KismetMathLibrary.LinearColorLerp` (struct :`R` 1.0 :`G` 1.0 :`B` 1.0 :`A` 1.0) (struct :`R` 1.0 :`G` 0.680619 :`B` 0.667 :`A` 1.0) (`self.UnderWaterTimer`))))
  (setmembers `PostProcessSettings` :`StructRef` (`/Game/Chameleon/Chameleon.Native Post Process` (`self.UnderWaterEffect`)) :`ColorGammaMidtones` (`KismetMathLibrary.MakeVector4` _r _g _b 1.0))
  ;[1 1 1] Wavy Displacement
  (set `/Game/Chameleon/Chameleon.Screen Waves X Tiling` _returnvalue _underwatereffect)
  (set `/Game/Chameleon/Chameleon.Screen Waves Y Tiling` _returnvalue _underwatereffect)
  ;[1 1 1] underwater blur
  (set `/Game/Chameleon/Chameleon.Blur Amount` (`KismetMathLibrary.MapRangeClamped` (`self.UnderWaterTimer`) 0.0 1.0 1.0 1.0) (`self.UnderwaterBlur`))
  ;[1 1 1] Underwater Flare
  (set `/Game/Chameleon/Chameleon.Anamorphic Lens Flares Intensity` (`KismetMathLibrary.MapRangeClamped` (`self.UnderWaterTimer`) 0.0 1.0 0.1 8.0) (`self.UnderwaterFlare`))
  ;[1 1 1] Darkenning
  (setmembers `PostProcessSettings` :`StructRef` (`/Game/Chameleon/Chameleon.Native Post Process` (`self.UnderWaterEffect`)) :`AutoExposureBias` (`KismetMathLibrary.MapRangeClamped` (`self.UnderWaterTimer`) 0.0 1.0 0.0 -1.0)))

(fn `UserConstructionScript`)