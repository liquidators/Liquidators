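; BP_ConstructionLight is a construction light prop for Room2 that switches a spotlight on and off.
; The SpotLight starts hidden at BeginPlay, and the Open/On and Close/Off events show or hide it.
; The construction script enables physics simulation on the static mesh when the Physics flag is set.
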(event `self.ReceiveBeginPlay`
  (`SceneComponent.SetVisibility` (`self.SpotLight`) false false))

(event `self.Open/On`
  (params (HorrorEvent :type Boolean))
  (`SceneComponent.SetVisibility` (`self.SpotLight`) true false))

(event `self.Close/Off`
  (params (HorrorEvent :type Boolean))
  (`SceneComponent.SetVisibility` (`self.SpotLight`) false false))

(fn `UserConstructionScript`
  (if (`self.Physics_?`)
    (`PrimitiveComponent.SetSimulatePhysics` (`self.StaticMesh`) true)))