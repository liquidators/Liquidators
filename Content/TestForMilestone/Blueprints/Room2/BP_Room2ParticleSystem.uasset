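; BP_Room2ParticleSystem is a Room 2 Blueprint that switches a group of nine waterfall effects on and off together.
; It deactivates all of them on BeginPlay, so the waterfalls start switched off.
; Two custom events, ActivatetheParticle and DeactivatetheParticle, activate the whole group with a reset or deactivate it, with no triggering logic inside this Blueprint.
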(event `self.ReceiveBeginPlay`
  (`self.Deactivate the Particle`))

(event `Deactivate the Particle`
  (`ActorComponent.Deactivate` (`self.waterfall1`))
  (`ActorComponent.Deactivate` (`self.waterfall2`))
  (`ActorComponent.Deactivate` (`self.waterfall3`))
  (`ActorComponent.Deactivate` (`self.waterfall4`))
  (`ActorComponent.Deactivate` (`self.waterfall5`))
  (`ActorComponent.Deactivate` (`self.waterfall66`))
  (`ActorComponent.Deactivate` (`self.waterfall77`))
  (`ActorComponent.Deactivate` (`self.waterfall88`))
  (`ActorComponent.Deactivate` (`self.waterfall99`)))

(event `Activate the Particle`
  (`ActorComponent.Activate` (`self.waterfall1`) true)
  (`ActorComponent.Activate` (`self.waterfall2`) true)
  (`ActorComponent.Activate` (`self.waterfall3`) true)
  (`ActorComponent.Activate` (`self.waterfall4`) true)
  (`ActorComponent.Activate` (`self.waterfall5`) true)
  (`ActorComponent.Activate` (`self.waterfall66`) true)
  (`ActorComponent.Activate` (`self.waterfall77`) true)
  (`ActorComponent.Activate` (`self.waterfall88`) true)
  (`ActorComponent.Activate` (`self.waterfall99`) true))

(fn `UserConstructionScript`)