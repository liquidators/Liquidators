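; Room 1 hazard actor that repeatedly damages the player while they overlap it, flagged as waste contact.
; On overlap it flags the character as touching a hazard and starts BurnMF, which deals damage and re-calls itself after a delay while Burning is set.
; A timed IfOverlap gate blocks rapid retriggering.
; Leaving clears the burning and contact flags and sets the character's walk speed to a fixed value.
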(event `self.ReceiveActorBeginOverlap`
  (params (OtherActor :type "Actor Object Reference"))
  ;[1 1 1] New Damage Trigger
  (if (== OtherActor (`GameplayStatics.GetPlayerPawn` 0))
    (if (not (`self.If Overlap`))
      (set `self.Burning` true)
      (`self.Burn MF`)
      (bind _asmy_character (cast `/Game/TestForMilestone/Blueprints/MyCharacter` (`GameplayStatics.GetPlayerCharacter` 0)))
      (set `/Game/TestForMilestone/Blueprints/MyCharacter.OverlappingHazard` true _asmy_character)
      (set `self.If Overlap` true)
      (`KismetSystemLibrary.Delay` 2.0)
      (set `self.If Overlap` false))))

(event `self.ReceiveActorEndOverlap`
  (params (OtherActor :type "Actor Object Reference"))
  ;[1 1 1] New Damage Trigger
  (if (== OtherActor (`GameplayStatics.GetPlayerPawn` 0))
    (set `self.Burning` false)
    (bind _asmy_character (cast `/Game/TestForMilestone/Blueprints/MyCharacter` (`GameplayStatics.GetPlayerCharacter` 0)))
    (set `/Game/TestForMilestone/Blueprints/MyCharacter.OverlappingHazard` false _asmy_character)
    (set `CharacterMovementComponent.MaxWalkSpeed` 150.0 (`Character.CharacterMovement` _asmy_character))
    (bind _asmaster (`/Game/HorrorEngine/Blueprints/Core/HorrorEngineFunctions.GetPlayer`))
    (set `/Game/HorrorEngine/HorrorEngine.IsCollidingWaste` false _asmaster)))

(event `Burn MF`
  ;[1 1 1] New Damage Trigger
  (if (`self.Burning`)
    (bind _asmaster (`/Game/HorrorEngine/Blueprints/Core/HorrorEngineFunctions.GetPlayer`))
    (set `/Game/HorrorEngine/HorrorEngine.IsCollidingWaste` true _asmaster)
    (`/Game/HorrorEngine/HorrorEngine.GetDamage` :`self` _asmaster :`DamagePoint` 20.0)
    (`KismetSystemLibrary.Delay` 2.0)
    (`self.Burn MF`)))

(fn `UserConstructionScript`)