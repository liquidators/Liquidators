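; Player pawn for a test level that can pick up and carry physics objects and toggle a Geiger counter.
; F traces a short ray from the camera and grabs a simulating component under a mass limit with a PhysicsHandle, or releases the one held.
; Tick keeps the handle's target at the HeldObjLocation component so the object follows the player.
; R flip-flops the Geiger counter component on and off.
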(event `self.ReceiveTick`
  (params (DeltaSeconds :type "Float (single-precision)"))
  (`PhysicsHandleComponent.SetTargetLocation` (`self.PhysicsHandle`) (`SceneComponent.K2_GetComponentLocation` (`self.HeldObjLocation`))))

(event `Key|R`
  (params (Key :type "Key Structure"))
  (bind _bp_geigercountercomponent (`self.BP_GeigerCounterComponent`))
  (:`Pressed`
    (`/Engine/EditorBlueprintResources/StandardMacros.FlipFlop`
      (:`A`
        (`/Game/GeigerCounter/Blueprints/BP_GeigerCounterComponent.SwitchOn` _bp_geigercountercomponent))
      (:`B`
        (`/Game/GeigerCounter/Blueprints/BP_GeigerCounterComponent.SwitchOff` _bp_geigercountercomponent)))))

(event `Key|F`
  (params (Key :type "Key Structure"))
  (:`Pressed`
    (if (`self.isHoldingObj`)
      (`self.drop`)
      (else
        (`self.pick up`)))))

(event `pick up`
  (bind _playercamera (`self.PlayerCamera`))
  (bind _returnvalue (`SceneComponent.K2_GetComponentLocation` _playercamera))
  (bind _outhit (`KismetSystemLibrary.LineTraceSingle` _returnvalue (+ _returnvalue (* (`SceneComponent.GetForwardVector` _playercamera) 300.0)) "TraceTypeQuery1"))
  (if true
    (bind (_bblockinghit _binitialoverlap _time _distance _location _impactpoint _normal _impactnormal _physmat _hitactor _hitcomponent) (`GameplayStatics.BreakHitResult` _outhit))
    (if (`SceneComponent.IsSimulatingPhysics` _hitcomponent "None")
      (if (< (`PrimitiveComponent.GetMass` _hitcomponent) 2000.0)
        (`PhysicsHandleComponent.GrabComponentAtLocation` (`self.PhysicsHandle`) _hitcomponent "None" (`SceneComponent.K2_GetComponentLocation` _hitcomponent))
        (set `self.isHoldingObj` true)))))

(event `drop`
  (`PhysicsHandleComponent.ReleaseComponent` (`self.PhysicsHandle`))
  (set `self.isHoldingObj` false))

(fn `UserConstructionScript`)