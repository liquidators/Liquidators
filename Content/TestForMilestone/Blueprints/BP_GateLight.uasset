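; BP_GateLight is a gate indicator light that turns green when opened or switched on and can be set red.
; Opening also calls HMCheckInteraction and sets the OnOff flag.
; Separate events raise the Billboard component by UpDistance, either eased over time or instantly.
; Save events add an asset record to the player's HESaveGameComponent cache and restore OnOff from it, reapplying green when on.
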(event `self.Open/On`
  (params (HorrorEvent :type Boolean))
  (`/Game/HorrorEngine/Blueprints/Core/HorrorEngineMacros.HM_CheckInteraction`)
  (`LightComponent.SetLightColor` (`self.PointLight`) (struct :`G` 1.0 :`A` 1.0) true)
  (set `self.On / Off` true))

(event `Become Red`
  (`LightComponent.SetLightColor` (`self.PointLight`) (struct :`R` 1.0 :`A` 1.0) true))

(event `MoveUp`
  (`KismetSystemLibrary.MoveComponentTo` (`self.Billboard`) (+ (`self.K2_GetActorLocation`) (`self.UpDistance`)) (`self.K2_GetActorRotation`) true true 4.0))

(event `/Game/HorrorEngine/Blueprints/Core/HorrorEngineInterface.CollectSaveData`
  (bind _asmaster (`/Game/HorrorEngine/Blueprints/Core/HorrorEngineFunctions.GetPlayer`))
  (`KismetArrayLibrary.Array_Add` (`/Game/HorrorEngine/Blueprints/Core/HE_SaveGameComponent.AssetCache` (`/Game/HorrorEngine/HorrorEngine.HE_SaveGameComponent` _asmaster)) (make `/Game/HorrorEngine/Blueprints/Structures/SaveStructures/AssetsSave` (`KismetSystemLibrary.GetObjectName` self) (`self.On / Off`) false false false 0.0 0.0 0 "+00000000.00:00:00.000000000" "NewEnumerator0" (struct :`Actor` "NewEnumerator0" :`MeshSettings` (struct) :`InspectionSettings` (struct :`InspectionPivotLocation` (0.0 0.0 0.0) :`Takeable` true :`InspectionAnimation` true :`InspectionAnimationSpeedSec` 0.5 :`InspectionBeginRotation` (struct) :`InspectionBeginScale` 1.0 :`MinZoomScale` 1.0 :`MaxZoomScale` 2.0 :`RotationSpeed` 2.5 :`SlideSpeed` 1.0 :`MaxSlideValue` 10.0 :`ItemName` "NSLOCTEXT(\"[757EC0F84F4BD84324410DB728049D8B]\", \"E10479CB4ED6E61BF521DC87652CC81C\", \"Item Name\")" :`ItemInformation` "NSLOCTEXT(\"[757EC0F84F4BD84324410DB728049D8B]\", \"E5BFEA9D49A7B02C7E9058BA3D79EBA0\", \"Item Information\")" :`ReadingText` "NSLOCTEXT(\"[757EC0F84F4BD84324410DB728049D8B]\", \"6D55437E4E382ED1A48F6C8D9A0BC256\", \"Reading Text\")" :`TakeButton` (struct :`ButtonText` "NSLOCTEXT(\"[757EC0F84F4BD84324410DB728049D8B]\", \"33EB0A144730904362AAD29FCEBD9C83\", \"Take\")") :`ExamineButton` (struct :`ButtonText` "NSLOCTEXT(\"[757EC0F84F4BD84324410DB728049D8B]\", \"CF9AAAAB4B99DBC8883310810D91F75F\", \"Examine\")") :`ZoomSlideButton` (struct :`ButtonText` "NSLOCTEXT(\"[757EC0F84F4BD84324410DB728049D8B]\", \"3638E1034DC77BA491B1BFBB770D8787\", \"Zoom/Slide\")") :`DismissButton` (struct :`ButtonText` "NSLOCTEXT(\"[757EC0F84F4BD84324410DB728049D8B]\", \"9A1FE3614B6F9F3EEF18598B4AB7A5F3\", \"Dismiss\")")) :`InventorySettings` (struct :`StorageType` "NewEnumerator3" :`NumberofItemstoAddInventory` 1 :`Interactable` true :`InteractionButton` (struct :`ButtonText` "NSLOCTEXT(\"[757EC0F84F4BD84324410DB728049D8B]\", \"54A0D8FA48B914BBEE8F72BA46EA7ED3\", \"Use\")") :`SwitchButton` (struct :`ButtonText` "NSLOCTEXT(\"[757EC0F84F4BD84324410DB728049D8B]\", \"C97FE65546C67952BAC4BFB9B2B4CB6F\", \"Switch\")") :`ZoomSlideButton` (struct :`ButtonText` "NSLOCTEXT(\"[757EC0F84F4BD84324410DB728049D8B]\", \"FEC4BD57437002113421E98C163F9B50\", \"Zoom/Slide\")") :`CloseInventoryButton` (struct :`ButtonText` "NSLOCTEXT(\"[757EC0F84F4BD84324410DB728049D8B]\", \"2229A1FE46D0166C48AA7198A7612067\", \"Close\")")) :`Pistol_MeshSettingsTop` (struct) :`Vhs_CurrentTime` "+00000000.00:00:00.000000000"))))

(event `/Game/HorrorEngine/Blueprints/Core/HorrorEngineInterface.RestoreSaveData`
  (params (AssetSave :type "/Game/HorrorEngine/Blueprints/Structures/SaveStructures/AssetsSave Structure"))
  (set `self.On / Off` (`.BooleanSlot01_63_ED79FB5D49E9ED6768D7AE96EDFDE8DB` (break `/Game/HorrorEngine/Blueprints/Structures/SaveStructures/AssetsSave` AssetSave)))
  (if (`self.On / Off`)
    (`LightComponent.SetLightColor` (`self.PointLight`) (struct :`G` 1.0 :`A` 1.0) true)))

(event `Change Location When Gate On`
  (`SceneComponent.K2_SetRelativeLocation` (`self.Billboard`) (+ (`self.K2_GetActorLocation`) (`self.UpDistance`)) false false))

(fn `UserConstructionScript`
  (`parent.UserConstructionScript`))