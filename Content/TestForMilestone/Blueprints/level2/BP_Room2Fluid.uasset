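; Water volume actor for room 2 that fades in underwater screen effects when the player's camera sinks below its surface.
; A looping timer checks box overlap and camera height, using paired DoOnce gates to play or quickly reverse the BlurStart timeline.
; The timeline drives tagged Chameleon post-process actors for waves, blur, flares, darkening and blue tint.
; MoveUp slowly raises the mesh, while the death trigger is left unconnected.
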(event `Update Water Visuals`
  (params (UnderWaterTimer :type "Float (double-precision)"))
  (set `self.UnderWaterTimer` UnderWaterTimer)
  (`self.UnderwaterVisuals`)
  (`self.ToggleOffUnderWaterEffect`)
  (if (>= (`self.UnderWaterTimer`) 1.0)
    _))

(event `self.ReceiveBeginPlay`
  (`|ExecutionSequence`
    (:`then_0`
      (bind _outactors (`GameplayStatics.GetAllActorsWithTag` "UnderWaterEffect"))
      (set `self.UnderWaterEffect` (cast `/Game/Chameleon/Chameleon` (`|GetArrayItem` _outactors) :!pure true))
      (`KismetSystemLibrary.K2_SetTimerDelegate` (delegate `UnderWater`) 0.2 true))
    (:`then_1`
      (bind _outactors_2 (`GameplayStatics.GetAllActorsWithTag` "UnderWaterBlur"))
      (set `self.UnderwaterBlur` (cast `/Game/Chameleon/Chameleon` (`|GetArrayItem` _outactors_2) :!pure true)))
    (:`then_2`
      (bind _outactors_3 (`GameplayStatics.GetAllActorsWithTag` "UnderWaterFlare"))
      (set `self.UnderwaterFlare` (cast `/Game/Chameleon/Chameleon` (`|GetArrayItem` _outactors_3) :!pure true)))
    (:`then_3`
      (bind _outactors_4 (`GameplayStatics.GetAllActorsWithTag` "UnderWaterBlue"))
      (set `self.UnderwaterBlue` (cast `/Game/Chameleon/Chameleon` (`|GetArrayItem` _outactors_4) :!pure true)))))

(event `StartUnderWaterVisualEffect`
  (`TimelineComponent.SetPlayRate` (`self.BlurStart`) (* 1.0 1.0))
  (set `/Game/Chameleon/Chameleon.Unbound` true (`self.UnderWaterEffect`))
  (set `/Game/Chameleon/Chameleon.Unbound` true (`self.UnderwaterBlue`))
  (set `/Game/Chameleon/Chameleon.Unbound` true (`self.UnderwaterFlare`))
  (set `/Game/Chameleon/Chameleon.Unbound` true (`self.UnderwaterBlur`))
  (bind (_direction _newtrack_0) (`Timeline|BlurStart` :!via `PlayFromStart` :!label _label)
    (:`Update`
      (`self.Update Water Visuals` _newtrack_0))))

(event `Reset Start Underwater`
  (goto _label_2 :!via `Reset`))

(event `UnderWater`
  (bind (_returnvalue_x _returnvalue_y _returnvalue_z) (`KismetMathLibrary.BreakVector` (`self.K2_GetActorLocation`)))
  (bind (_returnvalue_x_2 _returnvalue_y_2 _returnvalue_z_2) (`KismetMathLibrary.BreakVector` (`PlayerCameraManager.GetCameraLocation` (`GameplayStatics.GetPlayerCameraManager` 0))))
  (if (`PrimitiveComponent.IsOverlappingActor` (`self.Box`) (`GameplayStatics.GetPlayerPawn` 0))
    (if (> (+ _returnvalue_z 5.0) _returnvalue_z_2)
      (`/Engine/EditorBlueprintResources/StandardMacros.DoOnce` false :!label _label_2
        (:`Completed`
          (`self.StartUnderWaterVisualEffect`)
          (`self.Reset Stop Underwater`)))
      (else
        (`/Engine/EditorBlueprintResources/StandardMacros.DoOnce` false :!label _label_3
          (:`Completed`
            (`self.StopUnderWaterVisualEffect`)
            (`self.Reset Start Underwater`)))))))

(event `StopUnderWaterVisualEffect`
  (set `/Game/Chameleon/Chameleon.Unbound` false (`self.UnderwaterBlue`))
  (`TimelineComponent.SetPlayRate` (`self.BlurStart`) (* 1.0 4.0))
  (goto _label :!via `Reverse`))

(event `Reset Stop Underwater`
  (goto _label_3 :!via `Reset`))

(event `Move Up`
  (bind _staticmeshcomponent (`self.StaticMeshComponent`))
  (bind (_relativelocation_x _relativelocation_y _relativelocation_z) (`KismetMathLibrary.BreakVector` (`SceneComponent.RelativeLocation` _staticmeshcomponent)))
  (`KismetSystemLibrary.MoveComponentTo` _staticmeshcomponent (`KismetMathLibrary.MakeVector` _relativelocation_x _relativelocation_y (+ _relativelocation_z 100.0)) (struct) false false 10.0))

(fn `ToggleOffUnderWaterEffect`
  (if (<= (`self.UnderWaterTimer`) 0.0)
    (set `/Game/Chameleon/Chameleon.Unbound` false (`self.UnderWaterEffect`))
    (set `/Game/Chameleon/Chameleon.Unbound` false (`self.UnderwaterFlare`))
    (set `/Game/Chameleon/Chameleon.Unbound` false (`self.UnderwaterBlur`))
    (else
      (set `/Game/Chameleon/Chameleon.Unbound` true (`self.UnderWaterEffect`))
      (set `/Game/Chameleon/Chameleon.Unbound` true (`self.UnderwaterFlare`))
      (set `/Game/Chameleon/Chameleon.Unbound` true (`self.UnderwaterBlur`)))))

(fn `UnderwaterVisuals`
  (bind _underwatereffect (`self.UnderWaterEffect`))
  (bind _returnvalue (`KismetMathLibrary.MapRangeClamped` (`self.UnderWaterTimer`) 0.0 1.0 0.0 25.0))
  ;[1 1 1] Wavy Displacement
  (set `/Game/Chameleon/Chameleon.Screen Waves X Tiling` _returnvalue _underwatereffect)
  (set `/Game/Chameleon/Chameleon.Screen Waves Y Tiling` _returnvalue _underwatereffect)
  ;[1 1 1] underwater blur
  (set `/Game/Chameleon/Chameleon.Blur Amount` (`KismetMathLibrary.MapRangeClamped` (`self.UnderWaterTimer`) 0.0 1.0 1.0 10.0) (`self.UnderwaterBlur`))
  ;[1 1 1] Underwater Flare
  (set `/Game/Chameleon/Chameleon.Anamorphic Lens Flares Intensity` (`KismetMathLibrary.MapRangeClamped` (`self.UnderWaterTimer`) 0.0 1.0 0.1 8.0) (`self.UnderwaterFlare`))
  ;[1 1 1] Darkenning
  (setmembers `PostProcessSettings` :`StructRef` (`/Game/Chameleon/Chameleon.Native Post Process` (`self.UnderWaterEffect`)) :`AutoExposureBias` (`KismetMathLibrary.MapRangeClamped` (`self.UnderWaterTimer`) 0.0 1.0 0.0 -8.0)))

(fn `UserConstructionScript`)