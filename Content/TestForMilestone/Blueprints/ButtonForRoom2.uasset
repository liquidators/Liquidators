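; Interactable Room 2 button that switches on linked actors and starts raising radioactive waste across five phase actor classes.
; Use triggers the waste rise immediately, guarded by IsTriggerred, while OpenOn activates targets and horror events before or after the animation.
; A timeline moves the button pivot along a selectable easing curve, swapping mesh and playing sounds.
; Close/Off is empty, leaving its switch-off logic disconnected; save restore reapplies state and pose.
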(event `self.Use`
  (params (HorrorEvent :type Boolean))
  ;[1 1 1] Interact Settings
  (`/Game/HorrorEngine/Blueprints/Core/HorrorEngineMacros.HM_CheckInteraction`)
  (if (`self.On / Off`)
    (`self.Close/Off` false)
    (else
      (`self.Open/On` false)
      (`self.Start using Button`))))

(event `self.Open/On`
  (params (HorrorEvent :type Boolean))
  (bind _transformtype (`self.TransformType`))
  (bind _actorstouse (`self.ActorsToUse`))
  (bind _returnvalue (or (`|EnumEquality` _transformtype "NewEnumerator0") (`|EnumEquality` _transformtype "NewEnumerator4")))
  ;[1 1 1] Open / Close Settings
  (`/Game/HorrorEngine/Blueprints/Core/HorrorEngineMacros.HM_CheckInteraction`)
  (if (not (`self.On / Off`))
    (if (not (`self.UseAfterAnimation`))
      (set `self.On / Off` true)
      (`self.Open/On` (`self.ActorsToUse`) false)
      (`self.HorrorEventCheck` "NewEnumerator3"))
    (set `self.InteractionEnabled` false)
    (bind (_direction _direct _direct__easy_ease_ _elastic _elastic__easy_ease_ _flip_flop _flip_flop__easy_ease_) (`Timeline|ButtonTimeline` :!via `PlayFromStart`)
      (:`Update`
        (bind _returnvalue_2 (select `/Game/HorrorEngine/Blueprints/Enums/TransfromType` (`self.TransformType`) :`NewEnumerator0` _direct :`NewEnumerator4` _direct__easy_ease_ :`NewEnumerator5` _elastic :`NewEnumerator8` _elastic__easy_ease_ :`NewEnumerator9` _flip_flop :`NewEnumerator13` _flip_flop__easy_ease_))
        (`SceneComponent.K2_SetRelativeLocationAndRotation` (`self.ButtonPivot`) (`KismetMathLibrary.VLerp` (`self.OffLocation`) (`self.OnLocation`) _returnvalue_2) (`KismetMathLibrary.RLerp` (`self.OffRotation`) (`self.OnRotation`) _returnvalue_2) false false))
      (:`Finished`
        (switch `ETimelineDirection` _direction
          (:`Forward`
            (`/Game/HorrorEngine/Blueprints/Core/HorrorEngineFunctions.SetMesh` (`self.Button`) (`self.ButtonOnMesh`))
            (if (`self.UseAfterAnimation`)
              (set `self.On / Off` true)
              (`self.Open/On` _actorstouse false)
              (`self.HorrorEventCheck` "NewEnumerator3")))
          (:`Backward`
            (`/Game/HorrorEngine/Blueprints/Core/HorrorEngineFunctions.SetMesh` (`self.Button`) (`self.ButtonOffMesh`))
            (if (`self.UseAfterAnimation`)
              (set `self.On / Off` false)
              (`self.Close/Off` _actorstouse false)
              (`self.HorrorEventCheck` "NewEnumerator4"))))
        (set `self.InteractionEnabled` true)
        (if (`self.StopSoundsAfterAnimation`)
          (`/Game/HorrorEngine/Blueprints/Core/HorrorEngineMacros.HM_StopAll3DSounds`)))
      (:`ButtonStartSound`
        (if _returnvalue
          (switch `ETimelineDirection` _direction
            (:`Forward`
              _)))
        (`/Game/HorrorEngine/Blueprints/Core/HorrorEngineMacros.HM_3DSound` null false (`self.TurnOnSound`) (`self.ButtonPivot`) (`self.SoundAttenuation`)))
      (:`ButtonEndSound`
        (if _returnvalue
          (switch `ETimelineDirection` _direction
            (:`Backward`
              _)))
        (`/Game/HorrorEngine/Blueprints/Core/HorrorEngineMacros.HM_3DSound` null false (`self.TurnOffSound`) (`self.ButtonPivot`) (`self.SoundAttenuation`))))))

(event `self.Close/Off`
  (params (HorrorEvent :type Boolean))
  ;[1 1 1] Open / Close Settings
)

(event `/Game/HorrorEngine/Blueprints/Core/HorrorEngineInterface.CollectSaveData`
  ;[0 1 0.5572] Save Settings
  (bind _asmaster (`/Game/HorrorEngine/Blueprints/Core/HorrorEngineFunctions.GetPlayer`))
  (`KismetArrayLibrary.Array_Add` (`/Game/HorrorEngine/Blueprints/Core/HE_SaveGameComponent.AssetCache` (`/Game/HorrorEngine/HorrorEngine.HE_SaveGameComponent` _asmaster)) (make `/Game/HorrorEngine/Blueprints/Structures/SaveStructures/AssetsSave` (`KismetSystemLibrary.GetObjectName` self) (`self.On / Off`) false false false 0.0 0.0 0 "+00000000.00:00:00.000000000" "NewEnumerator0" (struct :`Actor` "NewEnumerator0" :`MeshSettings` (struct) :`InspectionSettings` (struct :`InspectionPivotLocation` (0.0 0.0 0.0) :`Takeable` true :`InspectionAnimation` true :`InspectionAnimationSpeedSec` 0.5 :`InspectionBeginRotation` (struct) :`InspectionBeginScale` 1.0 :`MinZoomScale` 1.0 :`MaxZoomScale` 2.0 :`RotationSpeed` 2.5 :`SlideSpeed` 1.0 :`MaxSlideValue` 10.0 :`ItemName` "NSLOCTEXT(\"[0512E7894598FB4A2F0E0ABB7DD1EF09]\", \"BC43AEEC46E64946091244BEF876D814\", \"Item Name\")" :`ItemInformation` "NSLOCTEXT(\"[0512E7894598FB4A2F0E0ABB7DD1EF09]\", \"878F6E5F4FBF59F40401249B1B64BF52\", \"Item Information\")" :`ReadingText` "NSLOCTEXT(\"[0512E7894598FB4A2F0E0ABB7DD1EF09]\", \"E3FD87454667DB430B23039A6D2B0858\", \"Reading Text\")" :`TakeButton` (struct :`ButtonText` "NSLOCTEXT(\"[0512E7894598FB4A2F0E0ABB7DD1EF09]\", \"1E3182B1490A69A144F44B9FA249AE45\", \"Take\")") :`ExamineButton` (struct :`ButtonText` "NSLOCTEXT(\"[0512E7894598FB4A2F0E0ABB7DD1EF09]\", \"B3DCF5474EF08070CF2FDABFA4731E19\", \"Examine\")") :`ZoomSlideButton` (struct :`ButtonText` "NSLOCTEXT(\"[0512E7894598FB4A2F0E0ABB7DD1EF09]\", \"1589E8EC4187E7CF524B289407B690A0\", \"Zoom/Slide\")") :`DismissButton` (struct :`ButtonText` "NSLOCTEXT(\"[0512E7894598FB4A2F0E0ABB7DD1EF09]\", \"A48782014CD57BEAF757A4BC12AA8BB0\", \"Dismiss\")")) :`InventorySettings` (struct :`StorageType` "NewEnumerator3" :`NumberofItemstoAddInventory` 1 :`Interactable` true :`InteractionButton` (struct :`ButtonText` "NSLOCTEXT(\"[0512E7894598FB4A2F0E0ABB7DD1EF09]\", \"32E900E345D096F3B13B1FA33A65D9AB\", \"Use\")") :`SwitchButton` (struct :`ButtonText` "NSLOCTEXT(\"[0512E7894598FB4A2F0E0ABB7DD1EF09]\", \"C407006047763C56448F15914A8F08DF\", \"Switch\")") :`ZoomSlideButton` (struct :`ButtonText` "NSLOCTEXT(\"[0512E7894598FB4A2F0E0ABB7DD1EF09]\", \"19C5F3594DE5DE1BC075AD85391A9176\", \"Zoom/Slide\")") :`CloseInventoryButton` (struct :`ButtonText` "NSLOCTEXT(\"[0512E7894598FB4A2F0E0ABB7DD1EF09]\", \"A9B299344E01C9AED719BB90778371E0\", \"Close\")")) :`Pistol_MeshSettingsTop` (struct) :`Vhs_CurrentTime` "+00000000.00:00:00.000000000"))))

(event `/Game/HorrorEngine/Blueprints/Core/HorrorEngineInterface.RestoreSaveData`
  (params (AssetSave :type "/Game/HorrorEngine/Blueprints/Structures/SaveStructures/AssetsSave Structure"))
  (bind _offrotation (`self.OffRotation`))
  (bind _offlocation (`self.OffLocation`))
  (bind _transformtype (`self.TransformType`))
  (bind _returnvalue (or (`|EnumEquality` _transformtype "NewEnumerator9") (`|EnumEquality` _transformtype "NewEnumerator13")))
  ;[0 1 0.5572] Save Settings
  (set `self.On / Off` (`.BooleanSlot01_63_ED79FB5D49E9ED6768D7AE96EDFDE8DB` (break `/Game/HorrorEngine/Blueprints/Structures/SaveStructures/AssetsSave` AssetSave)))
  (`/Game/HorrorEngine/Blueprints/Core/HorrorEngineFunctions.SetMesh` (`self.Button`) (select `bool` (`self.On / Off`) :`false` (`self.ButtonOffMesh`) :`true` (`self.ButtonOnMesh`)))
  (`SceneComponent.K2_SetRelativeLocationAndRotation` (`self.ButtonPivot`) (select `bool` _returnvalue :`false` (select `bool` (`self.On / Off`) :`false` _offlocation :`true` (`self.OnLocation`)) :`true` _offlocation) (select `bool` _returnvalue :`false` (select `bool` (`self.On / Off`) :`false` _offrotation :`true` (`self.OnRotation`)) :`true` _offrotation) false false))

(fn `UserConstructionScript`
  (bind _offrotation (`self.OffRotation`))
  (bind _offlocation (`self.OffLocation`))
  (bind _transformtype (`self.TransformType`))
  (bind _returnvalue (or (`|EnumEquality` _transformtype "NewEnumerator9") (`|EnumEquality` _transformtype "NewEnumerator13")))
  (`/Game/HorrorEngine/Blueprints/Core/HorrorEngineMacros.HM_DefaultConstructions` (`self.CreateNewHorrorEvent`))
  (`/Game/HorrorEngine/Blueprints/Core/HorrorEngineFunctions.SetMesh` (`self.ButtonBase`) (`self.ButtonBaseMesh`))
  (`/Game/HorrorEngine/Blueprints/Core/HorrorEngineFunctions.SetMesh` (`self.Button`) (select `bool` (`self.On / Off`) :`false` (`self.ButtonOffMesh`) :`true` (`self.ButtonOnMesh`)))
  (`/Game/HorrorEngine/Blueprints/Core/HorrorEngineFunctions.PlayRate` (`self.ButtonTimeline`) (`self.Animation Speed (Sec)`))
  (`SceneComponent.K2_SetRelativeLocationAndRotation` (`self.ButtonPivot`) (select `bool` _returnvalue :`false` (select `bool` (`self.On / Off`) :`false` _offlocation :`true` (`self.OnLocation`)) :`true` _offlocation) (select `bool` _returnvalue :`false` (select `bool` (`self.On / Off`) :`false` _offrotation :`true` (`self.OnRotation`)) :`true` _offrotation) false false))