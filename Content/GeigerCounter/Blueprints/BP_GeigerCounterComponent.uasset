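; Actor component that gives its owner a working Geiger counter, spawning BP_GeigerCounter on a named skeletal mesh socket with on/off switching.
; Each tick, it sphere-overlaps radioactive waste and weights sources by distance, control-rotation angle and line-trace occlusion.
; Summed radiation feeds the text readout, while the strongest volume and shortest randomized interval drive a self-restarting tick-sound timer, the interpolated needle and a high-level needle rattle.
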(event `SwitchOn`
  ;[1 1 1] Switch Rotation
  (`GameplayStatics.PlaySound2D` "/Game/GeigerCounter/Audio/SoundCues/Cue_SwitchON.Cue_SwitchON" 1.0 1.0 0.0 null null)
  (`/Game/GeigerCounter/Blueprints/BP_GeigerCounter.SwitchOn` (`self.BP_GeigerCounter`)))

(event `SwitchOff`
  ;[1 1 1] Switch Rotation
  (`GameplayStatics.PlaySound2D` "/Game/GeigerCounter/Audio/SoundCues/Cue_SwitchOFF.Cue_SwitchOFF" 1.0 1.0 0.0 null null)
  (`/Game/GeigerCounter/Blueprints/BP_GeigerCounter.SwitchOff` (`self.BP_GeigerCounter`)))

(event `self.ReceiveBeginPlay`
  ;[1 1 1] Spawning Geiger Counter, attaching it to skeleton
  (`|ExecutionSequence`
    (:`then_0`
      (bind _returnvalue (`|SpawnActorFromClass` "/Game/GeigerCounter/Blueprints/BP_GeigerCounter.BP_GeigerCounter_C" (`KismetMathLibrary.MakeTransform` (0.0 0.0 0.0)) "Undefined" "OverrideRootScale" null null))
      (set `self.BP_GeigerCounter` _returnvalue)
      (for _array_element (`SceneComponent.GetChildrenComponents` (`Actor.RootComponent` (`self.GetOwner`)) true)
        (if (`KismetStringLibrary.EqualEqual_StrStr` (`KismetSystemLibrary.GetObjectName` _array_element) (`self.CharacterMeshName`))
          (bind _asskeletal_mesh_component (cast `SkeletalMeshComponent` _array_element))
          (set `self.SkeletalMesh` _asskeletal_mesh_component)))
      (`/Engine/EditorBlueprintResources/StandardMacros.IsValid` (`self.SkeletalMesh`)
        (:`Is Valid`
          (`Actor.K2_AttachToComponent` (`self.BP_GeigerCounter`) (`self.SkeletalMesh`) (`self.SocketName`) "SnapToTarget" "SnapToTarget" "SnapToTarget" true))
        (:`Is Not Valid`
          (`KismetSystemLibrary.PrintString` "Error: Character Mesh Name not found" true true (struct :`R` 1.0 :`A` 1.0)))))
    (:`then_1`
      (bind _returnvalue_2 (`GameplayStatics.SpawnSound2D` "/Game/GeigerCounter/Audio/SoundCues/Cue_Ticking.Cue_Ticking" 1.0 1.0 0.0 null false false))
      (set `self.GeigerSound_Cue` _returnvalue_2)
      (`KismetSystemLibrary.K2_SetTimerDelegate` (delegate `TickingSound`) (`self.Tick Frequency`) :!label _label)
      (`AudioComponent.Play` (`self.GeigerSound_Cue`) 0.0))))

(event `TickingSound`
  ;[1 1 1] Spawning Geiger Counter, attaching it to skeleton
  (goto _label))

(event `self.ReceiveTick`
  (params (DeltaSeconds :type "Float (single-precision)"))
  (bind _occlusioneffect (`self.OcclusionEffect`))
  (bind _returnvalue (`Actor.K2_GetActorLocation` (`self.GetOwner`)))
  (`|ExecutionSequence`
    (:`then_1`
      (bind _outactors (`KismetSystemLibrary.SphereOverlapActors` (`Actor.K2_GetActorLocation` (`self.GetOwner`)) (`self.OuterDistance`) (`|MakeArray` "ObjectTypeQuery2" :!type "EObjectTypeQuery Enum") (`self.RadioactiveWasteBaseClass`)))
      (set `self.Volume Multiplier` 0.0)
      (set `self.Total Detected Radiation` 0.0)
      (set `self.Tick Frequency` 0.5)
      (for _array_element _outactors
        (bind _returnvalue_2 (`Actor.K2_GetActorLocation` _array_element))
        ;[1 1 1] OcclusionEffect
        (bind _outhit (`KismetSystemLibrary.LineTraceSingle` _returnvalue _returnvalue_2 "TraceTypeQuery1"))
        (bind _returnvalue_3 (- _returnvalue_2 _returnvalue))
        (bind _returnvalue_4 (`KismetMathLibrary.Normal` _returnvalue_3))
        (bind _returnvalue_5 (`KismetMathLibrary.DegAcos` (`KismetMathLibrary.Dot_VectorVector` _returnvalue_4 (`KismetMathLibrary.GetForwardVector` (`Pawn.GetControlRotation` (`GameplayStatics.GetPlayerCharacter` 0))))))
        (bind _returnvalue_6 (`KismetMathLibrary.VSize` _returnvalue_3))
        (bind _returnvalue_7 (- (`KismetMathLibrary.VSize` (- (+ _returnvalue_2 (* (`KismetMathLibrary.GreaterGreater_VectorRotator` _returnvalue_4 (struct :`Yaw` 90.0)) (`self.DirectionalSensitivity`))) _returnvalue)) _returnvalue_6))
        (bind _returnvalue_8 (* (`KismetMathLibrary.MapRangeClamped` _returnvalue_5 (* _returnvalue_7 0.4) _returnvalue_7 1.0 (`KismetMathLibrary.MapRangeClamped` (`self.RotationImpact`) 0.0 1.0 1.0)) (`KismetMathLibrary.MapRangeClamped` _returnvalue_6 (`self.InnerDistance`) (`self.OuterDistance`) 1.0)))
        (bind _returnvalue_9 (`KismetMathLibrary.SelectFloat` 1.0 (`KismetMathLibrary.MapRangeClamped` _occlusioneffect 0.0 1.0 1.0) (== (`.ImpactPoint` (`GameplayStatics.BreakHitResult` _outhit)) _returnvalue_2 :`ErrorTolerance` 100.0)))
        (set `self.Volume Multiplier` (`KismetMathLibrary.FMax` (`self.Volume Multiplier`) (* (+ _returnvalue_8 (`KismetMathLibrary.RandomFloatInRange` 0.0 (`KismetMathLibrary.MultiplyMultiply_FloatFloat` _returnvalue_8 4.0))) _returnvalue_9)) :!pinned true) ; Set Volume Mulitplier
        (bind _output_get (set `self.Total Detected Radiation` (+ (* _returnvalue_9 _returnvalue_8) (`self.Total Detected Radiation`)) :!pinned true)) ; Set Total Detect Radiation
        (bind _returnvalue_10 (`KismetMathLibrary.MapRangeClamped` _returnvalue_5 (* _returnvalue_7 0.3) (* _returnvalue_7 2.0) 0.0 0.1))
        (set `self.Tick Frequency` (`KismetMathLibrary.FMin` (/ (* (`KismetMathLibrary.MapRangeClamped` _returnvalue_9 0.0 1.0 (`KismetMathLibrary.MapRangeClamped` _occlusioneffect 0.0 1.0 1.0 4.0) 1.0) (* (`KismetMathLibrary.MultiplyMultiply_FloatFloat` (+ (* (+ _returnvalue_10 (`KismetMathLibrary.RandomFloatInRange` (/ _returnvalue_10 2.0) _returnvalue_10)) (`self.RotationImpact`)) (`KismetMathLibrary.MapRangeClamped` _returnvalue_6 (`self.InnerDistance`) (`self.OuterDistance`) (`KismetMathLibrary.RandomFloatInRange` 0.03 0.07) (`KismetMathLibrary.RandomFloatInRange` 0.2 0.5))) 2.0) 2.0)) 1.0) (`self.Tick Frequency`)) :!pinned true) ; Set Tick Frequency
        (`TextRenderComponent.K2_SetText` (`/Game/GeigerCounter/Blueprints/BP_GeigerCounter.TextRender` (`self.BP_GeigerCounter`)) (`KismetTextLibrary.Conv_DoubleToText` _output_get "HalfToEven")))
      (`|ExecutionSequence`
        (:`then_0`
          ;[1 1 1] Needle movement
          (bind _output_get_2 (set `self.NeedleMovementInterpolate` (`KismetMathLibrary.FInterpTo` (`self.NeedleMovementInterpolate`) (`KismetMathLibrary.MapRangeClamped` (* (`KismetMathLibrary.MultiplyMultiply_FloatFloat` (`KismetMathLibrary.MapRangeClamped` (/ 1.0 (`self.Tick Frequency`)) 2.0 200.0 0.0 1.0) 0.5) (`KismetMathLibrary.FClamp` (`self.Volume Multiplier`))) 0.0 1.0 -33.0 45.0) (`GameplayStatics.GetWorldDeltaSeconds`) (`self.NeedleFlickeringAmount`))))
          (`SceneComponent.K2_SetRelativeRotation` (`/Game/GeigerCounter/Blueprints/BP_GeigerCounter.NullNeedle` (`self.BP_GeigerCounter`)) (`KismetMathLibrary.MakeRotator` 0.0 0.0 (`KismetMathLibrary.FClamp` _output_get_2 -33.0 33.0)) false false))
        (:`then_1`
          ;[1 1 1] Volume
          (`AudioComponent.SetVolumeMultiplier` (`self.GeigerSound_Cue`) (* (`self.Volume Multiplier`) (`self.Volume`)))
          ;[1 1 1] Needle Sound
          (bind _output_get_3 (set `self.NeedleTreshold` (* (/ 1.0 (`self.Tick Frequency`)) (`self.Volume Multiplier`))))
          (if (and (> _output_get_3 100.0) (`self.NeedlePlay`))
            (`/Engine/EditorBlueprintResources/StandardMacros.DoOnce` false :!label _label_2
              (:`Completed`
                (`GameplayStatics.SpawnSound2D` "/Game/GeigerCounter/Audio/SoundCues/Cue_Needle.Cue_Needle" (* (`KismetMathLibrary.MapRangeClamped` (`self.NeedleTreshold`) 150.0 300.0 0.0 1.0) (`self.VolumeNeedle`)) 1.0 0.0 null :!label _label_3)
                (`KismetSystemLibrary.Delay` (* (`KismetMathLibrary.RandomFloatInRange` 0.01 0.03) (`KismetMathLibrary.MapRangeClamped` (`self.NeedleTreshold`) 150.0 300.0 2.0 1.0)))
                (if (> (`self.NeedleTreshold`) 100.0)
                  (goto _label_3))))
            (else
              (goto _label_2 :!via `Reset`))))))))