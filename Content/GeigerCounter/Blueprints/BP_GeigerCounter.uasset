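; Geiger counter actor that displays the player's health and drives eight directional indicator lights.
; Tick polls the player to scale and toggle permanent and temporary health bars, lerping the temporary one, and updates readouts for max health and health deficit.
; Per-light events select slow yellow or fast red blinking via light function materials; Off darkens corner lights but resets center lights to steady white.
; A timeline rotates the on/off switch.
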(event `SwitchOn`
  ;[1 1 1] Switch Rotation
  (bind (_direction _switchrotation) (`Timeline|Switch` :!label _label)
    (:`Update`
      (`SceneComponent.K2_SetRelativeRotation` (`self.NullSwitch`) (`KismetMathLibrary.MakeRotator` 0.0 0.0 _switchrotation) false false))))

(event `SwitchOff`
  ;[1 1 1] Switch Rotation
  (goto _label :!via `ReverseFromEnd`))

(event `self.ReceiveTick`
  (params (DeltaSeconds :type "Float (single-precision)"))
  (bind _permanent_healthbar (`self.Permanent HealthBar`))
  (bind _temp_healthbar (`self.Temp HealthBar`))
  (bind (_relativescale3d_x _relativescale3d_y _relativescale3d_z) (`KismetMathLibrary.BreakVector` (`SceneComponent.RelativeScale3D` _temp_healthbar)))
  (bind (_relativescale3d_x_2 _relativescale3d_y_2) (`KismetMathLibrary.BreakVector` (`SceneComponent.RelativeScale3D` _permanent_healthbar)))
  (`|ExecutionSequence`
    (:`then_0`
      (bind _asmaster (`/Game/HorrorEngine/Blueprints/Core/HorrorEngineFunctions.GetPlayer`))
      (bind _maxhealth (`/Game/HorrorEngine/HorrorEngine.MaxHealth` _asmaster))
      (bind _healthupperbound (`/Game/HorrorEngine/HorrorEngine.HealthUpperBound` _asmaster))
      (if (>= _maxhealth _healthupperbound)
        (`SceneComponent.SetVisibility` _permanent_healthbar false false)
        (`SceneComponent.SetVisibility` (`self.Permanent HealthBar`) false false)
        (else
          (`SceneComponent.SetVisibility` (`self.Permanent HealthBar`) true false)
          (`SceneComponent.SetRelativeScale3D` _permanent_healthbar (`KismetMathLibrary.MakeVector` _relativescale3d_x_2 _relativescale3d_y_2 (`KismetMathLibrary.MapRangeClamped` _maxhealth 0.0 _healthupperbound (`self.ZScaleHealthBar`)))))))
    (:`then_1`
      (bind _asmaster_2 (`/Game/HorrorEngine/Blueprints/Core/HorrorEngineFunctions.GetPlayer`))
      (bind _health (`/Game/HorrorEngine/HorrorEngine.Health` _asmaster_2))
      (bind _healthupperbound_2 (`/Game/HorrorEngine/HorrorEngine.HealthUpperBound` _asmaster_2))
      (if (>= _health _healthupperbound_2)
        (`SceneComponent.SetVisibility` _temp_healthbar false false)
        (else
          (`SceneComponent.SetVisibility` _temp_healthbar true false)
          (`SceneComponent.SetRelativeScale3D` _temp_healthbar (`KismetMathLibrary.MakeVector` _relativescale3d_x _relativescale3d_y (`KismetMathLibrary.Lerp` _relativescale3d_z (`KismetMathLibrary.MapRangeClamped` (- _healthupperbound_2 _health) _healthupperbound_2 0.0 (`self.ZScaleHealthBar`)) 0.2))))))
    (:`then_2`
      (bind _asmaster_3 (`/Game/HorrorEngine/Blueprints/Core/HorrorEngineFunctions.GetPlayer`))
      (`TextRenderComponent.K2_SetText` (`self.TempHealth`) (`KismetTextLibrary.Conv_IntToText` (`KismetMathLibrary.FTrunc` (- (`/Game/HorrorEngine/HorrorEngine.HealthUpperBound` _asmaster_3) (`/Game/HorrorEngine/HorrorEngine.Health` _asmaster_3)))))
      (bind _asmaster_4 (`/Game/HorrorEngine/Blueprints/Core/HorrorEngineFunctions.GetPlayer`))
      (`TextRenderComponent.K2_SetText` (`self.PermHealth`) (`KismetTextLibrary.Conv_IntToText` (`KismetMathLibrary.FTrunc` (`/Game/HorrorEngine/HorrorEngine.MaxHealth` _asmaster_4)))))))

(event `self.ReceiveBeginPlay`)

(event `Back Left Slow Blink`
  ;[1 1 1] Back Left Lighting
  (`self.AdjuistBlinkSpeed` (`self.bllight`)))

(event `Front Left Slow Blink`
  ;[1 1 1] Front Left Lighting
  (`self.AdjuistBlinkSpeed` (`self.fllight`)))

(event `Back Left Fast Blink`
  ;[1 1 1] Back Left Lighting
  (`self.AdjuistBlinkSpeed` (`self.bllight`) true))

(event `Front Left Fast Blink`
  ;[1 1 1] Front Left Lighting
  (`self.AdjuistBlinkSpeed` (`self.fllight`) true))

(event `Left Center Slow Blink`
  ;[1 1 1] Left Center Lighting
  (`self.AdjuistBlinkSpeed` (`self.lclight`)))

(event `Back Left Off`
  ;[1 1 1] Back Left Lighting
  (`LightComponent.SetIntensity` (`self.bllight`) 0.0))

(event `Front Left Off`
  ;[1 1 1] Front Left Lighting
  (`LightComponent.SetIntensity` (`self.fllight`) 0.0))

(event `Left Center Fast Blink`
  ;[1 1 1] Left Center Lighting
  (`self.AdjuistBlinkSpeed` (`self.lclight`) true))

(event `Back Center Slow Blink`
  ;[1 1 1] Back Center Lighting
  (`self.AdjuistBlinkSpeed` (`self.bclight`)))

(event `Left Center Off`
  ;[1 1 1] Left Center Lighting
  (`self.Set To Default Light` (`self.lclight`)))

(event `Back Center Fast Blink`
  ;[1 1 1] Back Center Lighting
  (`self.AdjuistBlinkSpeed` (`self.bclight`) true))

(event `Front Center Slow Blink`
  ;[1 1 1] Front Center Lighting
  (`self.AdjuistBlinkSpeed` (`self.fclight`)))

(event `Right Center Slow Blink`
  ;[1 1 1] Right Center Lighting
  (`self.AdjuistBlinkSpeed` (`self.rclight`)))

(event `Back Center Off`
  ;[1 1 1] Back Center Lighting
  (`self.Set To Default Light` (`self.bclight`)))

(event `Front Center Fast Blink`
  ;[1 1 1] Front Center Lighting
  (`self.AdjuistBlinkSpeed` (`self.fclight`) true))

(event `Right Center Fast Blink`
  ;[1 1 1] Right Center Lighting
  (`self.AdjuistBlinkSpeed` (`self.rclight`) true))

(event `Back Right Slow Blink`
  ;[1 1 1] Back Right Lighting
  (`self.AdjuistBlinkSpeed` (`self.brlight`)))

(event `Front Center Off`
  ;[1 1 1] Front Center Lighting
  (`self.Set To Default Light` (`self.fclight`)))

(event `Right Center Off`
  ;[1 1 1] Right Center Lighting
  (`self.Set To Default Light` (`self.rclight`)))

(event `Back Right Fast Blink`
  ;[1 1 1] Back Right Lighting
  (`self.AdjuistBlinkSpeed` (`self.brlight`) true))

(event `Back Right Off`
  ;[1 1 1] Back Right Lighting
  (`LightComponent.SetIntensity` (`self.brlight`) 0.0))

(event `Front Right Slow Blink`
  ;[1 1 1] Front Right Lighting
  (`self.AdjuistBlinkSpeed` (`self.frlight`)))

(event `Front Right Fast Blink`
  ;[1 1 1] Front Right Lighting
  (`self.AdjuistBlinkSpeed` (`self.frlight`) true))

(event `Front Right Off`
  ;[1 1 1] Front Right Lighting
  (`LightComponent.SetIntensity` (`self.frlight`) 0.0))

(fn `AdjuistBlinkSpeed`
  (params (Light :type "SpotLightComponent Object Reference") (Fast :type Boolean))
  (if Fast
    (`LightComponent.SetLightFunctionMaterial` Light (`self.FastLightFunction`))
    (`LightComponent.SetIntensity` Light (`self.LightFastBlinkingIntensity`))
    (`LightComponent.SetLightColor` Light (struct :`R` 1.0 :`A` 1.0) true)
    (else
      (`LightComponent.SetLightFunctionMaterial` Light (`self.SlowLightFunction`))
      (`LightComponent.SetIntensity` Light (`self.LightSlowBlinkingIntensity`))
      (`LightComponent.SetLightColor` Light (struct :`R` 1.0 :`G` 0.924422 :`A` 1.0) true))))

(fn `Set To Default Light`
  (params (self2 :type "LightComponent Object Reference"))
  (`LightComponent.SetLightFunctionMaterial` self2 null)
  (`LightComponent.SetIntensity` self2 10.0)
  (`LightComponent.SetLightColor` self2 (struct :`R` 1.0 :`G` 1.0 :`B` 1.0 :`A` 1.0) true))

(fn `UserConstructionScript`)